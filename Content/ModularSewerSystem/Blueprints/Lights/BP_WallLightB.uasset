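; BP_WallLightB is a configurable wall light prop for the modular sewer system, built from a static mesh and two point lights.
; Its construction script applies the WallLightMat material to the mesh and gives both point lights the same LightColor and Intensity.
; The event graph holds only disabled stub events, so the light has no runtime logic.
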(event EventBeginPlay)

(event Collision|EventActorBeginOverlap
  (params (OtherActor :type Actor%20Object%20Reference)))

(event EventTick
  (params (DeltaSeconds :type Float%20%28single-precision%29)))

(fn ConstructionScript
  (Rendering|Material|SetMaterial (Variables|Default|GetSM_WallLightB) 0 (Variables|Default|GetWallLightMat))
  (Rendering|Components|Light|SetLightColor (Variables|Default|GetPointLight) (Variables|Default|GetLightColor) true)
  (Rendering|Components|Light|SetLightColor (Variables|Default|GetPointLight1) (Variables|Default|GetLightColor) true)
  (Rendering|Components|Light|SetIntensity (Variables|Default|GetPointLight1) (Variables|Default|GetIntensity))
  (Rendering|Components|Light|SetIntensity (Variables|Default|GetPointLight) (Variables|Default|GetIntensity)))