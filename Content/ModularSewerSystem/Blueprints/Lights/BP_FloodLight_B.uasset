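; BP_FloodLight_B is a configurable floodlight prop from the modular sewer system, set up entirely in its construction script.
; It pitches the light root by a Rotation variable and applies a shared color to one spot light and two point lights.
; The spot light takes the full Intensity while the point lights get one fiftieth of it.
; Both floodlight meshes receive the FloodlightMat material in slot 1, and the event graph is unused.
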(event EventBeginPlay)

(event Collision|EventActorBeginOverlap
  (params (OtherActor :type Actor%20Object%20Reference)))

(event EventTick
  (params (DeltaSeconds :type Float%20%28single-precision%29)))

(fn ConstructionScript
  (Transformation|SetRelativeRotation (Variables|Default|GetLightRoot) (Math|Rotator|MakeRotator 0.0 (Variables|Default|GetRotation) 0.0) false false)
  (Utilities|FlowControl|Sequence
    (:then_0
      (Rendering|Components|Light|SetLightColor (Variables|Default|GetPointLight) (Variables|Default|GetLightColor) true)
      (Rendering|Components|Light|SetLightColor (Variables|Default|GetPointLight1) (Variables|Default|GetLightColor) true)
      (Rendering|Components|Light|SetLightColor (Variables|Default|GetSpotLight) (Variables|Default|GetLightColor) true))
    (:then_1
      (Rendering|Components|Light|SetIntensity (Variables|Default|GetPointLight) (/ (Variables|Default|GetIntensity) 5e+01))
      (Rendering|Components|Light|SetIntensity (Variables|Default|GetPointLight1) (/ (Variables|Default|GetIntensity) 5e+01))
      (Rendering|Components|Light|SetIntensity (Variables|Default|GetSpotLight) (Variables|Default|GetIntensity)))
    (:then_2
      (Rendering|Material|SetMaterial (Variables|Default|GetSM_FloodLightB_Light) 1 (Variables|Default|GetFloodlightMat))
      (Rendering|Material|SetMaterial (Variables|Default|GetSM_FloodLightB_Light_2) 1 (Variables|Default|GetFloodlightMat)))))