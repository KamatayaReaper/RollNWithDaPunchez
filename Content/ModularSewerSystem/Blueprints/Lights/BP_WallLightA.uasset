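; BP_WallLightA is a configurable wall light prop from the Modular Sewer System.
; Its construction script applies the WallLightMat material to the first slot of the SMWallLightA mesh.
; The same script pushes the shared LightColor and Intensity variables to both point light components, so the pair always matches.
; It has no runtime logic, as BeginPlay is empty.
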(event EventBeginPlay)

(fn ConstructionScript
  (Rendering|Material|SetMaterial (Variables|Default|GetSM_WallLightA) 0 (Variables|Default|GetWallLightMat))
  (Rendering|Components|Light|SetLightColor (Variables|Default|GetPointLight1) (Variables|Default|GetLightColor) true)
  (Rendering|Components|Light|SetLightColor (Variables|Default|GetPointLight) (Variables|Default|GetLightColor) true)
  (Rendering|Components|Light|SetIntensity (Variables|Default|GetPointLight1) (Variables|Default|GetIntensity))
  (Rendering|Components|Light|SetIntensity (Variables|Default|GetPointLight) (Variables|Default|GetIntensity)))