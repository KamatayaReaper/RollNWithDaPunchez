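; Overlap trigger actor that turns a referenced skeletal mesh actor into a ragdoll in the map.
; On any actor overlap, it toggles the visibility of Show, enables physics simulation at full blend weight on Object's bodies from the Hips bone down, and destroys the Destroy actor.
; The whole sequence requires a valid Show reference, while Object and Destroy are each validity-checked inside it.
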(event EventBeginPlay)

(event Collision|EventActorBeginOverlap
  (params (OtherActor :type Actor%20Object%20Reference))
  (bind _returnvalue (Utilities|Name|MakeLiteralName "Hips"))
  (bind _show (Variables|Default|Getshow))
  (bind _destroy (Variables|Default|GetDestroy))
  (bind _object (Variables|Default|GetObject))
  (bind _skeletalmeshcomponent (Variables|/Script/Engine.SkeletalMeshActor|GetSkeletalMeshComponent _object))
  (Utilities|IsValid _show
    (:Is%20Valid
      (Rendering|ToggleVisibility _show false)
      (Utilities|IsValid _object
        (:Is%20Valid
          (Class|SkeletalMeshComponent|SetAllBodiesBelowSimulatePhysics _skeletalmeshcomponent _returnvalue true true)
          (Class|SkeletalMeshComponent|SetAllBodiesBelowPhysicsBlendWeight _skeletalmeshcomponent _returnvalue 1.0 false true))
        (:Is%20Not%20Valid
          _))
      (Utilities|IsValid _destroy
        (:Is%20Valid
          (Actor|DestroyActor _destroy))))))

(event EventTick
  (params (DeltaSeconds :type Float%20%28single-precision%29)))

(fn ConstructionScript)