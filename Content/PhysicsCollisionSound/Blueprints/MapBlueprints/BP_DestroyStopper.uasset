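; BP_DestroyStopper is an interactable actor that removes its Cube component, apparently a blocker, when the E key is pressed inside its trigger.
; Begin and end overlap set an Intrigger flag, toggle the Press component's visibility, and open or close a Gate.
; The E key feeds that Gate, so the validity-checked destroy only runs while it is open.
; Overlaps are not filtered by actor.
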(event EventBeginPlay)

(event Collision|EventActorBeginOverlap
  (params (OtherActor :type Actor%20Object%20Reference))
  (bind _cube (Variables|Default|GetCube))
  (Variables|Default|SetIntrigger true)
  (if (Variables|Default|GetIntrigger)
    (Rendering|ToggleVisibility (Variables|Default|Getpress) false)
    (Utilities|FlowControl|Gate true) ; enters at Open
    (else
      (Rendering|ToggleVisibility (Variables|Default|Getpress) false)
      (Utilities|FlowControl|Gate true) ; enters at Close
    )))

(event EventTick
  (params (DeltaSeconds :type Float%20%28single-precision%29)))

(event Collision|EventActorEndOverlap
  (params (OtherActor :type Actor%20Object%20Reference))
  (bind _cube (Variables|Default|GetCube))
  (Variables|Default|SetIntrigger false)
  (if (Variables|Default|GetIntrigger)
    (Rendering|ToggleVisibility (Variables|Default|Getpress) false)
    (Utilities|FlowControl|Gate true) ; enters at Open
    (else
      (Rendering|ToggleVisibility (Variables|Default|Getpress) false)
      (Utilities|FlowControl|Gate true) ; enters at Close
    )))

(event Input|KeyboardEvents|E
  (params (Key :type Key%20Structure))
  (bind _cube (Variables|Default|GetCube))
  (:Pressed
    (Utilities|FlowControl|Gate true
      (:Exit
        (Utilities|IsValid _cube
          (:Is%20Valid
            (Components|DestroyComponent _cube)))))))

(fn ConstructionScript)