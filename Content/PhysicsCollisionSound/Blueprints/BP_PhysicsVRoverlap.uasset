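; BP_PhysicsVRoverlap is a component that notifies BP_PhysicsCollisionSound components when its owning actor starts or stops overlapping, apparently for VR interaction sounds.
; It scans the other actor's overlapping components for a sound component as first child.
; On begin, it calls VRoverlap, sets state flags and passes the owner and its closest collision point.
; On end, it clears the active flag and actor reference.
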(event Custom|BeginOverlap
  (params (OverlappedActor :type Actor%20Object%20Reference) (OtherActor :type Actor%20Object%20Reference))
  (bind _returnvalue (Components|GetOwner))
  (for _array_element (Class|Actor|GetOverlappingComponents OtherActor)
    (bind _asbp_physics_collision_sound (Utilities|Casting|CastToBP_PhysicsCollisionSound (Components|GetChildComponent _array_element 0)))
    (Variables|/Game/PhysicsCollisionSound/Blueprints/BP_PhysicsCollisionSound.BP_PhysicsCollisionSound_C|SetDoNotTouchThisVarVRoverlap _asbp_physics_collision_sound true)
    (Default|VRoverlap _asbp_physics_collision_sound)
    (Variables|/Game/PhysicsCollisionSound/Blueprints/BP_PhysicsCollisionSound.BP_PhysicsCollisionSound_C|SetDoNotChangeThisBool _asbp_physics_collision_sound true)
    (Variables|/Game/PhysicsCollisionSound/Blueprints/BP_PhysicsCollisionSound.BP_PhysicsCollisionSound_C|SetDoNotChangeThisActor _asbp_physics_collision_sound _returnvalue)
    (Variables|/Game/PhysicsCollisionSound/Blueprints/BP_PhysicsCollisionSound.BP_PhysicsCollisionSound_C|SetDoNotChangeThisVector _asbp_physics_collision_sound (.OutPointOnBody (Collision|GetClosestPointonCollision (Actor|GetComponentbyClass _returnvalue "/Script/Engine.PrimitiveComponent") (Transformation|GetWorldLocation (Variables|/Game/PhysicsCollisionSound/Blueprints/BP_PhysicsCollisionSound.BP_PhysicsCollisionSound_C|GetGetOwnerThis _asbp_physics_collision_sound)) "None")))))

(event Custom|EndOverlap
  (params (OverlappedActor :type Actor%20Object%20Reference) (OtherActor :type Actor%20Object%20Reference))
  (for _array_element (Class|Actor|GetOverlappingComponents OtherActor)
    (bind _asbp_physics_collision_sound (Utilities|Casting|CastToBP_PhysicsCollisionSound (Components|GetChildComponent _array_element 0)))
    (Variables|/Game/PhysicsCollisionSound/Blueprints/BP_PhysicsCollisionSound.BP_PhysicsCollisionSound_C|SetDoNotChangeThisBool _asbp_physics_collision_sound false)
    (Variables|/Game/PhysicsCollisionSound/Blueprints/BP_PhysicsCollisionSound.BP_PhysicsCollisionSound_C|SetDoNotChangeThisActor _asbp_physics_collision_sound 0)))

(event EventBeginPlay
  (bind _returnvalue (Components|GetOwner))
  (Collision|BindEventtoOnActorBeginOverlap _returnvalue (delegate Custom|BeginOverlap))
  (Collision|BindEventtoOnActorEndOverlap _returnvalue (delegate Custom|EndOverlap)))