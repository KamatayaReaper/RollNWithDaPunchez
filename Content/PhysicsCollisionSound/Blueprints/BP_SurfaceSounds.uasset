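; BP_SurfaceSounds is a Blueprint in the physics collision sound system that holds noise damper hit sounds.
; On BeginPlay it walks NoiseDamperHit2Array in reverse and removes invalid entries, so removals do not disrupt the remaining indices.
; If CacheSounds is enabled, it then primes NoiseDamperHit1 and every remaining array sound ahead of playback.
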(event EventBeginPlay
  (bind _noisedamperhit2array (Variables|Default|GetNoiseDamperHit2Array))
  (bind (_arrayindex _arrayelement) (Utilities|Array|ReverseforEachLoop _noisedamperhit2array)
    (:LoopBody
      (Utilities|IsValid _arrayelement
        (:Is%20Not%20Valid
          (Utilities|Array|RemoveIndex _noisedamperhit2array _arrayindex))))
    (:Completed
      (if (Variables|Default|GetCacheSounds)
        (Class|GameplayStatics|PrimeSound (Variables|Default|GetNoiseDamperHit1))
        (for _array_element (Variables|Default|GetNoiseDamperHit2Array)
          (Class|GameplayStatics|PrimeSound _array_element))))))