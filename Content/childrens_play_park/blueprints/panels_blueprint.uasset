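; Configurable panel actor for the children's play park, pairing a mesh with a text label, set up entirely in the construction script.
; PanelIndex keeps the default mesh or swaps in one of three alternative panel meshes, hiding the text for the second variant.
; All handled variants share the same text and world size update, then the text color is applied.
; The event graph holds only disabled placeholder events, so there is no runtime logic.
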(event EventBeginPlay)

(event Collision|EventActorBeginOverlap
  (params (OtherActor :type Actor%20Object%20Reference)))

(event EventTick
  (params (DeltaSeconds :type Float%20%28single-precision%29)))

(fn ConstructionScript
  (bind _panel (Variables|Default|Getpanel))
  (bind _textrender (Variables|Default|Gettextrender))
  (Utilities|FlowControl|Sequence
    (:then_0
      (switch int (Variables|Settings|Getpanel_index)
        (:0
          _)
        (:1
          (Components|StaticMesh|SetStaticMesh _panel "/Game/childrens_play_park/assets/panels_2_static_mesh.panels_2_static_mesh")
          (Rendering|SetVisibility _textrender false true))
        (:2
          (Components|StaticMesh|SetStaticMesh _panel "/Game/childrens_play_park/assets/panels_3_static_mesh.panels_3_static_mesh"))
        (:3
          (Components|StaticMesh|SetStaticMesh _panel "/Game/childrens_play_park/assets/panels_4_static_mesh.panels_4_static_mesh")))
      (Rendering|Components|TextRender|SetText _textrender (Variables|Settings|Gettext))
      (Rendering|Components|TextRender|SetWorldSize _textrender (Variables|Settings|Getsize)))
    (:then_1
      (Rendering|Components|TextRender|SetTextRenderColor (Variables|Default|Gettextrender) (Variables|Settings|Getcolor)))))