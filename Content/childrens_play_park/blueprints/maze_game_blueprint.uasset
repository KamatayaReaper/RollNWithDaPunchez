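; Modular maze-game Blueprint for a children's play park; its construction script builds a circle, tunnel, wall or ground piece based on the Module setting.
; Each module stacks or repeats instanced meshes by size parameters, with optional angled tunnels, end and side walls, rooftop, stairs or slide.
; Shared helper functions handle visibility, wall mesh swaps and colouring by fixed choice or random material.
; Wall props include static meshes or physics-simulated skeletal fabric and bags.
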(event EventBeginPlay)

(event Collision|EventActorBeginOverlap
  (params (OtherActor :type Actor%20Object%20Reference)))

(event EventTick
  (params (DeltaSeconds :type Float%20%28single-precision%29)))

(fn ConstructionScript
  (switch Utilities|FlowControl|Switch|Switchonmodules_name_enumeration (Variables|Settings|GetModule)
    (:NewEnumerator0
      (|Mod_0_cercle_2))
    (:NewEnumerator1
      (|Mod_1_tunnel_2))
    (:NewEnumerator2
      (|Mod_2_wall_2))
    (:NewEnumerator3
      (|Mod_3_ground_2))))

(fn VisibilityFunction
  (params (Condition :type Boolean) (Target :type Scene%20Component%20Object%20Reference))
  (if Condition
    (Rendering|SetVisibility Target true false)
    (else
      (Rendering|SetVisibility Target false true))))

(fn ColorFunction
  (params (Selection :type garden_game_enumeration%20Enum :default "NewEnumerator0") (Target :type Primitive%20Component%20Object%20Reference) (ElementIndex :type Integer))
  (if (Variables|Settings|Getcolor_random)
    (Rendering|Material|SetMaterial Target ElementIndex (.OutItem (Utilities|Array|Random (Utilities|Array|MakeArray "/Game/childrens_play_park/materials/maze_game_material_Inst1.maze_game_material_Inst1" "/Game/childrens_play_park/materials/maze_game_material_Inst2.maze_game_material_Inst2" "/Game/childrens_play_park/materials/maze_game_material_Inst3.maze_game_material_Inst3" "/Game/childrens_play_park/materials/maze_game_material_Inst4.maze_game_material_Inst4" "/Game/childrens_play_park/materials/maze_game_material_Inst5.maze_game_material_Inst5"))))
    (else
      (switch Utilities|FlowControl|Switch|Switchongarden_game_enumeration Selection
        (:NewEnumerator0
          (Rendering|Material|SetMaterial Target ElementIndex "/Game/childrens_play_park/materials/maze_game_material_Inst1.maze_game_material_Inst1"))
        (:NewEnumerator1
          (Rendering|Material|SetMaterial Target ElementIndex "/Game/childrens_play_park/materials/maze_game_material_Inst2.maze_game_material_Inst2"))
        (:NewEnumerator2
          (Rendering|Material|SetMaterial Target ElementIndex "/Game/childrens_play_park/materials/maze_game_material_Inst3.maze_game_material_Inst3"))
        (:NewEnumerator3
          (Rendering|Material|SetMaterial Target ElementIndex "/Game/childrens_play_park/materials/maze_game_material_Inst4.maze_game_material_Inst4"))
        (:NewEnumerator4
          (Rendering|Material|SetMaterial Target ElementIndex "/Game/childrens_play_park/materials/maze_game_material_Inst5.maze_game_material_Inst5"))))))

(fn ColorWallGroundFunction
  (params (Selection :type garden_game_enumeration%20Enum :default "NewEnumerator0") (Target :type Primitive%20Component%20Object%20Reference) (ElementIndex :type Integer))
  (if (Variables|Settings|Getcolor_random)
    (Rendering|Material|SetMaterial Target ElementIndex (.OutItem (Utilities|Array|Random (Utilities|Array|MakeArray 0 0 0 0))))
    (else
      (switch Utilities|FlowControl|Switch|Switchongarden_game_enumeration Selection
        (:NewEnumerator0
          (Rendering|Material|SetMaterial Target ElementIndex 0))
        (:NewEnumerator1
          (Rendering|Material|SetMaterial Target ElementIndex 0))
        (:NewEnumerator2
          (Rendering|Material|SetMaterial Target ElementIndex 0))
        (:NewEnumerator3
          (Rendering|Material|SetMaterial Target ElementIndex 0))
        (:NewEnumerator4
          (Rendering|Material|SetMaterial Target ElementIndex 0))))))

(fn WallTypeFunction
  (params (Target_wall :type Static%20Mesh%20Component%20Object%20Reference) (NewMesh :type Static%20Mesh%20Object%20Reference))
  (bind _returnvalue (Transformation|GetSocketTransform Target_wall "socket_props" "RTS_World"))
  (bind _wall_type_2_instance (Variables|Default|Getwall_type_2_instance))
  (Components|StaticMesh|SetStaticMesh Target_wall NewMesh)
  (switch int (Variables|Settings|ModuleWall|Getwall_type)
    (:0
      _)
    (:1
      (Components|InstancedStaticMesh|AddInstance _wall_type_2_instance (Math|Transform|MakeTransform (.location _returnvalue) (.rotation _returnvalue) "1.200000,1.200000,1.200000") true)
      (CallFunction|ColorFunction (Variables|Settings|ModuleWall|Colors|Wall|Getwall_type_2) _wall_type_2_instance)))
  (return))