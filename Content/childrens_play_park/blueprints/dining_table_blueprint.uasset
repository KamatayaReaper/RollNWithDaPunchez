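; Configurable dining table prop with chairs and optional tableware, assembled entirely in the Construction Script.
; NumberChairs cumulatively reveals up to four chairs, ColorChairs picks their pink, green, blue or random material instance, and Dining shows the tableware.
; Random mode rerolls these settings after the chair reveal has run, then scatters plates and cups inside Box at fixed height with random yaw and randomizes chair materials.
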(event EventBeginPlay)

(event Collision|EventActorBeginOverlap
  (params (OtherActor :type Actor%20Object%20Reference)))

(event EventTick
  (params (DeltaSeconds :type Float%20%28single-precision%29)))

(fn ConstructionScript
  (bind _array (Utilities|Array|MakeArray "/Game/childrens_play_park/materials/dining_table_material_Inst.dining_table_material_Inst" "/Game/childrens_play_park/materials/dining_table_material_Inst_1.dining_table_material_Inst_1" "/Game/childrens_play_park/materials/dining_table_material_Inst_2.dining_table_material_Inst_2"))
  (bind _box (Variables|Default|GetBox))
  (bind _chair2 (Variables|Default|Getchair2))
  (bind _outitem (Utilities|Array|Random _array))
  (bind _returnvalue (Transformation|GetWorldLocation _box))
  (bind _returnvalue_2 (Components|Box|GetScaledBoxExtent _box))
  (bind _returnvalue_3 (Math|Random|RandomPointinBoundingBox _returnvalue _returnvalue_2))
  (bind (_x _y) (Math|Vector|BreakVector _returnvalue_3))
  (if (Variables|Settings|Getrandom)
    (Utilities|FlowControl|Sequence
      (:then_0
        (|CollapseGraph_2_2_2 (stale _output_get)))
      (:then_1
        (Variables|Settings|Setcolor_chairs "NewEnumerator3")
        (bind _output_get (Variables|Settings|Setnumber_chairs (Math|Random|RandomIntegerinRange 0 4)))
        (Variables|Settings|Setdining? (Math|Random|RandomBool))
        (switch Utilities|FlowControl|Switch|Switchoncolor_chairs_enumeration (Variables|Settings|Getcolor_chairs)
          (:NewEnumerator3
            (for _index (range 0 11)
              (Transformation|SetWorldLocation (Utilities|Array|Get(acopy) (Utilities|Array|MakeArray (Variables|Default|Getplate1) (Variables|Default|Getplate) (Variables|Default|Getcup1) (Variables|Default|Getcup)) _index) (Math|Vector|MakeVector _x _y 9e+01) false false)
              (Transformation|SetWorldRotation (Utilities|Array|Get(acopy) (Utilities|Array|MakeArray (Variables|Default|Getplate1) (Variables|Default|Getplate) (Variables|Default|Getcup1) (Variables|Default|Getcup)) _index) (Math|Rotator|MakeRotator 0.0 0.0 (Math|Random|RandomFloatinRange 0.0 5e+02)) false false)
              (|random_dining_2_2)
              (Rendering|Material|SetMaterial _chair2 0 _outitem)
              (Rendering|Material|SetMaterial (Variables|Default|Getchair4) 0 _outitem)
              (Rendering|Material|SetMaterial (Variables|Default|Getchair3) 0 _outitem)
              (Rendering|Material|SetMaterial _chair2 0 _outitem))))))
    (else
      (Utilities|FlowControl|Sequence
        (:then_0
          (|CollapseGraph_2_2 (Variables|Settings|Getnumber_chairs)))
        (:then_4
          (switch Utilities|FlowControl|Switch|Switchoncolor_chairs_enumeration (Variables|Settings|Getcolor_chairs)
            (:NewEnumerator0
              (Rendering|Material|SetMaterial _chair2 0 "/Game/childrens_play_park/materials/dining_table_material_Inst_1.dining_table_material_Inst_1"))
            (:NewEnumerator1
              (Rendering|Material|SetMaterial _chair2 0 "/Game/childrens_play_park/materials/dining_table_material_Inst.dining_table_material_Inst"))
            (:NewEnumerator2
              (Rendering|Material|SetMaterial _chair2 0 "/Game/childrens_play_park/materials/dining_table_material_Inst_2.dining_table_material_Inst_2"))
            (:NewEnumerator3
              (Rendering|Material|SetMaterial _chair2 0 _outitem)
              (Rendering|Material|SetMaterial (Variables|Default|Getchair4) 0 _outitem)
              (Rendering|Material|SetMaterial (Variables|Default|Getchair3) 0 _outitem)
              (Rendering|Material|SetMaterial _chair2 0 _outitem))))
        (:then_5
          (|random_dining_2_2_2))))))