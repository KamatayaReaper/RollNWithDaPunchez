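; Procedural children's play-park structure that assembles a configurable mattress floor with optional walls, slide and toys in the Construction Script.
; Length and width settings drive instanced-mesh ground and wall pieces and resize and shift a Box component.
; The Box positions the slide, which gets a random yaw on wider layouts, and bounds the random placement of three toy types.
; ColorFunction applies the selected material per part, or random ones when ColorRandom is on.
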(event EventBeginPlay)

(event Collision|EventActorBeginOverlap
  (params (OtherActor :type Actor%20Object%20Reference)))

(event EventTick
  (params (DeltaSeconds :type Float%20%28single-precision%29)))

(fn ConstructionScript
  (bind _box (Variables|Default|GetBox))
  (bind _slide (Variables|Default|Getslide))
  (bind _wall3 (Variables|Default|Getwall3))
  (bind _color_mattress (Variables|Settings|Colors|Getcolor_mattress))
  (bind _structure_width (Variables|Settings|Size|GetStructure%20Width))
  (bind _box_2 (Variables|Default|GetBox))
  (bind _box_3 (Variables|Default|GetBox))
  (bind _box_4 (Variables|Default|GetBox))
  (bind _structure_width_2 (Variables|Settings|Size|GetStructure%20Width))
  (bind _box_5 (Variables|Default|GetBox))
  (bind _color_wall (Variables|Settings|Colors|Getcolor_wall))
  (bind _toys2 (Variables|Default|Gettoys2))
  (bind _toys1 (Variables|Default|Gettoys1))
  (bind _toys3 (Variables|Default|Gettoys3))
  (bind _ground1 (Variables|Default|Getground1))
  (bind _ground2 (Variables|Default|Getground2))
  (bind _returnvalue (Transformation|GetWorldLocation _box))
  (bind _returnvalue_2 (Components|Box|GetScaledBoxExtent _box))
  (bind _returnvalue_3 (Transformation|GetWorldLocation _box_2))
  (bind _returnvalue_4 (Transformation|GetRelativeTransform _box_3))
  (bind _relativelocation (Variables|/Script/Engine.SceneComponent|GetRelativeLocation _box_5))
  (bind _returnvalue_5 (Math|Random|RandomPointinBoundingBox _returnvalue _returnvalue_2))
  (bind (_x _y) (Math|Vector|BreakVector _returnvalue_5))
  (Utilities|FlowControl|Sequence
    (:then_0
      (for _index (range 0 (Variables|Settings|Size|Getstructure_length))
        (Utilities|FlowControl|Sequence
          (:then_0
            (if (== _structure_width 2)
              (Transformation|SetRelativeTransform (Variables|Default|GetBox) (Math|Transform|MakeTransform "0, 0, 0" "0, 0, 0" (Math|Vector|MakeVector (.x (.scale (Transformation|GetRelativeTransform (Variables|Default|GetBox)))) (Math|Conversions|ToFloat(Integer) (* (/ _index 1) 3)) 1.0)) false false)
              (else
                (if (== _structure_width 1) :!label _label
                  _
                  (else
                    _)))))
          (:then_1
            (goto _label)))
        (Components|InstancedStaticMesh|AddInstance (Variables|Default|Getground) (Math|Transform|MakeTransform (Math|Vector|MakeVector 0.0 (Math|Conversions|ToFloat(Integer) (* _index 200)) 0.0) "0, 0, 0" "1.000000,1.000000,1.000000") false)
        (Transformation|SetRelativeLocation (Variables|Default|GetBox) (Math|Vector|MakeVector 0.0 (/ (Math|Conversions|ToFloat(Integer) (* _index 200)) 2.0) 0.0) false false)
        (if (Variables|Settings|Add|Getwall?)
          (Components|InstancedStaticMesh|AddInstance (Variables|Default|Getwall) (Math|Transform|MakeTransform (Math|Vector|MakeVector (Math|Conversions|ToFloat(Integer) (* _index 200)) 0.0 0.0) "0, 0, 0" "1.000000,1.000000,1.000000") false)
          (Components|InstancedStaticMesh|AddInstance (Variables|Default|Getwall3) (Math|Transform|MakeTransform (Math|Vector|MakeVector (Math|Conversions|ToFloat(Integer) (* _index 200)) 0.0 0.0) "0, 0, 0" "1.000000,1.000000,1.000000") false)
          (CallFunction|ColorFunction (Variables|Default|Getwall2) _color_wall)
          (CallFunction|ColorFunction (Variables|Default|Getwall) _color_wall)
          (CallFunction|ColorFunction (Variables|Default|Getwall1) _color_wall)
          (CallFunction|ColorFunction (Variables|Default|Getwall3) _color_wall))
        (if (== _structure_width_2 2)
          (Transformation|SetWorldLocation _box_2 (+ _returnvalue_3 "200.000000,0.000000,0.000000") false false)
          (bind _returnvalue_6 (Components|InstancedStaticMesh|AddInstance _ground2 (Math|Transform|MakeTransform "0, 0, 0" "0, 0, 0" "1.000000,1.000000,1.000000") false))
          (for _index_2 (range _returnvalue_6 (Variables|Settings|Size|Getstructure_length))
            (Components|InstancedStaticMesh|AddInstance _ground2 (Math|Transform|MakeTransform (Math|Vector|MakeVector 0.0 (Math|Conversions|ToFloat(Integer) (* _index_2 200)) 0.0) "0, 0, 0" "1.000000,1.000000,1.000000") false)
            (Transformation|SetRelativeTransform (Variables|Default|GetBox) (Math|Transform|MakeTransform "200.000000,0.000000,0.000000" "0, 0, 0" "9.000000,3.000000,1.000000") false false)
            (Transformation|SetRelativeLocation _wall3 (Math|Vector|MakeVector 499.0 0.0 28.0) false false)
            (Transformation|SetRelativeTransform _box_4 (Math|Transform|MakeTransform (Variables|/Script/Engine.SceneComponent|GetRelativeLocation _box_4) "0, 0, 0" (Math|Vector|MakeVector 9.0 3.0 1.0)) false false)
            (bind _returnvalue_7 (Components|InstancedStaticMesh|AddInstance _ground1 (Math|Transform|MakeTransform "0, 0, 0" "0, 0, 0" "1.000000,1.000000,1.000000") false))
            (for _index_3 (range _returnvalue_7 (Variables|Settings|Size|Getstructure_length))
              (Components|InstancedStaticMesh|AddInstance _ground1 (Math|Transform|MakeTransform (Math|Vector|MakeVector 0.0 (Math|Conversions|ToFloat(Integer) (* _index_3 200)) 0.0) "0, 0, 0" "1.000000,1.000000,1.000000") false)
              (if (Variables|Settings|Add|Getwall?)
                (for _index_4 (range 0 (Variables|Settings|Size|GetStructure%20Width))
                  (Components|InstancedStaticMesh|AddInstance (Variables|Default|Getwall1) (Math|Transform|MakeTransform (Math|Vector|MakeVector (Math|Conversions|ToFloat(Integer) (* _index_4 202)) 0.0 0.0) "0, 0, 0" "1.000000,1.000000,1.000000") false)))))
          (elif (== _structure_width_2 1)
            (Transformation|SetWorldLocation _box_2 (+ _returnvalue_3 "100.000000,0.000000,0.000000") false false)
            (Transformation|SetRelativeTransform _box_3 (Math|Transform|MakeTransform (.location _returnvalue_4) (.rotation _returnvalue_4) (Math|Vector|MakeVector 6.0 3.0 1.0)) false false)
            (Transformation|SetRelativeLocation _wall3 (Math|Vector|MakeVector 299.0 0.0 28.0) false false)
            (bind _returnvalue_8 (Components|InstancedStaticMesh|AddInstance _ground1 (Math|Transform|MakeTransform "0, 0, 0" "0, 0, 0" "1.000000,1.000000,1.000000") false))
            (for _index_5 (range _returnvalue_8 (Variables|Settings|Size|Getstructure_length))
              (Components|InstancedStaticMesh|AddInstance _ground1 (Math|Transform|MakeTransform (Math|Vector|MakeVector 0.0 (Math|Conversions|ToFloat(Integer) (* _index_5 200)) 0.0) "0, 0, 0" "1.000000,1.000000,1.000000") false)
              (if (Variables|Settings|Add|Getwall?)
                (for _index_6 (range 0 (Variables|Settings|Size|GetStructure%20Width))
                  (Components|InstancedStaticMesh|AddInstance (Variables|Default|Getwall1) (Math|Transform|MakeTransform (Math|Vector|MakeVector (Math|Conversions|ToFloat(Integer) (* _index_6 202)) 0.0 0.0) "0, 0, 0" "1.000000,1.000000,1.000000") false))))
            (elif (Variables|Settings|Add|Getwall?)
              (for _index_7 (range 0 (Variables|Settings|Size|GetStructure%20Width))
                (Components|InstancedStaticMesh|AddInstance (Variables|Default|Getwall1) (Math|Transform|MakeTransform (Math|Vector|MakeVector (Math|Conversions|ToFloat(Integer) (* _index_7 202)) 0.0 0.0) "0, 0, 0" "1.000000,1.000000,1.000000") false)))))))
    (:then_1
      (CallFunction|ColorFunction (Variables|Default|Getground2) _color_mattress)
      (CallFunction|ColorFunction (Variables|Default|Getground1) _color_mattress)
      (CallFunction|ColorFunction (Variables|Default|Getground) _color_mattress))
    (:then_2
      (if (Variables|Settings|Add|Getslide?)
        (Components|StaticMesh|SetStaticMesh _slide "/Game/childrens_play_park/assets/garden_game_slide_static_mesh.garden_game_slide_static_mesh")
        (Transformation|SetRelativeLocation _slide (Math|Vector|MakeVector (.x _relativelocation) (.y _relativelocation) 17.0) false false)
        (CallFunction|ColorFunction _slide (Variables|Settings|Colors|Getcolor_slide))
        (if (== (Variables|Settings|Size|GetStructure%20Width) 0)
          (Transformation|SetRelativeRotation _slide (Math|Rotator|MakeRotator 0.0 0.0 9e+01) false false)
          (else
            (Transformation|SetRelativeRotation _slide (Math|Rotator|MakeRotator 0.0 0.0 (Math|Random|RandomFloatinRange 0.0 1.8e+02)) false false)))
        (else
          (Components|StaticMesh|SetStaticMesh _slide 0))))
    (:then_3
      (if (Variables|Settings|Add|Gettoys?)
        (Components|InstancedStaticMesh|AddInstance _toys2 (Math|Transform|MakeTransform (Math|Vector|MakeVector _x _y 1e+01) "0, 0, 0" "1.000000,1.000000,1.000000") true)
        (CallFunction|ColorFunction _toys2 (Variables|Settings|Colors|Getcolor_toys_2))
        (Components|InstancedStaticMesh|AddInstance _toys1 (Math|Transform|MakeTransform (Math|Vector|MakeVector _x _y 1e+01) "0, 0, 0" "1.000000,1.000000,1.000000") true)
        (CallFunction|ColorFunction _toys1 (Variables|Settings|Colors|Getcolor_toys_1))
        (Components|InstancedStaticMesh|AddInstance _toys3 (Math|Transform|MakeTransform (Math|Vector|MakeVector _x _y 1e+01) "0, 0, 0" "1.000000,1.000000,1.000000") true)
        (CallFunction|ColorFunction _toys3 (Variables|Settings|Colors|Getcolor_toys_3))))))

(fn ColorFunction
  (params (Target :type Primitive%20Component%20Object%20Reference) (Selection :type garden_game_enumeration%20Enum :default "NewEnumerator0"))
  (bind _array (Utilities|Array|MakeArray "/Game/childrens_play_park/materials/garden_game_material_Inst.garden_game_material_Inst" "/Game/childrens_play_park/materials/garden_game_material_Inst1.garden_game_material_Inst1" "/Game/childrens_play_park/materials/garden_game_material_Inst2.garden_game_material_Inst2" "/Game/childrens_play_park/materials/garden_game_material_Inst3.garden_game_material_Inst3" "/Game/childrens_play_park/materials/garden_game_material_Inst4.garden_game_material_Inst4"))
  (bind _outitem (Utilities|Array|Random _array))
  (if (Variables|Settings|Getcolor_random)
    (Rendering|Material|SetMaterial (Variables|Default|Gettoys3) 0 _outitem)
    (Rendering|Material|SetMaterial (Variables|Default|Getwall) 0 _outitem)
    (Rendering|Material|SetMaterial (Variables|Default|Getground1) 0 _outitem)
    (Rendering|Material|SetMaterial (Variables|Default|Getslide) 0 _outitem)
    (Rendering|Material|SetMaterial (Variables|Default|Gettoys1) 0 _outitem)
    (Rendering|Material|SetMaterial (Variables|Default|Gettoys2) 0 _outitem)
    (else
      (switch Utilities|FlowControl|Switch|Switchongarden_game_enumeration Selection
        (:NewEnumerator0
          (Rendering|Material|SetMaterial Target 0 "/Game/childrens_play_park/materials/garden_game_material_Inst.garden_game_material_Inst"))
        (:NewEnumerator1
          (Rendering|Material|SetMaterial Target 0 "/Game/childrens_play_park/materials/garden_game_material_Inst2.garden_game_material_Inst2"))
        (:NewEnumerator2
          (Rendering|Material|SetMaterial Target 0 "/Game/childrens_play_park/materials/garden_game_material_Inst3.garden_game_material_Inst3"))
        (:NewEnumerator3
          (Rendering|Material|SetMaterial Target 0 "/Game/childrens_play_park/materials/garden_game_material_Inst1.garden_game_material_Inst1"))
        (:NewEnumerator4
          (Rendering|Material|SetMaterial Target 0 "/Game/childrens_play_park/materials/garden_game_material_Inst4.garden_game_material_Inst4"))))))