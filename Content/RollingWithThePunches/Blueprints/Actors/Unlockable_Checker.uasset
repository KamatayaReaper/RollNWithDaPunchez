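; Level actor that decides at BeginPlay whether the first-person player can still unlock the current level's unlockable.
; It caches the player character, then, if unlockables are available in the level, checks for a save game slot named after the current level.
; An existing save sets the player's CanUnlock to false and a missing one sets it to true, with the result printed to screen.
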(event EventBeginPlay
  (Utilities|FlowControl|Sequence
    (:then_0
      (bind _asbp_first_person_character (Utilities|Casting|CastToBP_FirstPersonCharacter (Game|GetPlayerCharacter 0)))
      (Variables|Default|SetPlayerRef _asbp_first_person_character))
    (:then_1
      (if (Variables|Default|GetUnlockablesAvailable?)
        (bind _returnvalue (Game|GetCurrentLevelName true))
        (bind _returnvalue_2 (SaveGame|DoesSaveGameExist _returnvalue))
        (if _returnvalue_2
          (bind _output_get (Variables|/Game/RollingWithThePunches/Blueprints/PlayerCharaacters/BP_FirstPersonCharacter.BP_FirstPersonCharacter_C|SetCanUnlock? (Variables|Default|GetPlayerRef) false))
          (Development|PrintString (Utilities|String|ToString(Boolean) _output_get))
          (else
            (bind _output_get_2 (Variables|/Game/RollingWithThePunches/Blueprints/PlayerCharaacters/BP_FirstPersonCharacter.BP_FirstPersonCharacter_C|SetCanUnlock? (Variables|Default|GetPlayerRef) true))
            (Development|PrintString (Utilities|String|ToString(Boolean) _output_get_2))))))))

(event Collision|EventActorBeginOverlap
  (params (OtherActor :type Actor%20Object%20Reference)))

(event EventTick
  (params (DeltaSeconds :type Float%20%28single-precision%29)))

(fn ConstructionScript)