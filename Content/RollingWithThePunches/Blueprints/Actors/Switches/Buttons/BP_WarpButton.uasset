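; Punchable warp button that teleports the player back to the location recorded at BeginPlay.
; Arm damage with enough ForceUnleashed calls Activate, whose timeline slides the button while moving the player; weaker hits buzz.
; A box overlap toggles a widget showing the required force.
; It also carries timed, reactivatable, single, paid and energized button logic that Activate bypasses, plus an unreachable quit-game chain.
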(event OnComponentBeginOverlap(Box)
  (params (OverlappedComponent :type Primitive%20Component%20Object%20Reference) (OtherActor :type Actor%20Object%20Reference) (OtherComp :type Primitive%20Component%20Object%20Reference) (OtherBodyIndex :type Integer) (bFromSweep :type Boolean) (SweepResult :type Hit%20Result%20Structure%20%28by%20ref%29))
  (if (== OtherActor (Variables|Default|GetPlayerRef))
    (Rendering|SetVisibility (Variables|Default|GetWidget) true false)))

(event OnComponentEndOverlap(Box)
  (params (OverlappedComponent :type Primitive%20Component%20Object%20Reference) (OtherActor :type Actor%20Object%20Reference) (OtherComp :type Primitive%20Component%20Object%20Reference) (OtherBodyIndex :type Integer))
  (if (== OtherActor (Variables|Default|GetPlayerRef))
    (Rendering|SetVisibility (Variables|Default|GetWidget) false false)))

(event Custom|ForceReactivatableOnce)

(event Custom|CountDown
  (if (Variables|Default|GetTimerActive?)
    (Utilities|FlowControl|Delay 1.0)
    (Audio|PlaySound2D "/Game/RollingWithThePunches/Assets/Sounds/Ticking/ClockTick.ClockTick" 1.0 1.0 0.0 0 0)
    (bind _output_get (Variables|Default|SetTimeRemaining (Math|Float|Clamp(Float) (- (Variables|Default|GetTimeRemaining) 1.0) 0.0 (Variables|Default|GetMaxTime))))
    (if (<= _output_get 0.0)
      (Utilities|FlowControl|Sequence
        (:then_0
          (Variables|Default|SetbCanBeDamaged true)
          (Variables|Default|SetTimerActive? false)
          (|CallParentFunction))
        (:then_1
          (Variables|Default|SetTimeRemaining (Variables|Default|GetMaxTime)))))))

(event Custom|ResetReactivatable
  (Variables|Default|SetbCanBeDamaged true))

(event Custom|ActivateTimedButton
  (bind _buttonalpha (Timeline|MoveButtonToTimer PlayFromStart)
    (:Update
      (Transformation|SetRelativeLocation (Variables|Default|GetButton) (Math|Vector|Lerp(Vector) "0,20.000000, 0" "0, 0, 0" _buttonalpha) false false)
      (Variables|Default|SetbCanBeDamaged false)
      (Variables|Default|SetTimerActive? true)
      (|CallParentFunction))))

(event Custom|ActivateReactivatableButton
  (bind _buttonalpha (Timeline|MoveButtonBack PlayFromStart)
    (:Update
      (Transformation|SetRelativeLocation (Variables|Default|GetButton) (Math|Vector|Lerp(Vector) "0,20.000000,0.000000" "0, 0, 0" _buttonalpha) false false)
      (Utilities|FlowControl|DoOnce false :!label _label
        (:Completed
          (Utilities|FlowControl|Sequence
            (:then_0
              (Utilities|FlowControl|FlipFlop
                (:A
                  (|CallParentFunction))
                (:B
                  (|CallParentFunction))))
            (:then_1
              (Utilities|FlowControl|Delay 5.0)
              (goto _label Reset))))))))

(event Custom|ActivateSingleButton
  (Utilities|FlowControl|DoOnce false
    (:Completed
      (Utilities|FlowControl|Sequence
        (:then_0
          (bind _buttonalpha (Timeline|MoveButton Play)
            (:Update
              (Transformation|SetRelativeLocation (Variables|Default|GetButton) (Math|Vector|Lerp(Vector) "0,20.000000, 0" "0, 0, 0" _buttonalpha) false false)
              (Variables|Default|SetbCanBeDamaged false)
              (|CallParentFunction))))
        (:then_1
          (if (Variables|Default|GetNotifiesPlayer?)
            (bind _returnvalue (UserInterface|CreateWidget "/Game/RollingWithThePunches/Blueprints/HUDs/Effect_HUDs/Notifications/ButtnNotification_HUD.ButtnNotification_HUD_C"))
            (UserInterface|Viewport|AddtoViewport _returnvalue 0)))))))

(event Custom|PayButton
  (bind _playerref (Variables|Default|GetPlayerRef))
  (if (>= (Variables|/Game/RollingWithThePunches/Blueprints/PlayerCharaacters/BP_FirstPersonCharacter.BP_FirstPersonCharacter_C|GetCurrentCoins (Variables|Default|GetPlayerRef)) (Variables|Default|GetCoinsRequired))
    (Variables|/Game/RollingWithThePunches/Blueprints/PlayerCharaacters/BP_FirstPersonCharacter.BP_FirstPersonCharacter_C|SetCurrentCoins _playerref (- (Variables|/Game/RollingWithThePunches/Blueprints/PlayerCharaacters/BP_FirstPersonCharacter.BP_FirstPersonCharacter_C|GetCurrentCoins _playerref) (Variables|Default|GetCoinsRequired)))
    (CallFunction|ActivatePaidButton)
    (else
      (bind _returnvalue (UserInterface|CreateWidget "/Game/RollingWithThePunches/Blueprints/HUDs/Effect_HUDs/Notifications/NotEnoughCoinsNotification_HUD.NotEnoughCoinsNotification_HUD_C"))
      (if (not (UserInterface|Viewport|IsinViewport _returnvalue))
        (UserInterface|Viewport|AddtoViewport _returnvalue 0)))))

(event Custom|ActivatePaidButton
  (CallFunction|CheckButtonLogic))

(event Custom|CheckButtonLogic
  (if (Variables|Default|GetTimed?)
    (CallFunction|ActivateTimedButton)
    (elif (Variables|Default|GetReactivatable?)
      (CallFunction|ActivateReactivatableButton)
      (else
        (CallFunction|ActivateSingleButton)))))

(event Custom|ActivateEnergizedButton
  (if (Variables|Default|GetEnergized?)
    (CallFunction|CheckButtonLogic)
    (else
      (bind _returnvalue (UserInterface|CreateWidget "/Game/RollingWithThePunches/Blueprints/HUDs/Effect_HUDs/Notifications/NeedsToBeChargedHUD.NeedsToBeChargedHUD_C"))
      (if (not (UserInterface|Viewport|IsinViewport _returnvalue))
        (UserInterface|Viewport|AddtoViewport _returnvalue 0)))))

(event EventBeginPlay
  (|CallParentFunction)
  (Utilities|FlowControl|Sequence
    (:then_0
      (bind _asbp_first_person_character (Utilities|Casting|CastToBP_FirstPersonCharacter (Game|Player|GetPlayerPawn 0)))
      (bind _output_get (Variables|Default|SetPlayerRef _asbp_first_person_character))
      (bind _asbp_arms (Utilities|Casting|CastToBP_Arms (Variables|/Script/Engine.ChildActorComponent|GetChildActor (Variables|/Game/RollingWithThePunches/Blueprints/PlayerCharaacters/BP_FirstPersonCharacter.BP_FirstPersonCharacter_C|GetArms _asbp_first_person_character))))
      (Variables|Default|SetArmRef _asbp_arms)
      (Variables|Default|SetPlayerStart (Transformation|GetActorLocation _output_get)))
    (:then_1
      (bind _asforce_required_hud (Utilities|Casting|CastToForceRequired_HUD (UserInterface|GetWidget (Variables|Default|GetWidget))))
      (Variables|/Game/RollingWithThePunches/Blueprints/HUDs/Effect_HUDs/ForceRequired_HUD.ForceRequired_HUD_C|SetForceRequired _asforce_required_hud (Variables|Default|GetForceRequired)))))

(event EventTick
  (params (DeltaSeconds :type Float%20%28single-precision%29))
  (CallFunction|CountDown))

(event EventDeactivate
  (|CallParentFunction))

(event EventActivate
  (bind _buttonalpha (Timeline|WarpTimeline Play)
    (:Update
      (Transformation|SetRelativeLocation (Variables|Default|GetButton) (Math|Vector|Lerp(Vector) "0,20.000000,0.000000" "0, 0, 0" _buttonalpha) false false)
      (Audio|PlaySoundatLocation "/Game/Interface_And_Item_Sounds/WAV/Special_Musical_04.Special_Musical_04" (Transformation|GetActorLocation) "0, 0, 0" 1.0 1.0 0.0 0 0 0 0)
      (Transformation|SetActorLocation (Variables|Default|GetPlayerRef) (Variables|Default|GetPlayerStart) false true))))

(event Game|Damage|EventAnyDamage
  (params (Damage :type Float%20%28single-precision%29) (DamageType :type Damage%20Type%20Object%20Reference) (InstigatedBy :type Controller%20Object%20Reference) (DamageCauser :type Actor%20Object%20Reference))
  (Utilities|Casting|CastToBP_DamageArms DamageType
    (:then
      (if (Variables|Default|GetbCanBeDamaged)
        (if (>= (Variables|/Game/RollingWithThePunches/Blueprints/Actors/Arm/BP_Arms.BP_Arms_C|GetForceUnleashed (Variables|Default|GetArmRef)) (Variables|Default|GetForceRequired))
          (Audio|PlaySoundatLocation "/Game/Interface_And_Item_Sounds/WAV/Flick_Switch_01.Flick_Switch_01" (Transformation|GetActorLocation) "0, 0, 0" 1.0 1.0 0.0 0 0 0 0)
          (Audio|PlaySoundatLocation "/Game/Interface_And_Item_Sounds/WAV/Coins_06.Coins_06" (Transformation|GetActorLocation) "0, 0, 0" 1.0 1.0 0.0 0 0 0 0)
          (Utilities|FlowControl|DoOnce false :!label _label
            (:Completed
              (CallFunction|Activate)
              (Utilities|FlowControl|Delay 1.0)
              (goto _label Reset)))
          (else
            (Audio|PlaySoundatLocation "/Game/Interface_And_Item_Sounds/WAV/Error_Buzz_05.Error_Buzz_05" (Transformation|GetActorLocation) "0, 0, 0" 1.0 1.0 0.0 0 0 0 0)))))
    (:CastFailed
      (Utilities|Casting|CastToBP_DamageProjectile DamageType))))

(fn ConstructionScript
  (|CallParentFunction))