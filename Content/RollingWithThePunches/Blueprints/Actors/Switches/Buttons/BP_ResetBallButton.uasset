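; Damage-triggered button that resets every boulder in the level at the cost of a 60-second time penalty and an added retry.
; A timeline animates the press and calls the boulder reset on each update, while DoOnce gates with delayed resets limit repeat triggering.
; The button is hidden unless marked Default or the player has checkpoints on.
; An overlap box shows its widget when the player is near.
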(event OnComponentBeginOverlap(Box)
  (params (OverlappedComponent :type Primitive%20Component%20Object%20Reference) (OtherActor :type Actor%20Object%20Reference) (OtherComp :type Primitive%20Component%20Object%20Reference) (OtherBodyIndex :type Integer) (bFromSweep :type Boolean) (SweepResult :type Hit%20Result%20Structure%20%28by%20ref%29))
  (if (== OtherActor (Variables|Default|GetPlayerRef))
    (Rendering|SetVisibility (Variables|Default|GetWidget) true false)))

(event OnComponentEndOverlap(Box)
  (params (OverlappedComponent :type Primitive%20Component%20Object%20Reference) (OtherActor :type Actor%20Object%20Reference) (OtherComp :type Primitive%20Component%20Object%20Reference) (OtherBodyIndex :type Integer))
  (if (== OtherActor (Variables|Default|GetPlayerRef))
    (Rendering|SetVisibility (Variables|Default|GetWidget) false false)))

(event Custom|SetBallLocation
  (bind _outactors (Actor|GetAllActorsOfClass "/Game/RollingWithThePunches/Blueprints/Actors/Boulders/BP_BoulderParent.BP_BoulderParent_C"))
  (for _array_element _outactors
    (Default|ResetBoulder _array_element)))

(event Custom|IncreasePlayerTime
  (bind _playerref (Variables|Default|GetPlayerRef))
  (Variables|/Game/RollingWithThePunches/Blueprints/PlayerCharaacters/BP_FirstPersonCharacter.BP_FirstPersonCharacter_C|SetLevelTime _playerref (+ (Variables|/Game/RollingWithThePunches/Blueprints/PlayerCharaacters/BP_FirstPersonCharacter.BP_FirstPersonCharacter_C|GetLevelTime _playerref) 6e+01))
  (bind _returnvalue (UserInterface|CreateWidget "/Game/RollingWithThePunches/Blueprints/HUDs/Effect_HUDs/ResetActive_HUD.ResetActive_HUD_C"))
  (UserInterface|Viewport|AddtoViewport _returnvalue 0))

(event Custom|IncreaseRetries
  (bind _playerref (Variables|Default|GetPlayerRef))
  (Variables|/Game/RollingWithThePunches/Blueprints/PlayerCharaacters/BP_FirstPersonCharacter.BP_FirstPersonCharacter_C|SetNumberOfRetries _playerref (+ (Variables|/Game/RollingWithThePunches/Blueprints/PlayerCharaacters/BP_FirstPersonCharacter.BP_FirstPersonCharacter_C|GetNumberOfRetries _playerref) 1)))

(event EventBeginPlay
  (Utilities|FlowControl|Sequence
    (:then_0
      (bind _asbp_first_person_character (Utilities|Casting|CastToBP_FirstPersonCharacter (Game|GetPlayerCharacter 0)))
      (bind _output_get (Variables|Default|SetPlayerRef _asbp_first_person_character))
      (Variables|Default|SetCheckpointOn? (Variables|/Game/RollingWithThePunches/Blueprints/PlayerCharaacters/BP_FirstPersonCharacter.BP_FirstPersonCharacter_C|GetCheckpointsOn? _output_get)))
    (:then_1
      (CallFunction|SetVisibility))))

(event Game|Damage|EventAnyDamage
  (params (Damage :type Float%20%28single-precision%29) (DamageType :type Damage%20Type%20Object%20Reference) (InstigatedBy :type Controller%20Object%20Reference) (DamageCauser :type Actor%20Object%20Reference))
  (Utilities|FlowControl|DoOnce false :!label _label
    (:Completed
      (Audio|PlaySoundatLocation "/Game/Interface_And_Item_Sounds/WAV/Flick_Switch_01.Flick_Switch_01" (Transformation|GetActorLocation) "0, 0, 0" 1.0 1.0 0.0 0 0 0 0)
      (Audio|PlaySoundatLocation "/Game/Interface_And_Item_Sounds/WAV/Coins_06.Coins_06" (Transformation|GetActorLocation) "0, 0, 0" 1.0 1.0 0.0 0 0 0 0)
      (bind _buttonalpha (Timeline|ActivateButton PlayFromStart)
        (:Update
          (Transformation|SetRelativeLocation (Variables|Default|GetButton) (Math|Vector|Lerp(Vector) "0,20.000000,0.000000" "0, 0, 0" _buttonalpha) false false)
          (CallFunction|SetBallLocation)
          (Utilities|FlowControl|Sequence
            (:then_0
              (Utilities|FlowControl|DoOnce false :!label _label_2
                (:Completed
                  (Audio|PlaySoundatLocation "/Game/RollingWithThePunches/Assets/Sounds/HUD_SFX/DJ_Laugh.DJ_Laugh" (Transformation|GetActorLocation) "0, 0, 0" 1.0 1.0 0.0 0 0 0 0)
                  (CallFunction|IncreasePlayerTime)
                  (CallFunction|IncreaseRetries)
                  (Utilities|FlowControl|Delay 3.0)
                  (goto _label_2 Reset))))
            (:then_1
              (Utilities|FlowControl|DoOnce false
                (:Completed
                  (Variables|/Game/RollingWithThePunches/Blueprints/PlayerCharaacters/BP_FirstPersonCharacter.BP_FirstPersonCharacter_C|SetBallReset? (Variables|Default|GetPlayerRef) true))))
            (:then_2
              (Utilities|FlowControl|Delay 3.0)
              (goto _label Reset))))))))

(fn ConstructionScript)

(fn SetVisibility
  (if (Variables|Default|GetDefault?)
    (Rendering|SetActorHiddenInGame false)
    (else
      (bind _output_get (Variables|Default|SetCheckpointOn? (Variables|/Game/RollingWithThePunches/Blueprints/PlayerCharaacters/BP_FirstPersonCharacter.BP_FirstPersonCharacter_C|GetCheckpointsOn? (Variables|Default|GetPlayerRef))))
      (if _output_get
        (Rendering|SetActorHiddenInGame false)
        (else
          (Rendering|SetActorHiddenInGame true))))))