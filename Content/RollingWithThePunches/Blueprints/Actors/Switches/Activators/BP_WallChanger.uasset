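; BP_WallChanger is a switch-activated actor that resizes its cube between a default and an altered scale.
; BeginAction plays a timeline that lerps the Scene component's scale, and ResetAction reverses it.
; The construction script applies the default scale and material and configures four decals' visibility and size.
; The timeline's water naming and disconnected InWater logic for player and boulders appear left over from a water-level actor, as overlap events do nothing.
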(event OnComponentBeginOverlap(Cube)
  (params (OverlappedComponent :type Primitive%20Component%20Object%20Reference) (OtherActor :type Actor%20Object%20Reference) (OtherComp :type Primitive%20Component%20Object%20Reference) (OtherBodyIndex :type Integer) (bFromSweep :type Boolean) (SweepResult :type Hit%20Result%20Structure%20%28by%20ref%29)))

(event OnComponentEndOverlap(Cube)
  (params (OverlappedComponent :type Primitive%20Component%20Object%20Reference) (OtherActor :type Actor%20Object%20Reference) (OtherComp :type Primitive%20Component%20Object%20Reference) (OtherBodyIndex :type Integer)))

(event EventBeginPlay
  (Transformation|SetRelativeScale3D (Variables|Default|GetScene) (Variables|Default|GetDefault%20Scale))
  (Variables|Default|SetDefautlMaterial (Rendering|Material|GetMaterial (Variables|Default|GetCube) 0))
  (Variables|Default|SetCurrentScale (Variables|/Script/Engine.SceneComponent|GetRelativeScale3D (Variables|Default|GetScene))))

(event Collision|EventActorBeginOverlap
  (params (OtherActor :type Actor%20Object%20Reference)))

(event EventTick
  (params (DeltaSeconds :type Float%20%28single-precision%29)))

(event EventBeginAction
  (|CallParentFunction)
  (bind _wateralpha (Timeline|AdjustWaterLevel Play)
    (:Update
      (Transformation|SetRelativeScale3D (Variables|Default|GetScene) (Math|Vector|Lerp(Vector) (Variables|Default|GetDefault%20Scale) (Variables|Default|GetAlteredScale) _wateralpha)))))

(event EventResetAction
  (|CallParentFunction)
  (bind _wateralpha (Timeline|AdjustWaterLevel Reverse)
    (:Update
      (Transformation|SetRelativeScale3D (Variables|Default|GetScene) (Math|Vector|Lerp(Vector) (Variables|Default|GetDefault%20Scale) (Variables|Default|GetAlteredScale) _wateralpha)))))

(fn ConstructionScript
  (|CallParentFunction)
  (Utilities|FlowControl|Sequence
    (:then_0
      (Transformation|SetRelativeScale3D (Variables|Default|GetScene) (Variables|Default|GetDefault%20Scale))
      (Rendering|Material|SetMaterial (Variables|Default|GetCube) 0 (Variables|Default|GetDefautlMaterial)))
    (:then_1
      (Rendering|SetVisibility (Variables|Default|GetDecal0) (Variables|Default|GetDecal%200Visible?) false)
      (Rendering|SetVisibility (Variables|Default|GetDecal1) (Variables|Default|GetDecal%201Visible?) false)
      (Rendering|SetVisibility (Variables|Default|GetDecal2) (Variables|Default|GetDecal%202Visible?) false)
      (Rendering|SetVisibility (Variables|Default|GetDecal3) (Variables|Default|GetDecal%203Visible?) false)
      (Transformation|SetRelativeScale3D (Variables|Default|GetDecal0) (Variables|Default|GetDecalSizes))
      (Transformation|SetRelativeScale3D (Variables|Default|GetDecal1) (Variables|Default|GetDecalSizes))
      (Transformation|SetRelativeScale3D (Variables|Default|GetDecal2) (Variables|Default|GetDecalSizes))
      (Transformation|SetRelativeScale3D (Variables|Default|GetDecal3) (Variables|Default|GetDecalSizes)))))