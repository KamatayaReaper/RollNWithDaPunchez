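; BP_BallRespawn is a switch activator that keeps a boulder spawned at its location and replaces it when activated.
; On BeginPlay it spawns a BP_BoulderParent at the actor's location and stores it in SpawnedBall.
; BeginAction calls the parent implementation, destroys the stored boulder without a validity check, then spawns and stores a fresh one at the same location.
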(event EventBeginPlay
  (bind _returnvalue (Game|SpawnActorfromClass "/Game/RollingWithThePunches/Blueprints/Actors/Boulders/BP_BoulderParent.BP_BoulderParent_C" (Math|Transform|MakeTransform (Transformation|GetActorLocation) "0, 0, 0" "1.000000,1.000000,1.000000") "Undefined" 0 0))
  (Variables|Default|SetSpawnedBall _returnvalue))

(event EventBeginAction
  (|CallParentFunction)
  (Actor|DestroyActor (Variables|Default|GetSpawnedBall))
  (bind _returnvalue (Game|SpawnActorfromClass "/Game/RollingWithThePunches/Blueprints/Actors/Boulders/BP_BoulderParent.BP_BoulderParent_C" (Math|Transform|MakeTransform (Transformation|GetActorLocation) "0, 0, 0" "1.000000,1.000000,1.000000") "Undefined" 0 0))
  (Variables|Default|SetSpawnedBall _returnvalue))

(fn ConstructionScript
  (|CallParentFunction))