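; BP_SlidingDoor is a switch-activated door that lowers out of the way and can return when reset.
; BeginAction and ResetAction extend parent events, each playing a sliding sound and driving the LowerDoor timeline forward or in reverse.
; The timeline lerps the Cube's relative location straight down without sweeping, while the construction script applies DecalSize to the decal's scale.
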(event EventBeginAction
  (|CallParentFunction)
  (Audio|PlaySoundatLocation "/Game/RollingWithThePunches/Assets/Sounds/SlidingDoor.SlidingDoor" (Transformation|GetActorLocation) "0, 0, 0" 1.0 1.0 0.0 0 0 0 0)
  (bind _movealpha (Timeline|LowerDoor Play)
    (:Update
      (Transformation|SetRelativeLocation (Variables|Default|GetCube) (Math|Vector|Lerp(Vector) "0, 0, 0" "0, 0,-500.000000" _movealpha) false false))))

(event EventResetAction
  (|CallParentFunction)
  (Audio|PlaySoundatLocation "/Game/RollingWithThePunches/Assets/Sounds/SlidingDoor.SlidingDoor" (Transformation|GetActorLocation) "0, 0, 0" 1.0 1.0 0.0 0 0 0 0)
  (bind _movealpha (Timeline|LowerDoor Reverse)
    (:Update
      (Transformation|SetRelativeLocation (Variables|Default|GetCube) (Math|Vector|Lerp(Vector) "0, 0, 0" "0, 0,-500.000000" _movealpha) false false))))

(fn ConstructionScript
  (|CallParentFunction)
  (Transformation|SetRelativeScale3D (Variables|Default|GetDecal) (Variables|Default|GetDecalSize)))