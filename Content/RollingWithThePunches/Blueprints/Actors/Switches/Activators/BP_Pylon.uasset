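; Electric pylon that relays charge to other electrical devices along up to four toggleable directions and can be rotated.
; While active, a looping timer line-traces each enabled direction and activates hit actors implementing BPI_Electricity.
; Incoming charge activates it through a DoOnce, and a retriggerable delay shuts it off one second after charging stops.
; A timeline yaws it by RotationFactor, either cumulatively or back and forth when FlipFlops is set.
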(event Custom|ShootElectricity
  (Utilities|FlowControl|Sequence
    (:then_0
      (CallFunction|ShootDirection0))
    (:then_1
      (CallFunction|ShootDirection1))
    (:then_2
      (CallFunction|ShootDirection2))
    (:then_3
      (CallFunction|ShootDirection3))))

(event Custom|DeactivatePylon
  (Rendering|Material|SetMaterial (Variables|Default|GetSphere) 0 "/Game/RollingWithThePunches/Blockmesh/Materials/Solid_Colors/Solid_LightBlue.Solid_LightBlue")
  (Utilities|Time|ClearandInvalidateTimerbyHandle (Variables|Default|GetPylonTimer)))

(event Custom|SetNewRotation
  (Variables|ElectricalDirection|SetCurrentRotation (Transformation|GetActorRotation)))

(event Custom|ActivatePylon
  (Rendering|Material|SetMaterial (Variables|Default|GetSphere) 0 "/Game/RollingWithThePunches/Assets/Material/Emissive/E_LightBlue.E_LightBlue")
  (bind _returnvalue (Utilities|Time|SetTimerbyEvent (delegate Custom|ShootElectricity) 0.02 true))
  (Variables|Default|SetPylonTimer _returnvalue))

(event Custom|ShootDirection3
  (bind _electritydirection3 (Variables|Default|GetElectrityDirection3))
  (bind _returnvalue (Transformation|GetWorldLocation _electritydirection3))
  (if (Variables|ElectricalDirection|GetDirection3Active?)
    (bind _outhit (Collision|LineTraceByChannel _returnvalue (+ _returnvalue (* (Math|Vector|GetForwardVector (Transformation|GetWorldRotation _electritydirection3)) 5e+03)) "TraceTypeQuery1" false 0 "ForOneFrame"))
    (CallFunction|CheckforHit _outhit)))

(event Custom|ShootDirection2
  (bind _electritydirection2 (Variables|Default|GetElectrityDirection2))
  (bind _returnvalue (Transformation|GetWorldLocation _electritydirection2))
  (if (Variables|ElectricalDirection|GetDirection2Active?)
    (bind _outhit (Collision|LineTraceByChannel _returnvalue (+ _returnvalue (* (Math|Vector|GetForwardVector (Transformation|GetWorldRotation _electritydirection2)) 5e+03)) "TraceTypeQuery1" false 0 "ForOneFrame"))
    (CallFunction|CheckforHit _outhit)))

(event Custom|ShootDirection0
  (bind _electritydirection0 (Variables|Default|GetElectrityDirection0))
  (bind _returnvalue (Transformation|GetWorldLocation _electritydirection0))
  (if (Variables|ElectricalDirection|GetDirection0Active?)
    (bind _outhit (Collision|LineTraceByChannel _returnvalue (+ _returnvalue (* (Math|Vector|GetForwardVector (Transformation|GetWorldRotation _electritydirection0)) 5e+03)) "TraceTypeQuery1" false 0 "ForOneFrame"))
    (CallFunction|CheckforHit _outhit)))

(event Custom|ShootDirection1
  (bind _electritydirection1 (Variables|Default|GetElectrityDirection1))
  (bind _returnvalue (Transformation|GetWorldLocation _electritydirection1))
  (if (Variables|ElectricalDirection|GetDirection1Active?)
    (bind _outhit (Collision|LineTraceByChannel _returnvalue (+ _returnvalue (* (Math|Vector|GetForwardVector (Transformation|GetWorldRotation _electritydirection1)) 5e+03)) "TraceTypeQuery1" false 0 "ForOneFrame"))
    (CallFunction|CheckforHit _outhit)))

(event EventBeginPlay
  (CallFunction|SetNewRotation)
  (if (Variables|Default|GetIsCharged?)
    (CallFunction|ActivatePylon)))

(event EventBeginAction
  (|CallParentFunction)
  (if (Variables|Default|GetIsCharged?)
    _))

(event EventActivateElectricalDevice
  (Utilities|FlowControl|Sequence
    (:then_0
      (Variables|Default|SetIsCharged? true)
      (Utilities|FlowControl|DoOnce false :!label _label
        (:Completed
          (CallFunction|ActivatePylon))))
    (:then_1
      (Utilities|FlowControl|RetriggerableDelay 1.0)
      (Variables|Default|SetIsCharged? false)
      (CallFunction|DeactivatePylon)
      (goto _label Reset))))

(event EventRotateElectricalDevice
  (bind _currentrotation (Variables|ElectricalDirection|GetCurrentRotation))
  (bind (_roll _pitch _yaw) (Math|Rotator|BreakRotator _currentrotation))
  (if (not (Variables|ElectricalDirection|GetFlipFlops?))
    (bind _rotatealpha (Timeline|RotatePylonTimeline PlayFromStart)
      (:Update
        (Transformation|SetActorRotation (Math|Rotator|Lerp(Rotator) (Variables|ElectricalDirection|GetCurrentRotation) (Math|Rotator|MakeRotator _roll _pitch (+ _yaw (Variables|ElectricalDirection|GetRotationFactor))) _rotatealpha)))
      (:Finished
        (CallFunction|SetNewRotation)))
    (else
      (Utilities|FlowControl|FlipFlop
        (:A
          (Timeline|RotatePylonTimeline PlayFromStart))
        (:B
          (Timeline|RotatePylonTimeline ReverseFromEnd))))))

(fn ConstructionScript
  (|CallParentFunction))

(fn CheckforHit
  (params (Hit :type Hit%20Result%20Structure%20%28by%20ref%29))
  (bind (_bblockinghit _binitialoverlap _time _distance _location _impactpoint _normal _impactnormal _physmat _hitactor) (Collision|BreakHitResult Hit))
  (if _bblockinghit
    (if (Utilities|DoesObjectImplementInterface _hitactor "/Game/RollingWithThePunches/Blueprints/Interface/BPI_Electricity.BPI_Electricity_C")
      (Class|BPIElectricity|ActivateElectricalDevice(Message) _hitactor))))