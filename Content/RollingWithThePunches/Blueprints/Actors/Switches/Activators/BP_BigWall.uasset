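; BP_BigWall is a switch-activated wall that slides between two points when its action begins and returns when reset.
; It extends a parent activator's begin and reset actions, playing or reversing the MoveWall timeline.
; The timeline's alpha interpolates the Cube's relative location between PointA and PointB without sweeping.
; The construction script scales the Cube to the WallSize variable.
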(event EventBeginPlay)

(event Collision|EventActorBeginOverlap
  (params (OtherActor :type Actor%20Object%20Reference)))

(event EventTick
  (params (DeltaSeconds :type Float%20%28single-precision%29)))

(event EventBeginAction
  (|CallParentFunction)
  (bind _movealpha (Timeline|MoveWall Play)
    (:Update
      (Transformation|SetRelativeLocation (Variables|Default|GetCube) (Math|Vector|Lerp(Vector) (Variables|Default|GetPointA) (Variables|Default|GetPointB) _movealpha) false false))))

(event EventResetAction
  (|CallParentFunction)
  (bind _movealpha (Timeline|MoveWall Reverse)
    (:Update
      (Transformation|SetRelativeLocation (Variables|Default|GetCube) (Math|Vector|Lerp(Vector) (Variables|Default|GetPointA) (Variables|Default|GetPointB) _movealpha) false false))))

(fn ConstructionScript
  (|CallParentFunction)
  (Transformation|SetRelativeScale3D (Variables|Default|GetCube) (Variables|Default|GetWallSize)))