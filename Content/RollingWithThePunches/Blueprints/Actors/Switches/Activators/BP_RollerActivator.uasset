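; Switch-activated actor that drives a child BP_Roller, changing how fast and in which direction it spins.
; On BeginPlay it caches the roller and passes it the configured scale and base rotation rate.
; BeginAction plays a timeline that lerps the roller's RotatingMovement rate from base to active rotation, and ResetAction reverses it.
; The construction script applies RollerScale to the actor.
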(event Custom|SetRotation
  (bind _rotationalpha (Timeline|RotationTimeline Play)
    (:Update
      (Variables|/Script/Engine.RotatingMovementComponent|SetRotationRate (Variables|/Game/RollingWithThePunches/Blueprints/Actors/Obstacles/Spinners/BP_Roller.BP_Roller_C|GetRotatingMovement (Variables|Default|GetRollerRef)) (Math|Rotator|Lerp(Rotator) (Variables|Default|GetBaseRotation) (Variables|Default|GetActiveRotation) _rotationalpha)))))

(event Custom|ResetRotation
  (bind _rotationalpha (Timeline|RotationTimeline Reverse)
    (:Update
      (Variables|/Script/Engine.RotatingMovementComponent|SetRotationRate (Variables|/Game/RollingWithThePunches/Blueprints/Actors/Obstacles/Spinners/BP_Roller.BP_Roller_C|GetRotatingMovement (Variables|Default|GetRollerRef)) (Math|Rotator|Lerp(Rotator) (Variables|Default|GetBaseRotation) (Variables|Default|GetActiveRotation) _rotationalpha)))))

(event EventBeginPlay
  (bind _asbp_roller (Utilities|Casting|CastToBP_Roller (Variables|/Script/Engine.ChildActorComponent|GetChildActor (Variables|Default|GetRoller))))
  (Variables|Default|SetRollerRef _asbp_roller)
  (Variables|/Game/RollingWithThePunches/Blueprints/Actors/Obstacles/Spinners/BP_Roller.BP_Roller_C|SetRollerScale (Variables|Default|GetRollerRef) (Variables|Default|GetRoller%20Scale))
  (Variables|/Game/RollingWithThePunches/Blueprints/Actors/Obstacles/Spinners/BP_Roller.BP_Roller_C|SetRollerRotation (Variables|Default|GetRollerRef) (Variables|Default|GetBaseRotation))
  (Variables|/Script/Engine.RotatingMovementComponent|SetRotationRate (Variables|/Game/RollingWithThePunches/Blueprints/Actors/Obstacles/Spinners/BP_Roller.BP_Roller_C|GetRotatingMovement (Variables|Default|GetRollerRef)) (Variables|Default|GetBaseRotation)))

(event Collision|EventActorBeginOverlap
  (params (OtherActor :type Actor%20Object%20Reference)))

(event EventTick
  (params (DeltaSeconds :type Float%20%28single-precision%29)))

(event EventBeginAction
  (CallFunction|SetRotation))

(event EventResetAction
  (CallFunction|ResetRotation))

(fn ConstructionScript
  (|CallParentFunction)
  (Transformation|SetActorScale3D (Variables|Default|GetRoller%20Scale)))