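; Teleporter switch activator whose action performs an instant, non-swept teleport to the world location of its linked exit point.
; BeginAction runs the teleport once per actor overlapping its box, but as written moves the activator itself rather than those actors.
; BeginPlay caches the player and last boulder found, and capsule overlaps record a teleportee, though none are used here.
; The construction script scales the cylinder by TeleporterSize.
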(event OnComponentBeginOverlap(Capsule)
  (params (OverlappedComponent :type Primitive%20Component%20Object%20Reference) (OtherActor :type Actor%20Object%20Reference) (OtherComp :type Primitive%20Component%20Object%20Reference) (OtherBodyIndex :type Integer) (bFromSweep :type Boolean) (SweepResult :type Hit%20Result%20Structure%20%28by%20ref%29))
  (Variables|Default|SetCurrentTeleportee OtherActor))

(event EventBeginPlay
  (Utilities|FlowControl|Sequence
    (:then_0
      (bind _asbp_first_person_character (Utilities|Casting|CastToBP_FirstPersonCharacter (Game|GetPlayerCharacter 0)))
      (Variables|Default|SetPlayerRef _asbp_first_person_character))
    (:then_1
      (bind _outactors (Actor|GetAllActorsOfClass "/Game/RollingWithThePunches/Blueprints/Actors/Boulders/BP_BoulderParent.BP_BoulderParent_C"))
      (for _array_element _outactors
        (Variables|Default|SetCurrentBall _array_element)))))

(event Collision|EventActorBeginOverlap
  (params (OtherActor :type Actor%20Object%20Reference)))

(event EventTick
  (params (DeltaSeconds :type Float%20%28single-precision%29)))

(event EventBeginAction
  (|CallParentFunction)
  (for _array_element (Collision|GetOverlappingActors (Variables|Default|GetBox) 0 :!class /Script/Engine.PrimitiveComponent)
    (Transformation|SetActorLocation (Transformation|GetWorldLocation (Variables|BP_TeleporterActivator_C|GetScene (Variables|Default|GetExitPointRef))) false true)))

(fn ConstructionScript
  (|CallParentFunction)
  (Transformation|SetRelativeScale3D (Variables|Default|GetCylinder) (Variables|Default|GetTeleporterSize)))