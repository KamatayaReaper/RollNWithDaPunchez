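; Switch-activated magnet beacon that applies magnetic force to nearby physics objects and spins while active.
; A looping timer sphere-traces around MagnetPullPoint and applies impulses to simulating bodies along the beacon-to-object direction, scaled by MagneticForce.
; BeginAction and ResetAction both toggle MagnetOn, starting or stopping the spin and timer.
; Switching off also toggles physics simulation on bodies in range to halt them.
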(event Custom|PullObjects
  (bind _magnetpullpoint (Variables|Default|GetMagnetPullPoint))
  (bind _returnvalue (Transformation|GetWorldLocation _magnetpullpoint))
  (bind _outhits (Collision|MultiSphereTraceForObjects _returnvalue _returnvalue (Variables|Default|GetMagnetRadius) (Utilities|Array|MakeArray "ObjectTypeQuery4") false 0 "None"))
  (for _array_element _outhits
    (if (Physics|IsSimulatingPhysics (.HitComponent (Collision|BreakHitResult _array_element)) "None")
      (Physics|AddImpulseatLocation (.HitComponent (Collision|BreakHitResult _array_element)) (* (Math|Vector|Normalize (- (Transformation|GetActorLocation (.HitActor (Collision|BreakHitResult _array_element))) (Transformation|GetActorLocation))) (Variables|Default|GetMagneticForce)) (Math|Vector|Normalize (- (Transformation|GetActorLocation (.HitActor (Collision|BreakHitResult _array_element))) (Transformation|GetActorLocation))) "None"))))

(event Custom|InitateMagneticForce
  (Variables|/Script/Engine.RotatingMovementComponent|SetRotationRate (Variables|Default|GetRotatingMovement) "0,1080.000000, 0")
  (bind _returnvalue (Utilities|Time|SetTimerbyEvent (delegate Custom|PullObjects) 0.2 true))
  (Variables|Default|SetMagnetTimer _returnvalue))

(event Custom|StopMagneticForce
  (Variables|/Script/Engine.RotatingMovementComponent|SetRotationRate (Variables|Default|GetRotatingMovement) "0, 0, 0")
  (Utilities|Time|ClearandInvalidateTimerbyHandle (Variables|Default|GetMagnetTimer)))

(event Custom|StopObjects
  (bind _magnetpullpoint (Variables|Default|GetMagnetPullPoint))
  (bind _returnvalue (Transformation|GetWorldLocation _magnetpullpoint))
  (bind _outhits (Collision|MultiSphereTraceForObjects _returnvalue _returnvalue (Variables|Default|GetMagnetRadius) (Utilities|Array|MakeArray "ObjectTypeQuery4") false 0 "None"))
  (for _array_element _outhits
    (if (Physics|IsSimulatingPhysics (.HitComponent (Collision|BreakHitResult _array_element)) "None")
      (Physics|SetSimulatePhysics (.HitComponent (Collision|BreakHitResult _array_element)) false)
      (Physics|SetSimulatePhysics (.HitComponent (Collision|BreakHitResult _array_element)) true))))

(event Custom|SwitchMagnet
  (if (Variables|Default|GetMagnetOn?)
    (Variables|Default|SetMagnetOn? false)
    (CallFunction|StopMagneticForce)
    (CallFunction|StopObjects)
    (else
      (Variables|Default|SetMagnetOn? true)
      (CallFunction|InitateMagneticForce))))

(event EventBeginPlay
  (if (Variables|Default|GetMagnetOn?)
    (CallFunction|InitateMagneticForce)))

(event EventBeginAction
  (CallFunction|SwitchMagnet))

(event EventResetAction
  (CallFunction|SwitchMagnet))

(fn ConstructionScript
  (|CallParentFunction))