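; BP_TrapDoorTrigger is a switch activator that rotates a Cylinder component between two orientations, presumably as a trap door.
; BeginAction calls the parent, then plays a timeline whose FlipAlpha lerps the component's relative rotation from RotationA to RotationB.
; ResetAction calls the parent, then reverses the same timeline to rotate it back.
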(event EventResetAction
  (|CallParentFunction)
  (bind _flipalpha (Timeline|Timeline_0 Reverse)
    (:Update
      (Transformation|SetRelativeRotation (Variables|Default|GetCylinder) (Math|Rotator|Lerp(Rotator) (Variables|Default|GetRotationA) (Variables|Default|GetRotationB) _flipalpha) false false))))

(event EventBeginAction
  (|CallParentFunction)
  (bind _flipalpha (Timeline|Timeline_0 Play)
    (:Update
      (Transformation|SetRelativeRotation (Variables|Default|GetCylinder) (Math|Rotator|Lerp(Rotator) (Variables|Default|GetRotationA) (Variables|Default|GetRotationB) _flipalpha) false false))))

(fn ConstructionScript
  (|CallParentFunction))