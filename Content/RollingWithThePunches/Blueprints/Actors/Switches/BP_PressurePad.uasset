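; Pressure pad switch that activates while the number of overlaps on its Box reaches ActorsNeededToActivate.
; Each begin or end overlap updates the count and calls Activate or Deactivate, both extending the parent class's events.
; The PadMove timeline lowers the pad mesh from the start on every Activate and reverses on Deactivate.
; Sounds play only when the count exactly hits the threshold on activation or zero on deactivation.
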(event OnComponentBeginOverlap(Box)
  (params (OverlappedComponent :type Primitive%20Component%20Object%20Reference) (OtherActor :type Actor%20Object%20Reference) (OtherComp :type Primitive%20Component%20Object%20Reference) (OtherBodyIndex :type Integer) (bFromSweep :type Boolean) (SweepResult :type Hit%20Result%20Structure%20%28by%20ref%29))
  (Math|Integer|IncrementInt (Variables|Default|GetActorsOnPressurePad)
    (:%20%20
      (if (>= (Variables|Default|GetActorsOnPressurePad) (Variables|Default|GetActorsNeededToActivate))
        (CallFunction|Activate)
        (else
          (CallFunction|Deactivate))))))

(event OnComponentEndOverlap(Box)
  (params (OverlappedComponent :type Primitive%20Component%20Object%20Reference) (OtherActor :type Actor%20Object%20Reference) (OtherComp :type Primitive%20Component%20Object%20Reference) (OtherBodyIndex :type Integer))
  (Math|Integer|DecrementInt (Variables|Default|GetActorsOnPressurePad)
    (:%20%20
      (if (>= (Variables|Default|GetActorsOnPressurePad) (Variables|Default|GetActorsNeededToActivate))
        (CallFunction|Activate)
        (else
          (CallFunction|Deactivate))))))

(event Custom|ActivatePressurePadSoundEnter
  (if (== (Variables|Default|GetActorsOnPressurePad) (Variables|Default|GetActorsNeededToActivate))
    (Audio|PlaySoundatLocation "/Game/Interface_And_Item_Sounds/WAV/Flick_Switch_02.Flick_Switch_02" (Transformation|GetActorLocation) "0, 0, 0" 1.0 1.0 0.0 0 0 0 0)
    (Audio|PlaySoundatLocation "/Game/Interface_And_Item_Sounds/WAV/Coins_06.Coins_06" (Transformation|GetActorLocation) "0, 0, 0" 1.0 1.0 0.0 0 0 0 0)))

(event Custom|ActivatePressurePadSoundExit
  (if (== (Variables|Default|GetActorsOnPressurePad) 0)
    (Audio|PlaySoundatLocation "/Game/Interface_And_Item_Sounds/WAV/Flick_Switch_02.Flick_Switch_02" (Transformation|GetActorLocation) "0, 0, 0" 1.0 1.0 0.0 0 0 0 0)))

(event EventBeginPlay
  (|CallParentFunction)
  (Variables|Default|SetActorsOnPressurePad 0))

(event Collision|EventActorBeginOverlap
  (params (OtherActor :type Actor%20Object%20Reference)))

(event EventTick
  (params (DeltaSeconds :type Float%20%28single-precision%29)))

(event EventActivate
  (|CallParentFunction)
  (Utilities|FlowControl|Sequence
    (:then_0
      (bind _padalpha (Timeline|PadMove PlayFromStart)
        (:Update
          (Transformation|SetRelativeLocation (Variables|Default|GetPressurePad) (Math|Vector|Lerp(Vector) "0, 0, 0" "0, 0,-5.000000" _padalpha) false false))))
    (:then_1
      (CallFunction|ActivatePressurePadSoundEnter))))

(event EventDeactivate
  (|CallParentFunction)
  (Utilities|FlowControl|Sequence
    (:then_0
      (bind _padalpha (Timeline|PadMove Reverse)
        (:Update
          (Transformation|SetRelativeLocation (Variables|Default|GetPressurePad) (Math|Vector|Lerp(Vector) "0, 0, 0" "0, 0,-5.000000" _padalpha) false false))))
    (:then_1
      (CallFunction|ActivatePressurePadSoundExit))))

(fn ConstructionScript
  (|CallParentFunction))