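; BP_SwitchReciever is an electrical receiver that powers linked switches or activators while it keeps receiving charge.
; ActivateElectricalDevice charges once, either energizing SwitchRef entries or calling BeginAction on ActivatorRef entries, as the Switch flag selects, and swaps to an emissive-style material.
; A retriggerable delay acts as a hold timer, discharging targets, restoring the material and re-arming the DoOnce one second after the last activation.
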(event Custom|ChargeDevice
  (for _array_element (Variables|Default|GetSwitchRef)
    (Variables|/Game/RollingWithThePunches/Blueprints/Actors/Switches/BP_SwitchParent.BP_SwitchParent_C|SetEnergized? _array_element true)))

(event Custom|DischargeDevice
  (if (Variables|Default|GetSwitch?)
    (for _array_element (Variables|Default|GetSwitchRef)
      (Variables|/Game/RollingWithThePunches/Blueprints/Actors/Switches/BP_SwitchParent.BP_SwitchParent_C|SetEnergized? _array_element false))
    (else
      (CallFunction|DischargeActivator))))

(event Custom|ChargeActivator
  (Utilities|FlowControl|DoOnce false
    (:Completed
      (for _array_element (Variables|Default|GetActivatorRef)
        (Default|BeginAction _array_element)))))

(event Custom|DischargeActivator
  (for _array_element (Variables|Default|GetActivatorRef)
    (Default|ResetAction _array_element))
  (Utilities|FlowControl|DoOnce false) ; enters at Reset
)

(event EventBeginPlay)

(event Collision|EventActorBeginOverlap
  (params (OtherActor :type Actor%20Object%20Reference)))

(event EventTick
  (params (DeltaSeconds :type Float%20%28single-precision%29)))

(event EventActivateElectricalDevice
  (Utilities|FlowControl|Sequence
    (:then_0
      (Variables|Default|SetIsCharged? true)
      (Utilities|FlowControl|DoOnce false :!label _label
        (:Completed
          (if (Variables|Default|GetSwitch?)
            (CallFunction|ChargeDevice)
            (Rendering|Material|SetMaterial (Variables|Default|GetMesh) 0 "/Game/RollingWithThePunches/Assets/Material/Emissive/E_LightBlue.E_LightBlue")
            (else
              (CallFunction|ChargeActivator)
              (Rendering|Material|SetMaterial (Variables|Default|GetMesh) 0 "/Game/RollingWithThePunches/Assets/Material/Emissive/E_LightBlue.E_LightBlue"))))))
    (:then_1
      (Utilities|FlowControl|RetriggerableDelay 1.0)
      (Variables|Default|SetIsCharged? false)
      (CallFunction|DischargeDevice)
      (Rendering|Material|SetMaterial (Variables|Default|GetMesh) 0 "/Game/RollingWithThePunches/Blockmesh/Materials/Solid_Colors/Solid_LightBlue.Solid_LightBlue")
      (goto _label Reset))))

(fn ConstructionScript)