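; Base projectile actor that can be repelled in the direction the player is looking.
; On BeginPlay it caches the first-person player character, and ActivateProjectileAction passes its unleashed force to RepelProjectile.
; RepelProjectile sets velocity along the camera's forward vector, scaling initial speed by a multiple of that force and falling back to plain initial speed if the result is zero.
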(event EventBeginPlay
  (bind _asbp_first_person_character (Utilities|Casting|CastToBP_FirstPersonCharacter (Game|GetPlayerCharacter 0)))
  (Variables|Default|SetPlayerRef _asbp_first_person_character))

(event Collision|EventActorBeginOverlap
  (params (OtherActor :type Actor%20Object%20Reference)))

(event EventTick
  (params (DeltaSeconds :type Float%20%28single-precision%29)))

(event EventActivateProjectileAction
  (params (ForceUnleashed :type Integer) (PunchDirection :type Vector :default "0, 0, 0"))
  (CallFunction|RepelProjectile ForceUnleashed))

(fn ConstructionScript)

(fn RepelProjectile
  (params (InputPin :type Integer))
  (bind _output_get (Variables|/Script/Engine.MovementComponent|SetVelocity (Variables|Default|GetProjectileMovement) (* (Math|Vector|GetForwardVector (Transformation|GetWorldRotation (Variables|/Game/RollingWithThePunches/Blueprints/PlayerCharaacters/BP_FirstPersonCharacter.BP_FirstPersonCharacter_C|GetFirstPersonCamera (Variables|Default|GetPlayerRef)))) (* (Variables|/Script/Engine.ProjectileMovementComponent|GetInitialSpeed (Variables|Default|GetProjectileMovement)) (* InputPin 5)))))
  (if (Utilities|Operators|EqualEqual :A _output_get)
    (Variables|/Script/Engine.MovementComponent|SetVelocity (Variables|Default|GetProjectileMovement) (* (Math|Vector|GetForwardVector (Transformation|GetWorldRotation (Variables|/Game/RollingWithThePunches/Blueprints/PlayerCharaacters/BP_FirstPersonCharacter.BP_FirstPersonCharacter_C|GetFirstPersonCamera (Variables|Default|GetPlayerRef)))) (* (Variables|/Script/Engine.ProjectileMovementComponent|GetInitialSpeed (Variables|Default|GetProjectileMovement)) 1.0)))))