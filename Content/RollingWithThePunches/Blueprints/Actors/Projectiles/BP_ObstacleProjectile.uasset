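; BP_ObstacleProjectile is a projectile that damages and shoves physics-simulated objects it hits.
; On Hit with a simulating component, it applies damage, then once adds a horizontal impulse at its location, scaled by ProjectileForce, and destroys itself.
; BeginPlay caches the player character for the IdentifyTarget function, which is unfinished: its checks lead to no action and its damage and hide logic never runs.
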(event EventBeginPlay
  (bind _asbp_first_person_character (Utilities|Casting|CastToBP_FirstPersonCharacter (Game|GetPlayerCharacter 0)))
  (Variables|Default|SetPlayerRef _asbp_first_person_character))

(event Collision|EventActorBeginOverlap
  (params (OtherActor :type Actor%20Object%20Reference)))

(event EventTick
  (params (DeltaSeconds :type Float%20%28single-precision%29)))

(event Collision|EventHit
  (params (MyComp :type Primitive%20Component%20Object%20Reference) (Other :type Actor%20Object%20Reference) (OtherComp :type Primitive%20Component%20Object%20Reference) (bSelfMoved :type Boolean) (HitLocation :type Vector :default "0, 0, 0") (HitNormal :type Vector :default "0, 0, 0") (NormalImpulse :type Vector :default "0, 0, 0") (Hit :type Hit%20Result%20Structure%20%28by%20ref%29))
  (bind _impulsevector (Variables|Default|GetImpulseVector))
  (bind _projectileforce (Variables|Default|GetProjectileForce))
  (bind _returnvalue (* _impulsevector _projectileforce))
  (if (Physics|IsSimulatingPhysics OtherComp "None")
    (Game|Damage|ApplyDamage Other 1.0 0 self (Variables|Default|GetDamageType))
    (Utilities|FlowControl|DoOnce false
      (:Completed
        (Physics|AddImpulseatLocation OtherComp (Math|Vector|MakeVector (.x _returnvalue) (.y _returnvalue) 0.0) (Transformation|GetActorLocation) "None")
        (Actor|DestroyActor) ; Then destroy this projectile
      ))))

(fn ConstructionScript)

(fn IdentifyTarget
  (params (OverlappedActor :type Actor%20Object%20Reference))
  (if (not (or (== OverlappedActor (Variables|Default|GetPlayerRef)) (== OverlappedActor 0)))
    (if (== OverlappedActor "/Game/RollingWithThePunches/Blueprints/Actors/Boulders/BP_BoulderParent.BP_BoulderParent")
      _)))