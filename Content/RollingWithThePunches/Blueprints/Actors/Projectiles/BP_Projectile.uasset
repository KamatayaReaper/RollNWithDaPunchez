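; Projectile actor that damages and pushes physics-simulating components it hits, then destroys itself.
; On hit it applies damage and an impulse scaled from its velocity at its own location.
; Any overlap also destroys it after a short delay.
; BeginPlay caches the player and arms for IdentifyTarget to exclude, but that overlap check has no effect, as its damage and sphere-hiding nodes are disconnected.
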(event EventBeginPlay
  (bind _asbp_first_person_character (Utilities|Casting|CastToBP_FirstPersonCharacter (Game|GetPlayerCharacter 0)))
  (bind _output_get (Variables|Default|SetPlayerRef _asbp_first_person_character))
  (bind _asbp_arms (Utilities|Casting|CastToBP_Arms (Variables|/Script/Engine.ChildActorComponent|GetChildActor (Variables|/Game/RollingWithThePunches/Blueprints/PlayerCharaacters/BP_FirstPersonCharacter.BP_FirstPersonCharacter_C|GetArms _output_get))))
  (Variables|Default|SetArmsRef _asbp_arms))

(event Collision|EventActorBeginOverlap
  (params (OtherActor :type Actor%20Object%20Reference))
  (CallFunction|IdentifyTarget OtherActor)
  (Utilities|FlowControl|Delay 0.2)
  (Actor|DestroyActor))

(event EventTick
  (params (DeltaSeconds :type Float%20%28single-precision%29)))

(event Collision|EventHit
  (params (MyComp :type Primitive%20Component%20Object%20Reference) (Other :type Actor%20Object%20Reference) (OtherComp :type Primitive%20Component%20Object%20Reference) (bSelfMoved :type Boolean) (HitLocation :type Vector :default "0, 0, 0") (HitNormal :type Vector :default "0, 0, 0") (NormalImpulse :type Vector :default "0, 0, 0") (Hit :type Hit%20Result%20Structure%20%28by%20ref%29))
  (if (Physics|IsSimulatingPhysics OtherComp "None")
    (Game|Damage|ApplyDamage Other 1.0 0 self (Variables|Default|GetDamageType))
    (Physics|AddImpulseatLocation OtherComp (* (Transformation|GetVelocity) (Variables|Default|GetProjectileForce)) (Transformation|GetActorLocation) "None")
    (Actor|DestroyActor) ; Then destroy this projectile
  ))

(fn ConstructionScript)

(fn IdentifyTarget
  (params (OverlappedActor :type Actor%20Object%20Reference))
  (if (not (or (== OverlappedActor (Variables|Default|GetPlayerRef)) (== OverlappedActor (Variables|Default|GetArmsRef))))
    (if (== OverlappedActor "/Game/RollingWithThePunches/Blueprints/Actors/Boulders/BP_BoulderParent.BP_BoulderParent")
      _)))