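; BP_LevelStarter is an actor that loads the first streaming sub-level when play begins.
; BeginPlay caches the first-person player character, stopping if the cast fails, then calls LoadSubLevel.
; LoadSubLevel requests a blocking load with visibility after load, then calls itself again until the sub-level is both loaded and visible.
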(event Custom|LoadSubLevel
  (bind _firstsublevel (Variables|Default|GetFirstSubLevel))
  (bind _returnvalue (Class|GameplayStatics|GetStreamingLevel _firstsublevel))
  (Game|LoadStreamLevel(byName) _firstsublevel true true)
  (if (Class|LevelStreaming|IsLevelLoaded _returnvalue)
    (if (not (Class|LevelStreaming|IsLevelVisible _returnvalue))
      (CallFunction|LoadSubLevel))
    (else
      (CallFunction|LoadSubLevel))))

(event EventBeginPlay
  (bind _asbp_first_person_character (Utilities|Casting|CastToBP_FirstPersonCharacter (Game|GetPlayerCharacter 0)))
  (Variables|Default|SetPlayerRef _asbp_first_person_character)
  (CallFunction|LoadSubLevel))

(fn ConstructionScript)