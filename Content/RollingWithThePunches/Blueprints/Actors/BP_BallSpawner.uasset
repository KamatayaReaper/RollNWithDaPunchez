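; BP_BallSpawner is an actor that spawns the boulder at its SpawnRef location.
; On BeginPlay it caches the first-person player character, registers itself as that character's BallSpawnerRef, then spawns a BoulderClass instance after a short delay.
; SetBoulderType maps the player's boulder type enum to a face-themed boulder Blueprint class, but is not called within this Blueprint.
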(event Custom|SpawnBoulder
  (Game|SpawnActorfromClass (Variables|Default|GetBoulderClass) (Math|Transform|MakeTransform (Transformation|GetWorldLocation (Variables|Default|GetSpawnRef)) "0, 0, 0" "1.000000,1.000000,1.000000") "Undefined" 0 0))

(event EventBeginPlay
  (bind _asbp_first_person_character (Utilities|Casting|CastToBP_FirstPersonCharacter (Game|GetPlayerCharacter 0)))
  (bind _output_get (Variables|Default|SetPlayerRef _asbp_first_person_character))
  (Variables|/Game/RollingWithThePunches/Blueprints/PlayerCharaacters/BP_FirstPersonCharacter.BP_FirstPersonCharacter_C|SetBallSpawnerRef _output_get self)
  (Utilities|FlowControl|Delay 0.2)
  (CallFunction|SpawnBoulder))

(event Collision|EventActorBeginOverlap
  (params (OtherActor :type Actor%20Object%20Reference)))

(event EventTick
  (params (DeltaSeconds :type Float%20%28single-precision%29)))

(fn ConstructionScript)

(fn SetBoulderType
  (switch Utilities|FlowControl|Switch|SwitchonE_BoulderType (Variables|/Game/RollingWithThePunches/Blueprints/PlayerCharaacters/BP_FirstPersonCharacter.BP_FirstPersonCharacter_C|GetEN_BoulderType (Variables|Default|GetPlayerRef))
    (:NewEnumerator0
      (Variables|Default|SetBoulderClass "/Game/RollingWithThePunches/Blueprints/Actors/Boulders/BP_CrazyFace.BP_CrazyFace_C"))
    (:NewEnumerator1
      (Variables|Default|SetBoulderClass "/Game/RollingWithThePunches/Blueprints/Actors/Boulders/BP_WuvFace.BP_WuvFace_C"))
    (:NewEnumerator2
      (Variables|Default|SetBoulderClass "/Game/RollingWithThePunches/Blueprints/Actors/Boulders/BP_GrrFace.BP_GrrFace_C"))
    (:NewEnumerator3
      (Variables|Default|SetBoulderClass "/Game/RollingWithThePunches/Blueprints/Actors/Boulders/BP_DoomFace.BP_DoomFace_C"))
    (:NewEnumerator4
      (Variables|Default|SetBoulderClass "/Game/RollingWithThePunches/Blueprints/Actors/Boulders/BP_MunchFace.BP_MunchFace_C"))
    (:NewEnumerator5
      (Variables|Default|SetBoulderClass "/Game/RollingWithThePunches/Blueprints/Actors/Boulders/BP_JackedFace.BP_JackedFace_C"))
    (:NewEnumerator6
      (Variables|Default|SetBoulderClass "/Game/RollingWithThePunches/Blueprints/Actors/Boulders/BP_BabuFace.BP_BabuFace_C"))
    (:NewEnumerator7
      (Variables|Default|SetBoulderClass "/Game/RollingWithThePunches/Blueprints/Actors/Boulders/BP_DPressFace.BP_DPressFace_C"))
    (:NewEnumerator8
      (Variables|Default|SetBoulderClass "/Game/RollingWithThePunches/Blueprints/Actors/Boulders/BP_SmugFace.BP_SmugFace_C"))))