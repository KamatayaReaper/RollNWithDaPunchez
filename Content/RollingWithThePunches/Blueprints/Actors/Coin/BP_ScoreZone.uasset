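; BP_ScoreZone is a trigger volume that awards coins to the player when a boulder enters it.
; It caches the first-person player character on BeginPlay, then on overlap with any BP_BoulderParent adds ScoreValue coins to that character and plays a coin sound at its location.
; The construction script sizes the box from ScoreBoxExtent, so each placed zone can be shaped per instance.
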(event EventBeginPlay
  (bind _asbp_first_person_character (Utilities|Casting|CastToBP_FirstPersonCharacter (Game|GetPlayerCharacter 0)))
  (Variables|Default|SetPlayerRef _asbp_first_person_character))

(event Collision|EventActorBeginOverlap
  (params (OtherActor :type Actor%20Object%20Reference))
  (Utilities|Casting|CastToBP_BoulderParent OtherActor)
  (Default|AddCoins (Variables|Default|GetPlayerRef) (Variables|Default|GetScoreValue))
  (Audio|PlaySoundatLocation "/Game/Interface_And_Item_Sounds/WAV/Coins_02.Coins_02" (Transformation|GetActorLocation) "0, 0, 0" 1.0 1.0 0.0 0 0 0 0))

(event EventTick
  (params (DeltaSeconds :type Float%20%28single-precision%29)))

(fn ConstructionScript
  (Components|Box|SetBoxExtent (Variables|Default|GetBox) (Variables|Default|GetScoreBoxExtent) true))