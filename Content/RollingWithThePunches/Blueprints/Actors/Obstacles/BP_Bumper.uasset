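; BP_Bumper is an obstacle actor that launches physics-simulating objects that touch it and plays a squash-and-stretch animation.
; A capsule overlap calls InitateBumper, which ignores non-simulating components and otherwise triggers the animation and applies a LaunchVector impulse scaled by BumperForce.
; The ExpandBumper timeline scales the cylinder between its BeginPlay scale and a SqueezeScale multiple.
; The impulse's Location receives a normalized actor-to-bumper direction rather than a world position.
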(event OnComponentBeginOverlap(Capsule)
  (params (OverlappedComponent :type Primitive%20Component%20Object%20Reference) (OtherActor :type Actor%20Object%20Reference) (OtherComp :type Primitive%20Component%20Object%20Reference) (OtherBodyIndex :type Integer) (bFromSweep :type Boolean) (SweepResult :type Hit%20Result%20Structure%20%28by%20ref%29))
  (CallFunction|InitateBumper OtherActor OtherComp))

(event Custom|ActivateBumper
  (bind _expandalpha (Timeline|ExpandBumper PlayFromStart)
    (:Update
      (Transformation|SetRelativeScale3D (Variables|Default|GetCylinder) (Math|Vector|Lerp(Vector) (Variables|Default|GetBaseScale) (* (Variables|Default|GetBaseScale) (Variables|Default|GetSqueezeScale)) _expandalpha)))))

(event EventBeginPlay
  (Variables|Default|SetBaseScale (Variables|/Script/Engine.SceneComponent|GetRelativeScale3D (Variables|Default|GetCylinder))))

(fn ConstructionScript)

(fn InitateBumper
  (params (Actor :type Actor%20Object%20Reference) (ActorComponet :type Primitive%20Component%20Object%20Reference))
  (if (Physics|IsSimulatingPhysics ActorComponet "None")
    (CallFunction|ActivateBumper)
    (Physics|AddImpulseatLocation ActorComponet (* (Variables|Default|GetLaunchVector) (Variables|Default|GetBumperForce)) (Math|Vector|Normalize (- (Transformation|GetActorLocation) (Transformation|GetActorLocation Actor))) "None")))