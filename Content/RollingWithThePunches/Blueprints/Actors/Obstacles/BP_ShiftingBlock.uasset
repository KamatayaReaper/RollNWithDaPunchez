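; BP_ShiftingBlock is an obstacle block that repeatedly shifts between a default and an altered scale.
; After a short BeginPlay delay, ShiftBlock waits BlockIntervals, then a FlipFlop alternates playing and reversing the ShiftWall timeline, with WallSpeed setting its rate.
; Timeline updates lerp the Scene component's scale and call ShiftBlock again, sustaining the cycle through its Delay.
; The construction script applies the default scale and cube material.
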(event Custom|ShiftBlock
  (Utilities|FlowControl|Delay (Variables|Default|GetBlockIntervals))
  (Utilities|FlowControl|FlipFlop
    (:A
      (bind _wateralpha (Timeline|ShiftWall Play)
        (:Update
          (Transformation|SetRelativeScale3D (Variables|Default|GetScene) (Math|Vector|Lerp(Vector) (Variables|Default|GetDefault%20Scale) (Variables|Default|GetAltered%20Scale) _wateralpha))
          (CallFunction|ShiftBlock))))
    (:B
      (Timeline|ShiftWall Reverse))))

(event EventBeginPlay
  (Transformation|SetRelativeScale3D (Variables|Default|GetScene) (Variables|Default|GetDefault%20Scale))
  (Variables|Default|SetCurrentScale (Variables|/Script/Engine.SceneComponent|GetRelativeScale3D (Variables|Default|GetScene)))
  (Variables|Default|SetDefaultMaterial (Rendering|Material|GetMaterial (Variables|Default|GetCube) 0))
  (Utilities|FlowControl|Delay 0.2)
  (CallFunction|ShiftBlock))

(event Collision|EventActorBeginOverlap
  (params (OtherActor :type Actor%20Object%20Reference)))

(event EventTick
  (params (DeltaSeconds :type Float%20%28single-precision%29)))

(fn ConstructionScript
  (Transformation|SetRelativeScale3D (Variables|Default|GetScene) (Variables|Default|GetDefault%20Scale))
  (Rendering|Material|SetMaterial (Variables|Default|GetCube) 0 (Variables|Default|GetDefaultMaterial)))