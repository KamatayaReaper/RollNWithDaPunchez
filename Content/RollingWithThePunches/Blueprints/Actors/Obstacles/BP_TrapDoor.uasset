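; BP_TrapDoor is an obstacle actor that automatically swings between two rotations on a repeating five-second delay.
; A FlipFlop alternately plays and reverses the MoveTrapDoor timeline, whose FlipAlpha interpolates the Cylinder's relative rotation between TurnA and TurnB.
; The cycle starts on BeginPlay and re-arms itself by calling TriggerTrapDoor from every timeline update, relying on Delay ignoring calls while it is pending.
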(event Custom|TriggerTrapDoor
  (Utilities|FlowControl|Delay 5.0)
  (Utilities|FlowControl|FlipFlop
    (:A
      (bind _flipalpha (Timeline|MoveTrapDoor Play)
        (:Update
          (Transformation|SetRelativeRotation (Variables|Default|GetCylinder) (Math|Rotator|Lerp(Rotator) (Variables|Default|GetTurnA) (Variables|Default|GetTurnB) _flipalpha) false false)
          (CallFunction|TriggerTrapDoor))))
    (:B
      (Timeline|MoveTrapDoor Reverse))))

(event EventBeginPlay
  (CallFunction|TriggerTrapDoor))

(fn ConstructionScript)