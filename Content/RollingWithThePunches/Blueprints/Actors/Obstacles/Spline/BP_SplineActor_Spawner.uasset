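; BP_SplineActor_Spawner is an obstacle spawner that creates an actor of ObstacleClass for a spline path when play begins.
; SpawnActor places the obstacle at the referenced path's spline world transform and stores the reference.
; It then hands the obstacle the path, a back-reference to the spawner and the looping settings.
; Reset shares that setup chain, reapplying those values to the existing obstacle without respawning it.
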(event Custom|SpawnActor
  (bind _returnvalue (Game|SpawnActorfromClass (Variables|Default|GetObstacleClass) (Transformation|GetWorldTransform (Variables|/Game/RollingWithThePunches/Blueprints/Actors/Obstacles/Spline/BP_Spline.BP_Spline_C|GetSpline (Variables|Default|GetSplinePathRef))) "Undefined" 0 0))
  (bind _output_get (Variables|Default|SetObstacleRef _returnvalue))
  (Variables|/Game/RollingWithThePunches/Blueprints/Actors/Obstacles/Spline/BP_SplineObstacle_Parent.BP_SplineObstacle_Parent_C|SetSplinePathRef _output_get (Variables|Default|GetSplinePathRef))
  (bind _output_get_2 (Variables|/Game/RollingWithThePunches/Blueprints/Actors/Obstacles/Spline/BP_SplineObstacle_Parent.BP_SplineObstacle_Parent_C|SetSpawnerRef (Variables|Default|GetObstacleRef) self))
  (Utilities|IsValid _output_get_2
    (:Is%20Valid
      _)
    (:Is%20Not%20Valid
      _))
  (Variables|/Game/RollingWithThePunches/Blueprints/Actors/Obstacles/Spline/BP_SplineObstacle_Parent.BP_SplineObstacle_Parent_C|SetLoop? (Variables|Default|GetObstacleRef) (Variables|Default|GetLooping?))
  (Variables|/Game/RollingWithThePunches/Blueprints/Actors/Obstacles/Spline/BP_SplineObstacle_Parent.BP_SplineObstacle_Parent_C|SetLoopTime (Variables|Default|GetObstacleRef) (Variables|Default|GetLoopTime)))

(event Custom|Reset
  (Variables|/Game/RollingWithThePunches/Blueprints/Actors/Obstacles/Spline/BP_SplineObstacle_Parent.BP_SplineObstacle_Parent_C|SetSplinePathRef (stale Custom|SpawnActor _output_get) (Variables|Default|GetSplinePathRef))
  (bind _output_get (Variables|/Game/RollingWithThePunches/Blueprints/Actors/Obstacles/Spline/BP_SplineObstacle_Parent.BP_SplineObstacle_Parent_C|SetSpawnerRef (Variables|Default|GetObstacleRef) self))
  (Utilities|IsValid _output_get
    (:Is%20Valid
      _)
    (:Is%20Not%20Valid
      _))
  (Variables|/Game/RollingWithThePunches/Blueprints/Actors/Obstacles/Spline/BP_SplineObstacle_Parent.BP_SplineObstacle_Parent_C|SetLoop? (Variables|Default|GetObstacleRef) (Variables|Default|GetLooping?))
  (Variables|/Game/RollingWithThePunches/Blueprints/Actors/Obstacles/Spline/BP_SplineObstacle_Parent.BP_SplineObstacle_Parent_C|SetLoopTime (Variables|Default|GetObstacleRef) (Variables|Default|GetLoopTime)))

(event EventBeginPlay
  (CallFunction|SpawnActor))

(fn ConstructionScript)