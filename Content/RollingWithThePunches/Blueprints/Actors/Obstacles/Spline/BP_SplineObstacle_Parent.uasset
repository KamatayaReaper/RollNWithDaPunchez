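; Parent Blueprint for obstacles that travel along a referenced spline path.
; After brief BeginPlay delays and a spawner reset, a timeline scaled by LoopTime sets the actor's location and rotation by distance along the spline.
; When the timeline finishes, it restarts from the beginning if Loop is set.
; A reverse-play event exists but is not called here, and the construction script's mesh assignment is disconnected.
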(event Custom|MoveObjectForward
  (bind _splinepathref (Variables|Default|GetSplinePathRef))
  (bind _spline (Variables|/Game/RollingWithThePunches/Blueprints/Actors/Obstacles/Spline/BP_Spline.BP_Spline_C|GetSpline _splinepathref))
  (Components|Timeline|SetPlayRate (Variables|Default|GetMoveObject) (/ 1.0 (Variables|Default|GetLoopTime)))
  (bind _movealpha (Timeline|MoveObject PlayFromStart)
    (:Update
      (Transformation|SetActorLocationAndRotation (Spline|GetLocationatDistanceAlongSpline _spline (Math|Float|Lerp 0.0 (Spline|GetSplineLength _spline) _movealpha) "World") (Spline|GetRotationatDistanceAlongSpline _spline (Math|Float|Lerp 0.0 (Spline|GetSplineLength _spline) _movealpha) "World")))
    (:Finished
      (CallFunction|DecideNextAction))))

(event Custom|DecideNextAction
  (if (Variables|Default|GetLoop?)
    (CallFunction|MoveObjectForward)))

(event Custom|MoveObjectBackwards
  (bind _splinepathref (Variables|Default|GetSplinePathRef))
  (bind _spline (Variables|/Game/RollingWithThePunches/Blueprints/Actors/Obstacles/Spline/BP_Spline.BP_Spline_C|GetSpline _splinepathref))
  (bind _movealpha (Timeline|MoveObject ReverseFromEnd)
    (:Update
      (Transformation|SetActorLocationAndRotation (Spline|GetLocationatDistanceAlongSpline _spline (Math|Float|Lerp 0.0 (Spline|GetSplineLength _spline) _movealpha) "World") (Spline|GetRotationatDistanceAlongSpline _spline (Math|Float|Lerp 0.0 (Spline|GetSplineLength _spline) _movealpha) "World")))
    (:Finished
      (CallFunction|DecideNextAction))))

(event EventBeginPlay
  (Utilities|FlowControl|Delay 0.2)
  (Default|Reset (Variables|Default|GetSpawnerRef))
  (Utilities|FlowControl|Delay 0.2)
  (CallFunction|MoveObjectForward))

(event Collision|EventActorBeginOverlap
  (params (OtherActor :type Actor%20Object%20Reference)))

(event EventTick
  (params (DeltaSeconds :type Float%20%28single-precision%29)))

(fn ConstructionScript)