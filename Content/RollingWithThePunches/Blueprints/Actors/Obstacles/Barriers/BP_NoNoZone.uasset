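; BP_NoNoZone is a barrier obstacle that teleports the first-person player character to a safe spot when it touches the barrier.
; The construction script sizes the barrier mesh and places the TeleportPoint component from exposed variables.
; On BeginPlay a downward line trace from TeleportPoint finds the ground and stores the hit location as the destination.
; Overlapping the barrier mesh moves the character straight to that stored location.
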(event OnComponentBeginOverlap(BarrierMesh)
  (params (OverlappedComponent :type Primitive%20Component%20Object%20Reference) (OtherActor :type Actor%20Object%20Reference) (OtherComp :type Primitive%20Component%20Object%20Reference) (OtherBodyIndex :type Integer) (bFromSweep :type Boolean) (SweepResult :type Hit%20Result%20Structure%20%28by%20ref%29))
  (bind _asbp_first_person_character (Utilities|Casting|CastToBP_FirstPersonCharacter OtherActor))
  (Transformation|SetActorLocation _asbp_first_person_character (Variables|Default|GetSpawnLocation) false true))

(event EventBeginPlay
  (bind _teleportpoint (Variables|Default|GetTeleportPoint))
  (bind _returnvalue (Transformation|GetWorldLocation _teleportpoint))
  (bind (_outhit _returnvalue_2) (Collision|LineTraceByChannel _returnvalue (- _returnvalue "0,0,5000.000000") "TraceTypeQuery1" false 0 "None"))
  (if _returnvalue_2
    (Variables|Default|SetSpawnLocation (.Location (Collision|BreakHitResult _outhit)))))

(event EventTick
  (params (DeltaSeconds :type Float%20%28single-precision%29)))

(fn ConstructionScript
  (Utilities|FlowControl|Sequence
    (:then_0
      (Transformation|SetRelativeScale3D (Variables|Default|GetBarrierMesh) (Variables|Default|GetBarrierSize)))
    (:then_1
      (Transformation|SetRelativeLocation (Variables|Default|GetTeleportPoint) (Variables|Default|GetTeleporterLocation) false false))))