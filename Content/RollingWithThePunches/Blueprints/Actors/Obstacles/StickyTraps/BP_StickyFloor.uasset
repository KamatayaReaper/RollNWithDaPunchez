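; BP_StickyFloor is a sticky trap obstacle that briefly halts boulders entering its Box volume.
; On overlap by a BP_BoulderParent, it switches off physics simulation on the boulder's Sphere and restores it after a half-second delay.
; A DoOnce gate prevents repeated triggering and resets when a boulder leaves the box.
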(event OnComponentBeginOverlap(Box)
  (params (OverlappedComponent :type Primitive%20Component%20Object%20Reference) (OtherActor :type Actor%20Object%20Reference) (OtherComp :type Primitive%20Component%20Object%20Reference) (OtherBodyIndex :type Integer) (bFromSweep :type Boolean) (SweepResult :type Hit%20Result%20Structure%20%28by%20ref%29))
  (bind _asbp_boulder_parent (Utilities|Casting|CastToBP_BoulderParent OtherActor))
  (if (== _asbp_boulder_parent OtherActor)
    (Utilities|FlowControl|DoOnce false
      (:Completed
        (Physics|SetSimulatePhysics (Variables|/Game/RollingWithThePunches/Blueprints/Actors/Boulders/BP_BoulderParent.BP_BoulderParent_C|GetSphere _asbp_boulder_parent) false)
        (Utilities|FlowControl|Delay 0.5)
        (Physics|SetSimulatePhysics (Variables|/Game/RollingWithThePunches/Blueprints/Actors/Boulders/BP_BoulderParent.BP_BoulderParent_C|GetSphere _asbp_boulder_parent) true)))))

(event OnComponentEndOverlap(Box)
  (params (OverlappedComponent :type Primitive%20Component%20Object%20Reference) (OtherActor :type Actor%20Object%20Reference) (OtherComp :type Primitive%20Component%20Object%20Reference) (OtherBodyIndex :type Integer))
  (bind _asbp_boulder_parent (Utilities|Casting|CastToBP_BoulderParent OtherActor))
  (if (== _asbp_boulder_parent OtherActor)
    (Utilities|FlowControl|DoOnce false) ; enters at Reset
  ))

(fn ConstructionScript)