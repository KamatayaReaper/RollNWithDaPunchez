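; BP_StickyParent is a parent obstacle for sticky traps that briefly halts physics objects touching it.
; On overlap with a simulating component, it waits briefly, disables that component's physics, then re-enables it after a pause.
; A DoOnce gates the effect and resets when a simulating component leaves.
; The construction script sets mesh scale and collision box placement and extent from variables; older boulder-specific logic remains disconnected.
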(event OnComponentBeginOverlap(StickyCollision)
  (params (OverlappedComponent :type Primitive%20Component%20Object%20Reference) (OtherActor :type Actor%20Object%20Reference) (OtherComp :type Primitive%20Component%20Object%20Reference) (OtherBodyIndex :type Integer) (bFromSweep :type Boolean) (SweepResult :type Hit%20Result%20Structure%20%28by%20ref%29))
  (if (Class|SceneComponent|IsAnySimulatingPhysics OtherComp)
    (Utilities|FlowControl|DoOnce false
      (:Completed
        (Utilities|FlowControl|Delay 0.25)
        (Physics|SetSimulatePhysics OtherComp false)
        (Utilities|FlowControl|Delay 0.5)
        (Physics|SetSimulatePhysics OtherComp true)))))

(event OnComponentEndOverlap(StickyCollision)
  (params (OverlappedComponent :type Primitive%20Component%20Object%20Reference) (OtherActor :type Actor%20Object%20Reference) (OtherComp :type Primitive%20Component%20Object%20Reference) (OtherBodyIndex :type Integer))
  (if (Class|SceneComponent|IsAnySimulatingPhysics OtherComp)
    (Utilities|FlowControl|DoOnce false) ; enters at Reset
  ))

(fn ConstructionScript
  (Transformation|SetRelativeScale3D (Variables|Default|GetMesh) (Variables|Default|GetMeshScale))
  (Transformation|SetRelativeLocation (Variables|Default|GetStickyCollision) (Variables|Default|GetStickyLocation) false false)
  (Components|Box|SetBoxExtent (Variables|Default|GetStickyCollision) (Variables|Default|GetStickyCollisionExtent) true))