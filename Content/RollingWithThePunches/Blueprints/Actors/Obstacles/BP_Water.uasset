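; BP_Water is a water volume obstacle that can shift between a default and altered scale, affecting characters and boulders inside it.
; When ShiftWater is enabled, a delay and FlipFlop alternately play and reverse a timeline that lerps the scale, re-triggering the shift from its update.
; Overlaps set InWater on boulders and on characters via Submerge-tagged components, which also refresh audio filter and stats.
; Exiting boulders receive the scale cached at BeginPlay as WaterVolume.
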(event OnComponentBeginOverlap(Cube)
  (params (OverlappedComponent :type Primitive%20Component%20Object%20Reference) (OtherActor :type Actor%20Object%20Reference) (OtherComp :type Primitive%20Component%20Object%20Reference) (OtherBodyIndex :type Integer) (bFromSweep :type Boolean) (SweepResult :type Hit%20Result%20Structure%20%28by%20ref%29))
  (Utilities|FlowControl|Sequence
    (:then_0
      (if (Components|ComponentHasTag OtherComp "Submerge")
        (bind _asbp_first_person_character (Utilities|Casting|CastToBP_FirstPersonCharacter OtherActor))
        (Variables|/Game/RollingWithThePunches/Blueprints/PlayerCharaacters/BP_FirstPersonCharacter.BP_FirstPersonCharacter_C|SetInWater? _asbp_first_person_character true)
        (Default|SetWaterAudioFilter _asbp_first_person_character)
        (Default|AdjustStatstoWater _asbp_first_person_character)))
    (:then_1
      (bind _asbp_boulder_parent (Utilities|Casting|CastToBP_BoulderParent OtherActor))
      (Variables|/Game/RollingWithThePunches/Blueprints/Actors/Boulders/BP_BoulderParent.BP_BoulderParent_C|SetInWater _asbp_boulder_parent true))))

(event OnComponentEndOverlap(Cube)
  (params (OverlappedComponent :type Primitive%20Component%20Object%20Reference) (OtherActor :type Actor%20Object%20Reference) (OtherComp :type Primitive%20Component%20Object%20Reference) (OtherBodyIndex :type Integer))
  (Utilities|FlowControl|Sequence
    (:then_0
      (if (Components|ComponentHasTag OtherComp "Submerge")
        (bind _asbp_first_person_character (Utilities|Casting|CastToBP_FirstPersonCharacter OtherActor))
        (Variables|/Game/RollingWithThePunches/Blueprints/PlayerCharaacters/BP_FirstPersonCharacter.BP_FirstPersonCharacter_C|SetInWater? _asbp_first_person_character false)
        (Default|SetWaterAudioFilter _asbp_first_person_character)
        (Default|AdjustStatstoWater _asbp_first_person_character)))
    (:then_1
      (bind _asbp_boulder_parent (Utilities|Casting|CastToBP_BoulderParent OtherActor))
      (Variables|/Game/RollingWithThePunches/Blueprints/Actors/Boulders/BP_BoulderParent.BP_BoulderParent_C|SetInWater _asbp_boulder_parent false)
      (Variables|/Game/RollingWithThePunches/Blueprints/Actors/Boulders/BP_BoulderParent.BP_BoulderParent_C|SetWaterVolume _asbp_boulder_parent (Variables|Default|GetCurrentWaterScale)))))

(event Custom|ShiftWater
  (if (Variables|Default|GetShiftWater?)
    (Utilities|FlowControl|Delay (Variables|Default|GetWaterInterval))
    (Utilities|FlowControl|FlipFlop
      (:A
        (bind _wateralpha (Timeline|MoveWater Play)
          (:Update
            (Transformation|SetRelativeScale3D (Variables|Default|GetScene) (Math|Vector|Lerp(Vector) (Variables|Default|GetDefault%20Water%20Scale) (Variables|Default|GetAlteredWaterScale) _wateralpha))
            (CallFunction|ShiftWater))))
      (:B
        (Timeline|MoveWater Reverse)))))

(event EventBeginPlay
  (Utilities|FlowControl|Sequence
    (:then_0
      (Transformation|SetRelativeScale3D (Variables|Default|GetScene) (Variables|Default|GetDefault%20Water%20Scale))
      (Variables|Default|SetCurrentWaterScale (Variables|/Script/Engine.SceneComponent|GetRelativeScale3D (Variables|Default|GetScene))))
    (:then_1
      (CallFunction|ShiftWater))))

(event Collision|EventActorBeginOverlap
  (params (OtherActor :type Actor%20Object%20Reference)))

(event EventTick
  (params (DeltaSeconds :type Float%20%28single-precision%29)))

(fn ConstructionScript
  (Transformation|SetRelativeScale3D (Variables|Default|GetScene) (Variables|Default|GetDefault%20Water%20Scale))
  (Rendering|Material|SetMaterial (Variables|Default|GetCube) 0 (Variables|Default|GetWaterMaterial)))