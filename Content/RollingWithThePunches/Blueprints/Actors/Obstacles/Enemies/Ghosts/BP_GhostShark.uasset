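; Ghost shark enemy obstacle that bites what enters its range, extending a parent ghost actor.
; BiteRange overlaps play a nom montage and push physics-simulating components by LaunchVector times BiteForce, passing a normalized direction as the impulse location.
; CheckSharkMouth drives the AnimBP's Mouth value from player camera distance to the head socket, raising it as the camera nears.
; Movement check and Tick are empty; speed initialization defers to the parent.
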(event OnComponentBeginOverlap(BiteRange)
  (params (OverlappedComponent :type Primitive%20Component%20Object%20Reference) (OtherActor :type Actor%20Object%20Reference) (OtherComp :type Primitive%20Component%20Object%20Reference) (OtherBodyIndex :type Integer) (bFromSweep :type Boolean) (SweepResult :type Hit%20Result%20Structure%20%28by%20ref%29))
  (CallFunction|BitePhysicsObject OtherActor OtherComp)
  (Animation|Montage|PlayMontage (Variables|Default|GetSkeletalMesh) "/Game/OceanAnimalsMegaPack/Animations/GreatWhiteShark/AM_Nom.AM_Nom"))

(event Custom|CheckSharkMouth
  (Variables|/Game/OceanAnimalsMegaPack/Animations/GreatWhiteShark/GreatWhiteShark_AnimBP.GreatWhiteShark_AnimBP_C|SetMouth (Variables|Default|GetGreatWhiteSharkAnimBP) (Math|Float|Lerp 1.0 0.0 (Math|Float|Clamp(Float) (/ (- (Math|Vector|VectorLength (- (Camera|GetCameraLocation (Game|GetPlayerCameraManager 0)) (Transformation|GetSocketLocation (Variables|Default|GetSkeletalMesh) "b_HeadSocket"))) 175.0) (Variables|Default|GetMouth_DistanceToOpen))))))

(event Custom|CheckSharkMovement)

(event Collision|EventActorBeginOverlap
  (params (OtherActor :type Actor%20Object%20Reference)))

(event EventBeginPlay
  (|CallParentFunction)
  (bind _asgreat_white_shark_anim_bp (Utilities|Casting|CastToGreatWhiteShark_AnimBP (Components|SkeletalMesh|GetAnimInstance (Variables|Default|GetSkeletalMesh))))
  (Variables|Default|SetGreatWhiteSharkAnimBP _asgreat_white_shark_anim_bp))

(event EventInitializeGhostSpeed
  (|CallParentFunction))

(event EventTick
  (params (DeltaSeconds :type Float%20%28single-precision%29)))

(fn ConstructionScript
  (|CallParentFunction))

(fn BitePhysicsObject
  (params (Actor :type Actor%20Object%20Reference) (ActorComponent :type Primitive%20Component%20Object%20Reference))
  (if (Physics|IsSimulatingPhysics ActorComponent "None")
    (Physics|AddImpulseatLocation ActorComponent (* (Variables|Default|GetLaunch%20Vector) (Variables|Default|GetBiteForce)) (Math|Vector|Normalize (- (Transformation|GetActorLocation) (Transformation|GetActorLocation Actor))) "None")))