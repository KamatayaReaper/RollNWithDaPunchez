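; Parent ghost enemy that chases the player using a homing projectile movement component aimed at the player's mesh.
; A punch disables homing and launches the ghost along the camera's forward vector at force-scaled speed, with a default for zero force.
; A force-scaled retriggerable delay then restores base speed and homing.
; Timeline-driven flip and spin events exist but are not called within this graph.
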(event Custom|RepelGhostSpeed
  (params (ForceUnleashed :type Integer))
  (Variables|/Script/Engine.ProjectileMovementComponent|SetInitialSpeed (Variables|Default|GetProjectileMovement) (* (* (Variables|Default|GetBaseGhostSpeed) ForceUnleashed) 3.0))
  (Variables|/Script/Engine.ProjectileMovementComponent|SetMaxSpeed (Variables|Default|GetProjectileMovement) (* (* (Variables|Default|GetBaseGhostSpeed) ForceUnleashed) 3.0))
  (Variables|/Script/Engine.MovementComponent|SetVelocity (Variables|Default|GetProjectileMovement) (* (Variables|Default|GetProjectileDirection) (* (Variables|/Script/Engine.ProjectileMovementComponent|GetInitialSpeed (Variables|Default|GetProjectileMovement)) 5.0))))

(event Custom|Follow%20Player
  (bind _asbp_first_person_character (Utilities|Casting|CastToBP_FirstPersonCharacter (Game|GetPlayerCharacter 0)))
  (bind _output_get (Variables|Default|SetPlayerRef _asbp_first_person_character))
  (Variables|/Script/Engine.ProjectileMovementComponent|SetHomingTargetComponent (Variables|Default|GetProjectileMovement) (Variables|/Script/Engine.Character|GetMesh _output_get)))

(event Custom|ResetGhost
  (Variables|/Script/Engine.ProjectileMovementComponent|SetbIsHomingProjectile (Variables|Default|GetProjectileMovement) true)
  (CallFunction|InitializeGhostSpeed)
  (CallFunction|FollowPlayer))

(event Custom|InitializeGhostSpeed
  (Variables|/Script/Engine.ProjectileMovementComponent|SetInitialSpeed (Variables|Default|GetProjectileMovement) (Variables|Default|GetBaseGhostSpeed))
  (Variables|/Script/Engine.ProjectileMovementComponent|SetMaxSpeed (Variables|Default|GetProjectileMovement) (Variables|Default|GetBaseGhostSpeed)))

(event Custom|FlipGhostRotation
  (Utilities|FlowControl|Delay 0.2)
  (Variables|/Script/Engine.ProjectileMovementComponent|SetbRotationFollowsVelocity (Variables|Default|GetProjectileMovement) false)
  (bind _flipalpha (Timeline|FlipGhostTimeline PlayFromStart)
    (:Update
      (Transformation|SetActorRotation (Math|Rotator|Lerp(Rotator) (Transformation|GetActorRotation) (Transformation|GetWorldRotation (Variables|/Game/RollingWithThePunches/Blueprints/PlayerCharaacters/BP_FirstPersonCharacter.BP_FirstPersonCharacter_C|GetFirstPersonCamera (Variables|Default|GetPlayerRef))) _flipalpha)))
    (:Finished
      (CallFunction|SpinGhost))))

(event Custom|SpinGhost
  (Utilities|FlowControl|DoOnce false
    (:Completed
      (bind _flipalpha (Timeline|SpinGhost_Timeline PlayFromStart)
        (:Update
          (Variables|/Script/Engine.RotatingMovementComponent|SetRotationRate (Variables|Default|GetRotatingMovement) (Math|Rotator|Lerp(Rotator) "0, 0, 0" "0, 0,1080.000000" _flipalpha)))))))

(event Custom|UndoGhostSpin
  (Utilities|FlowControl|Sequence
    (:then_0
      (Utilities|FlowControl|DoOnce false) ; enters at Reset
    )
    (:then_1
      (bind _flipalpha (Timeline|SpinGhost_Timeline ReverseFromEnd)
        (:Update
          (Variables|/Script/Engine.RotatingMovementComponent|SetRotationRate (Variables|Default|GetRotatingMovement) (Math|Rotator|Lerp(Rotator) "0, 0, 0" "0, 0,1080.000000" _flipalpha)))))))

(event EventBeginPlay
  (Utilities|FlowControl|Sequence
    (:then_0
      (CallFunction|FollowPlayer))
    (:then_1
      (CallFunction|InitializeGhostSpeed))))

(event EventActivateProjectileAction
  (params (ForceUnleashed :type Integer) (PunchDirection :type Vector :default "0, 0, 0"))
  (CallFunction|RepelGhost ForceUnleashed PunchDirection)
  (Utilities|FlowControl|Sequence
    (:then_0
      (Utilities|FlowControl|RetriggerableDelay (Math|Conversions|ToFloat(Integer) (* ForceUnleashed 3)))
      (CallFunction|ResetGhost))))

(fn ConstructionScript)

(fn RepelGhost
  (params (PunchForce :type Integer) (PunchDirection :type Vector))
  (if (== PunchForce 0)
    (Variables|/Script/Engine.ProjectileMovementComponent|SetbIsHomingProjectile (Variables|Default|GetProjectileMovement) false)
    (Variables|Default|SetProjectileDirection (Math|Vector|GetForwardVector (Variables|/Game/RollingWithThePunches/Blueprints/PlayerCharaacters/BP_FirstPersonCharacter.BP_FirstPersonCharacter_C|GetFirstPersonCamera (Variables|Default|GetPlayerRef))))
    (CallFunction|RepelGhostSpeed (LocalVariables|GetDefaultPunchForce))
    (else
      (Variables|/Script/Engine.ProjectileMovementComponent|SetbIsHomingProjectile (Variables|Default|GetProjectileMovement) false)
      (Variables|Default|SetProjectileDirection (Math|Vector|GetForwardVector (Transformation|GetWorldRotation (Variables|/Game/RollingWithThePunches/Blueprints/PlayerCharaacters/BP_FirstPersonCharacter.BP_FirstPersonCharacter_C|GetFirstPersonCamera (Variables|Default|GetPlayerRef)))))
      (CallFunction|RepelGhostSpeed PunchForce))))