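; Base enemy Blueprint that chases the player character and is destroyed when its health runs out.
; A recursive AIMoveTo loop re-targets the player whenever a move succeeds or fails.
; If Stun is set when the loop restarts, the enemy moves to its own location, waits a few seconds, clears Stun and resumes chasing.
; AnyDamage reduces clamped CurrentHealth, which starts at MaxHealth.
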(event Custom|BeginEnemyLogic
  (if (not (Variables|Default|GetStun?))
    (AI|AIMoveTo self "0, 0,0.000000" (Variables|Default|GetPlayerRef) 5.0 false
      (:OnSuccess
        _)
      (:OnFail
        _))
    (CallFunction|BeginEnemyLogic)
    (else
      (AI|AIMoveTo self (Transformation|GetActorLocation) 0 5.0 false
        (:OnSuccess
          _)
        (:OnFail
          _))
      (Utilities|FlowControl|Delay 5.0)
      (Variables|Default|SetStun? false)
      (CallFunction|BeginEnemyLogic))))

(event EventBeginPlay
  (Variables|Default|SetCurrentHealth (Variables|Default|GetMaxHealth))
  (bind _asbp_first_person_character (Utilities|Casting|CastToBP_FirstPersonCharacter (Game|GetPlayerCharacter 0)))
  (Variables|Default|SetPlayerRef _asbp_first_person_character)
  (CallFunction|BeginEnemyLogic))

(event Game|Damage|EventAnyDamage
  (params (Damage :type Float%20%28single-precision%29) (DamageType :type Damage%20Type%20Object%20Reference) (InstigatedBy :type Controller%20Object%20Reference) (DamageCauser :type Actor%20Object%20Reference))
  (bind _output_get (Variables|Default|SetCurrentHealth (Math|Float|Clamp(Float) (- (Variables|Default|GetCurrentHealth) Damage) 0.0 (Variables|Default|GetMaxHealth))))
  (if (<= _output_get 0.0)
    (Actor|DestroyActor)))

(fn ConstructionScript)