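; BP_Lift is an obstacle actor whose cube moves back and forth between two points on a repeating cycle.
; A delay feeds a FlipFlop that alternately plays and reverses the MoveLift timeline, which lerps the cube's relative location.
; Timeline updates re-call TriggerLift, so the delay restarts the cycle without a separate timer.
; The construction script applies configurable cube scale and materials for cube and ring.
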(event Custom|TriggerLift
  (Utilities|FlowControl|Delay (Variables|Default|GetLiftIntervals))
  (Utilities|FlowControl|FlipFlop
    (:A
      (bind _liftalpha (Timeline|MoveLift Play)
        (:Update
          (Transformation|SetRelativeLocation (Variables|Default|GetCube) (Math|Vector|Lerp(Vector) (Variables|Default|GetPointA) (Variables|Default|GetPointB) _liftalpha) false false)
          (CallFunction|TriggerLift))))
    (:B
      (Timeline|MoveLift Reverse))))

(event EventBeginPlay
  (CallFunction|TriggerLift))

(fn ConstructionScript
  (Utilities|FlowControl|Sequence
    (:then_0
      (Transformation|SetRelativeScale3D (Variables|Default|GetCube) (Variables|Default|GetLiftScale)))
    (:then_1
      (Rendering|Material|SetMaterial (Variables|Default|GetCube) 0 (Variables|Default|GetCubeMat)))
    (:then_2
      (Rendering|Material|SetMaterial (Variables|Default|GetRing) 0 (Variables|Default|GetRingMat)))))