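; BP_FlipperBasic is an obstacle flipper that swings on a looping timer and launches physics objects it hits.
; Each trigger opens a CanLaunch window while a timeline rotates the Cylinder, then closes it and resets the DoOnce.
; During that window, the first simulating component overlapping FlipperCollision gets an impulse from LaunchVector and FlipperForce, applied at a normalized offset direction as location.
; A sphere-trace knockback event is only called from unconnected logic.
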(event OnComponentBeginOverlap(FlipperCollision)
  (params (OverlappedComponent :type Primitive%20Component%20Object%20Reference) (OtherActor :type Actor%20Object%20Reference) (OtherComp :type Primitive%20Component%20Object%20Reference) (OtherBodyIndex :type Integer) (bFromSweep :type Boolean) (SweepResult :type Hit%20Result%20Structure%20%28by%20ref%29))
  (if (Variables|Default|GetCanLaunch?)
    (if (Physics|IsSimulatingPhysics OtherComp "None")
      (Utilities|FlowControl|DoOnce false
        (:Completed
          (CallFunction|LaunchPhysicsObject OtherActor OtherComp))))))

(event Custom|TriggerFlipper
  (Variables|Default|SetCanLaunch? true)
  (bind _flipperalpha (Timeline|MoveFlipper PlayFromStart)
    (:Update
      (Transformation|SetRelativeRotation (Variables|Default|GetCylinder) (Math|Rotator|Lerp(Rotator) "0, 0, 0" (Variables|Default|GetFlipperRoation) _flipperalpha) false false))
    (:Finished
      (Variables|Default|SetCanLaunch? false)
      (CallFunction|ResetCollision))))

(event Custom|FlipperKnockback
  (bind _arrow (Variables|Default|GetArrow))
  (bind _returnvalue (Transformation|GetWorldLocation _arrow))
  (if (Variables|Default|GetCanLaunch?)
    (bind _outhit (Collision|SphereTraceByChannel _returnvalue (+ _returnvalue (* (Math|Vector|GetForwardVector (Transformation|GetWorldRotation _arrow)) 2.5e+02)) 75.0 "TraceTypeQuery1" false 0 "None"))
    (if (.bBlockingHit (Collision|BreakHitResult _outhit))
      (if (Physics|IsSimulatingPhysics (.HitComponent (Collision|BreakHitResult _outhit)) "None")
        (bind _returnvalue_2 (Physics|GetPhysicsLinearVelocity (.HitComponent (Collision|BreakHitResult _outhit)) "None"))
        (Physics|AddImpulseatLocation (.HitComponent (Collision|BreakHitResult _outhit)) (* _returnvalue_2 (Variables|Default|GetFlipperForce)) (.Location (Collision|BreakHitResult _outhit)) "None")))))

(event Custom|ResetCollision
  (Utilities|FlowControl|DoOnce false) ; enters at Reset
)

(event EventBeginPlay
  (Utilities|Time|SetTimerbyEvent (delegate Custom|TriggerFlipper) (Variables|Default|GetFlipperInterval) true))

(event EventTick
  (params (DeltaSeconds :type Float%20%28single-precision%29)))

(fn ConstructionScript)

(fn LaunchPhysicsObject
  (params (Actor :type Actor%20Object%20Reference) (ActorComponent :type Primitive%20Component%20Object%20Reference))
  (Physics|AddImpulseatLocation ActorComponent (* (Variables|Default|GetLaunch%20Vector) (Variables|Default|GetFlipperForce)) (Math|Vector|Normalize (- (Transformation|GetActorLocation Actor) (Transformation|GetActorLocation))) "None"))