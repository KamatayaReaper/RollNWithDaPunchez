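; BP_TeleporterParent is a base teleporter obstacle actor that maintains references to the player character and the current boulder, with no teleport logic of its own.
; On BeginPlay it caches the first-person player and the last BP_BoulderParent actor found in the level.
; A fast looping timer runs ResetBoulder, which searches for a boulder again whenever the stored reference becomes invalid.
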(event Custom|ResetBoulder
  (Utilities|IsValid (Variables|Default|GetCurrentBoulder)
    (:Is%20Not%20Valid
      (bind _outactors (Actor|GetAllActorsOfClass "/Game/RollingWithThePunches/Blueprints/Actors/Boulders/BP_BoulderParent.BP_BoulderParent_C"))
      (for _array_element _outactors
        (Variables|Default|SetCurrentBoulder _array_element)))))

(event EventBeginPlay
  (Utilities|FlowControl|Sequence
    (:then_0
      (bind _outactors (Actor|GetAllActorsOfClass "/Game/RollingWithThePunches/Blueprints/Actors/Boulders/BP_BoulderParent.BP_BoulderParent_C"))
      (for _array_element _outactors
        (bind _output_get (Variables|Default|SetCurrentBoulder _array_element))))
    (:then_1
      (bind _asbp_first_person_character (Utilities|Casting|CastToBP_FirstPersonCharacter (Game|GetPlayerCharacter 0)))
      (bind _output_get_2 (Variables|Default|SetPlayerRef _asbp_first_person_character)))
    (:then_2
      (Utilities|Time|SetTimerbyEvent (delegate Custom|ResetBoulder) 0.1 true))))

(event Collision|EventActorBeginOverlap
  (params (OtherActor :type Actor%20Object%20Reference)))

(event EventTick
  (params (DeltaSeconds :type Float%20%28single-precision%29)))

(fn ConstructionScript)