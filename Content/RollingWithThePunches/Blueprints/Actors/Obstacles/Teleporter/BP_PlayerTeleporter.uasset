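; BP_PlayerTeleporter is an obstacle actor that teleports the player to a linked end point when the player overlaps it.
; On overlap, it checks that the other actor is the referenced player, then moves it to the world location of the TeleportEndPoint's Arrow component.
; The move is an unswept teleport that changes only location, with no rotation applied.
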(event EventBeginPlay
  (|CallParentFunction) ; This node is disabled and will not be called.\nDrag off pins to build functionality.
)

(event Collision|EventActorBeginOverlap
  (params (OtherActor :type Actor%20Object%20Reference))
  (if (== OtherActor (Variables|Default|GetPlayerRef))
    (Transformation|SetActorLocation (Variables|Default|GetPlayerRef) (Transformation|GetWorldLocation (Variables|/Game/RollingWithThePunches/Blueprints/Actors/Obstacles/Teleporter/BP_TeleporterParent.BP_TeleporterParent_C|GetArrow (Variables|Default|GetTeleportEndPoint))) false true)))

(event EventTick
  (params (DeltaSeconds :type Float%20%28single-precision%29))
  (|CallParentFunction DeltaSeconds) ; This node is disabled and will not be called.\nDrag off pins to build functionality.
)

(fn ConstructionScript
  (|CallParentFunction))