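; BP_BoulderTeleporter is an obstacle actor that teleports the boulder to a linked end point.
; When its capsule is overlapped, it checks whether the other actor is the stored CurrentBoulder reference.
; On a match it prints a debug message and moves the boulder's root component, without sweeping, to the world location of the TeleportEndPoint's arrow.
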(event OnComponentBeginOverlap(Capsule)
  (params (OverlappedComponent :type Primitive%20Component%20Object%20Reference) (OtherActor :type Actor%20Object%20Reference) (OtherComp :type Primitive%20Component%20Object%20Reference) (OtherBodyIndex :type Integer) (bFromSweep :type Boolean) (SweepResult :type Hit%20Result%20Structure%20%28by%20ref%29))
  (if (== OtherActor (Variables|Default|GetCurrentBoulder))
    (Development|PrintString "Hello")
    (Transformation|SetWorldLocation (Variables|/Script/Engine.Actor|GetRootComponent (Variables|Default|GetCurrentBoulder)) (Transformation|GetWorldLocation (Variables|/Game/RollingWithThePunches/Blueprints/Actors/Obstacles/Teleporter/BP_TeleporterParent.BP_TeleporterParent_C|GetArrow (Variables|Default|GetTeleportEndPoint))) false true)))

(event Collision|EventActorBeginOverlap
  (params (OtherActor :type Actor%20Object%20Reference)))

(fn ConstructionScript
  (|CallParentFunction))