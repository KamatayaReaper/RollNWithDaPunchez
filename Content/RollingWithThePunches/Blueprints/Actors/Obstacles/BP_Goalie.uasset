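; BP_Goalie is a moving obstacle that repels physics objects and can be knocked over by damage.
; The construction script sets its movement component's path from the origin to PosB, with GoalieSpeed as the duration.
; Box overlaps apply a strong impulse opposite to the incoming object's velocity.
; Any damage plays a timeline that flips the Cylinder, with its Update triggering a delayed reverse to stand it back up.
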(event OnComponentBeginOverlap(Box)
  (params (OverlappedComponent :type Primitive%20Component%20Object%20Reference) (OtherActor :type Actor%20Object%20Reference) (OtherComp :type Primitive%20Component%20Object%20Reference) (OtherBodyIndex :type Integer) (bFromSweep :type Boolean) (SweepResult :type Hit%20Result%20Structure%20%28by%20ref%29))
  (if (Physics|IsSimulatingPhysics OtherComp "None")
    (bind _returnvalue (Physics|GetPhysicsLinearVelocity OtherComp "None"))
    (Physics|AddImpulseatLocation OtherComp (* _returnvalue -2e+03) (Transformation|GetActorLocation) "None")))

(event Custom|KnockGoalie
  (bind _flipalpha (Timeline|FlipGoalie Play)
    (:Update
      (Transformation|SetRelativeRotation (Variables|Default|GetCylinder) (Math|Rotator|Lerp(Rotator) "-90.000000, 0,0.000000" "0.000000,90.000000,-90.000000" _flipalpha) false false)
      (CallFunction|ResetGoalie))))

(event Custom|ResetGoalie
  (Utilities|FlowControl|Delay 3.0)
  (bind _flipalpha (Timeline|FlipGoalie Reverse)
    (:Update
      (Transformation|SetRelativeRotation (Variables|Default|GetCylinder) (Math|Rotator|Lerp(Rotator) "-90.000000, 0,0.000000" "0.000000,90.000000,-90.000000" _flipalpha) false false)
      (CallFunction|ResetGoalie))))

(event EventBeginPlay)

(event Game|Damage|EventAnyDamage
  (params (Damage :type Float%20%28single-precision%29) (DamageType :type Damage%20Type%20Object%20Reference) (InstigatedBy :type Controller%20Object%20Reference) (DamageCauser :type Actor%20Object%20Reference))
  (CallFunction|KnockGoalie))

(fn ConstructionScript
  (Utilities|FlowControl|Sequence
    (:then_0
      (Class|InterptoMovementComponent|AddControlPointPosition (Variables|Default|GetGoalieMovement) "0, 0, 0" true)
      (Class|InterptoMovementComponent|AddControlPointPosition (Variables|Default|GetGoalieMovement) (Variables|Default|GetPosB) true))
    (:then_1
      (Variables|/Script/Engine.InterpToMovementComponent|SetDuration (Variables|Default|GetGoalieMovement) (Variables|Default|GetGoalieSpeed)))))