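; Conveyor belt obstacle, filed under Scrapped, that carries actors and physics objects along its Arrow's forward direction.
; Each tick moves actors overlapping the Box by Speed using an unswept world offset.
; Tick also triggers a Delay-throttled sphere trace from Arrow to Scene, drawn persistently, that impulses the simulating component hit with a Speed-derived force.
; The construction script applies mesh scale and trace endpoint positions from variables.
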(event Custom|MovePhysicsObjects
  (Utilities|FlowControl|Delay (Variables|Default|GetPushRate))
  (bind _outhit (Collision|SphereTraceForObjects (Transformation|GetWorldLocation (Variables|Default|GetArrow)) (Transformation|GetWorldLocation (Variables|Default|GetScene)) (Variables|Default|GetConveyerRadius) (Utilities|Array|MakeArray "ObjectTypeQuery4" "ObjectTypeQuery2") false 0 "Persistent"))
  (if (.bBlockingHit (Collision|BreakHitResult _outhit))
    (if (Physics|IsSimulatingPhysics (.HitComponent (Collision|BreakHitResult _outhit)) "None")
      (Physics|AddImpulseatLocation (.HitComponent (Collision|BreakHitResult _outhit)) (* (Variables|Default|GetConveyerDirection) (Variables|Default|GetConveyerForce)) (.ImpactPoint (Collision|BreakHitResult _outhit)) "None"))))

(event Custom|Set%20ConveyerForce
  (Variables|Default|SetConveyerForce (* (Variables|Default|GetSpeed) 1e+01)))

(event EventBeginPlay
  (Utilities|FlowControl|Sequence
    (:then_0
      (Variables|Default|SetConveyerDirection (Math|Vector|GetForwardVector (Transformation|GetWorldRotation (Variables|Default|GetArrow)))))
    (:then_1
      (CallFunction|SetConveyerForce))))

(event EventTick
  (params (DeltaSeconds :type Float%20%28single-precision%29))
  (Utilities|FlowControl|Sequence
    (:then_0
      (CallFunction|MovePhysicsObjects))
    (:then_1
      (for _array_element (Collision|GetOverlappingActors (Variables|Default|GetBox) 0 :!class /Script/Engine.PrimitiveComponent)
        (Transformation|AddActorWorldOffset _array_element (* (* DeltaSeconds (Variables|Default|GetSpeed)) (Math|Vector|GetForwardVector (Transformation|GetWorldRotation (Variables|Default|GetArrow)))))))))

(fn ConstructionScript
  (Utilities|FlowControl|Sequence
    (:then_0
      (Transformation|SetRelativeScale3D (Variables|Default|GetStaticMesh) (Variables|Default|GetConveyerSize)))
    (:then_1
      (Transformation|SetRelativeLocation (Variables|Default|GetArrow) (Variables|Default|GetArrowLocation) false false))
    (:then_2
      (Transformation|SetRelativeLocation (Variables|Default|GetScene) (Variables|Default|GetEndLocation) false false))))