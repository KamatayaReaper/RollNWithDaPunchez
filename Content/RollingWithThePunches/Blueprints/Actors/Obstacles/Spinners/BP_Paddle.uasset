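; BP_Paddle is a spinner obstacle with up to four paddles that rotate continuously.
; On BeginPlay it copies its RotationRate variable into the RotatingMovement component, then shows or hides each paddle from per-paddle visibility flags.
; Each paddle's collision follows its visibility, with query and physics when visible and none when hidden, so one Blueprint supports different paddle layouts.
; The construction script is empty, so this setup is applied only at runtime.
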(event Custom|SetPaddleVisibility
  (Rendering|SetVisibility (Variables|Default|GetPaddle1) (Variables|Default|GetPaddle1_Visible?) false)
  (Rendering|SetVisibility (Variables|Default|GetPaddle2) (Variables|Default|GetPadde2_Visible?) false)
  (Rendering|SetVisibility (Variables|Default|GetPaddle3) (Variables|Default|GetPaddle3_Visible?) false)
  (Rendering|SetVisibility (Variables|Default|GetPaddle4) (Variables|Default|GetPaddle4_Visible?) false)
  (CallFunction|SetPaddleCollision))

(event Custom|SetPaddleCollision
  (Utilities|FlowControl|Sequence
    (:then_0
      (if (Rendering|IsVisible (Variables|Default|GetPaddle1))
        (Collision|SetCollisionEnabled (Variables|Default|GetPaddle1) "QueryAndPhysics")
        (else
          (Collision|SetCollisionEnabled (Variables|Default|GetPaddle1) "NoCollision"))))
    (:then_1
      (if (Rendering|IsVisible (Variables|Default|GetPaddle2))
        (Collision|SetCollisionEnabled (Variables|Default|GetPaddle2) "QueryAndPhysics")
        (else
          (Collision|SetCollisionEnabled (Variables|Default|GetPaddle2) "NoCollision"))))
    (:then_2
      (if (Rendering|IsVisible (Variables|Default|GetPaddle3))
        (Collision|SetCollisionEnabled (Variables|Default|GetPaddle3) "QueryAndPhysics")
        (else
          (Collision|SetCollisionEnabled (Variables|Default|GetPaddle3) "NoCollision"))))
    (:then_3
      (if (Rendering|IsVisible (Variables|Default|GetPaddle4))
        (Collision|SetCollisionEnabled (Variables|Default|GetPaddle4) "QueryAndPhysics")
        (else
          (Collision|SetCollisionEnabled (Variables|Default|GetPaddle4) "NoCollision"))))))

(event EventBeginPlay
  (Utilities|FlowControl|Sequence
    (:then_0
      (Variables|/Script/Engine.RotatingMovementComponent|SetRotationRate (Variables|Default|GetRotatingMovement) (Variables|Default|GetRotation%20Rate)))
    (:then_1
      (CallFunction|SetPaddleVisibility))))

(fn ConstructionScript)