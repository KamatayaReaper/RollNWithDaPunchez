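; BP_Boostpad is a boost pad obstacle that launches the player and physics objects overlapping its BoostZone.
; Both follow the BoostDirection component's forward vector: the player via LaunchCharacter with overridden velocity, simulating components via added linear velocity.
; An IncreasePhysicsBoost event, with no live call in this graph, raises the physics force until a retriggerable delay resets it.
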(event OnComponentBeginOverlap(BoostZone)
  (params (OverlappedComponent :type Primitive%20Component%20Object%20Reference) (OtherActor :type Actor%20Object%20Reference) (OtherComp :type Primitive%20Component%20Object%20Reference) (OtherBodyIndex :type Integer) (bFromSweep :type Boolean) (SweepResult :type Hit%20Result%20Structure%20%28by%20ref%29))
  (bind _boostforce (Variables|Default|GetBoostForce))
  (Utilities|FlowControl|Sequence
    (:then_0
      (CallFunction|LaunchPlayer _boostforce _boostforce OtherActor))
    (:then_1
      (if (Physics|IsSimulatingPhysics OtherComp "None")
        (Physics|SetPhysicsLinearVelocity OtherComp (* (Math|Vector|GetForwardVector (Transformation|GetWorldRotation (Variables|Default|GetBoostDirection))) (Variables|Default|GetBoostPhysicsForce)) true "None")))))

(event Custom|IncreasePhysicsBoost
  (bind _output_get (Variables|Default|SetBoostMultiplier (+ (Variables|Default|GetBoostMultiplier) 1)))
  (Variables|Default|SetBoostPhysicsForce (* _output_get (Variables|Default|GetBoostPhysicsForce)))
  (Utilities|FlowControl|RetriggerableDelay 3.0)
  (Variables|Default|SetBoostMultiplier 1)
  (Variables|Default|SetBoostPhysicsForce 1e+05))

(event EventBeginPlay
  (bind _asbp_first_person_character (Utilities|Casting|CastToBP_FirstPersonCharacter (Game|GetPlayerCharacter 0)))
  (Variables|Default|SetPlayerRef _asbp_first_person_character))

(event Collision|EventActorBeginOverlap
  (params (OtherActor :type Actor%20Object%20Reference)))

(event EventTick
  (params (DeltaSeconds :type Float%20%28single-precision%29)))

(fn ConstructionScript)

(fn LaunchPlayer
  (params (Boost_X :type Float%20%28double-precision%29) (Boost_Y :type Float%20%28double-precision%29) (Actor :type Actor%20Object%20Reference))
  (if (== Actor (Variables|Default|GetPlayerRef))
    (Character|LaunchCharacter (Variables|Default|GetPlayerRef) (* (Math|Vector|GetForwardVector (Transformation|GetWorldRotation (Variables|Default|GetBoostDirection))) (Math|Vector|MakeVector Boost_X Boost_Y 1e+02)) true true)))