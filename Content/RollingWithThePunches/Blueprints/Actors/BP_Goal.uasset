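; Goal actor that detects when a boulder rests inside its sphere trigger.
; Overlap begin and end toggle sound, spin and materials, and set the player's BallIn flag and HUD completion display.
; Tick feeds a Delay-throttled distance check that shows the goal's widget only when the player is roughly 25 meters or farther away.
; The construction script scales the range ring from GoalRingSize.
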(event OnComponentBeginOverlap(Sphere)
  (params (OverlappedComponent :type Primitive%20Component%20Object%20Reference) (OtherActor :type Actor%20Object%20Reference) (OtherComp :type Primitive%20Component%20Object%20Reference) (OtherBodyIndex :type Integer) (bFromSweep :type Boolean) (SweepResult :type Hit%20Result%20Structure%20%28by%20ref%29))
  (bind _asbp_boulder_parent (Utilities|Casting|CastToBP_BoulderParent OtherActor))
  (if (== _asbp_boulder_parent OtherActor)
    (Audio|PlaySoundatLocation "/Game/RollingWithThePunches/Assets/Sounds/ActivateGoal.ActivateGoal" (Transformation|GetActorLocation) "0, 0, 0" 1.0 1.0 0.0 0 0 0 0)
    (Variables|/Script/Engine.RotatingMovementComponent|SetRotationRate (Variables|Default|GetRotatingMovement) "0,720.000000, 0")
    (Rendering|Material|SetMaterial (Variables|Default|GetSignal) 0 "/Game/RollingWithThePunches/Assets/Material/Emissive/E_OceanGreen.E_OceanGreen")
    (Rendering|Material|SetMaterial (Variables|Default|GetGoalRange) 0 "/Game/RollingWithThePunches/Assets/Material/MI_GoalTouched.MI_GoalTouched")
    (Variables|/Game/RollingWithThePunches/Blueprints/PlayerCharaacters/BP_FirstPersonCharacter.BP_FirstPersonCharacter_C|SetBallIn? (Variables|Default|GetPlayerRef) true)
    (Default|ShowCompletion (Variables|/Game/RollingWithThePunches/Blueprints/PlayerCharaacters/BP_FirstPersonCharacter.BP_FirstPersonCharacter_C|GetPlayerHUDRef (Variables|Default|GetPlayerRef)))))

(event OnComponentEndOverlap(Sphere)
  (params (OverlappedComponent :type Primitive%20Component%20Object%20Reference) (OtherActor :type Actor%20Object%20Reference) (OtherComp :type Primitive%20Component%20Object%20Reference) (OtherBodyIndex :type Integer))
  (bind _asbp_boulder_parent (Utilities|Casting|CastToBP_BoulderParent OtherActor))
  (if (== _asbp_boulder_parent OtherActor)
    (Audio|PlaySoundatLocation "/Game/RollingWithThePunches/Assets/Sounds/DeActivateGoal.DeActivateGoal" (Transformation|GetActorLocation) "0, 0, 0" 1.0 1.0 0.0 0 0 0 0)
    (Variables|/Script/Engine.RotatingMovementComponent|SetRotationRate (Variables|Default|GetRotatingMovement) "0, 0, 0")
    (Rendering|Material|SetMaterial (Variables|Default|GetSignal) 0 "/Game/RollingWithThePunches/Assets/Material/Emissive/E_Watermelon.E_Watermelon")
    (Rendering|Material|SetMaterial (Variables|Default|GetGoalRange) 0 "/Game/RollingWithThePunches/Assets/Material/MI_GoalUntrouched.MI_GoalUntrouched")
    (Variables|/Game/RollingWithThePunches/Blueprints/PlayerCharaacters/BP_FirstPersonCharacter.BP_FirstPersonCharacter_C|SetBallIn? (Variables|Default|GetPlayerRef) false)
    (Default|HideCompletion (Variables|/Game/RollingWithThePunches/Blueprints/PlayerCharaacters/BP_FirstPersonCharacter.BP_FirstPersonCharacter_C|GetPlayerHUDRef (Variables|Default|GetPlayerRef)))))

(event Custom|CheckDistance
  (bind _widget (Variables|Default|GetWidget))
  (Utilities|FlowControl|Delay 0.2)
  (if (>= (Math|Float|Round (/ (Math|Vector|VectorLength (- (Transformation|GetWorldLocation (Variables|Default|GetWidget)) (Transformation|GetActorLocation (Pawn|GetControlledPawn (Game|GetPlayerController 0))))) 1e+02)) 25)
    (Rendering|SetVisibility _widget true false)
    (else
      (Rendering|SetVisibility _widget false false))))

(event EventBeginPlay
  (bind _asbp_first_person_character (Utilities|Casting|CastToBP_FirstPersonCharacter (Game|GetPlayerCharacter 0)))
  (Variables|Default|SetPlayerRef _asbp_first_person_character))

(event Collision|EventActorBeginOverlap
  (params (OtherActor :type Actor%20Object%20Reference)))

(event EventTick
  (params (DeltaSeconds :type Float%20%28single-precision%29))
  (CallFunction|CheckDistance))

(fn ConstructionScript
  (Transformation|SetRelativeScale3D (Variables|Default|GetGoalRange) (Variables|Default|GetGoalRingSize)))