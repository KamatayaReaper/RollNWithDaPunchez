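; BP_JellyfishDecoration is a decorative jellyfish actor built on a skeletal mesh.
; Its construction script calls the parent's, then assigns three material variables across the mesh's four slots, reusing the first in two of them.
; The event graph holds only disabled default events, so the Blueprint adds no runtime logic of its own.
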(event EventBeginPlay
  (|CallParentFunction) ; This node is disabled and will not be called.\nDrag off pins to build functionality.
)

(event Collision|EventActorBeginOverlap
  (params (OtherActor :type Actor%20Object%20Reference))
  (|CallParentFunction OtherActor) ; This node is disabled and will not be called.\nDrag off pins to build functionality.
)

(event EventTick
  (params (DeltaSeconds :type Float%20%28single-precision%29))
  (|CallParentFunction DeltaSeconds) ; This node is disabled and will not be called.\nDrag off pins to build functionality.
)

(fn ConstructionScript
  (|CallParentFunction)
  (Rendering|Material|SetMaterial (Variables|Default|GetSkeletalMesh) 0 (Variables|Default|GetMat0))
  (Rendering|Material|SetMaterial (Variables|Default|GetSkeletalMesh) 1 (Variables|Default|GetMat1))
  (Rendering|Material|SetMaterial (Variables|Default|GetSkeletalMesh) 2 (Variables|Default|GetMat0))
  (Rendering|Material|SetMaterial (Variables|Default|GetSkeletalMesh) 3 (Variables|Default|GetMat2)))