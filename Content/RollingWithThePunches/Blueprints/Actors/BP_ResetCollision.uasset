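; BP_ResetCollision is a reset volume that returns the player and boulders when they enter its box.
; On BeginPlay it caches the first-person character and its starting location.
; On overlap it calls ResetBoulder on boulder actors, teleports the player back to that start, and plays a sound at the volume's location.
; The construction script sizes the box from the BoxRange variable.
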(event OnComponentBeginOverlap(Box)
  (params (OverlappedComponent :type Primitive%20Component%20Object%20Reference) (OtherActor :type Actor%20Object%20Reference) (OtherComp :type Primitive%20Component%20Object%20Reference) (OtherBodyIndex :type Integer) (bFromSweep :type Boolean) (SweepResult :type Hit%20Result%20Structure%20%28by%20ref%29))
  (Utilities|FlowControl|Sequence
    (:then_0
      (bind _asbp_boulder_parent (Utilities|Casting|CastToBP_BoulderParent OtherActor))
      (Default|ResetBoulder _asbp_boulder_parent))
    (:then_1
      (if (== OtherActor (Variables|Default|GetPlayerRef))
        (Transformation|SetActorLocation (Variables|Default|GetPlayerRef) (Variables|Default|GetPlayerStart) false true)))
    (:then_2
      (Audio|PlaySoundatLocation "/Game/Interface_And_Item_Sounds/WAV/Special_Musical_04.Special_Musical_04" (Transformation|GetActorLocation) "0, 0, 0" 1.0 1.0 0.0 0 0 0 0))))

(event EventBeginPlay
  (Utilities|FlowControl|Sequence
    (:then_0
      (bind _asbp_first_person_character (Utilities|Casting|CastToBP_FirstPersonCharacter (Game|GetPlayerCharacter 0)))
      (bind _output_get (Variables|Default|SetPlayerRef _asbp_first_person_character))
      (Variables|Default|SetPlayerStart (Transformation|GetActorLocation _output_get)))))

(fn ConstructionScript
  (Components|Box|SetBoxExtent (Variables|Default|GetBox) (Variables|Default|GetBoxRange) true))