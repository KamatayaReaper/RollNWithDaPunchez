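; First-person arms actor that handles the player's alternating charged punches and an Uppercut or Fireball special.
; Timelines drive charge, which sets force tier, impact size and hit-stop duration.
; Punches and uppercuts sphere-trace from the camera, then dispatch by physics state, component tag or interface to push, damage, stun or deflect; other surfaces launch the player.
; Hit stop uses time dilation, and specials recharge on a Tick-driven cooldown.
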(event Custom|StartCharging
  (if (Variables|Punch|GetCanPunch?)
    (Variables|Punch|SetIsCharging? true)
    (Components|Timeline|SetPlayRate (Variables|Default|GetChargePunch) (/ 1.0 (Variables|Punch|GetChargeTime)))
    (bind _chargealpha (Timeline|ChargePunch Play)
      (:Update
        (bind _output_get (Variables|Punch|SetCurrentCharge (Math|Float|Clamp(Float) _chargealpha)))
        (if (>= _output_get 1.0)
          (Variables|Punch|SetCanPunch? false)
          (CallFunction|ReleaseCharge))))))

(event Custom|ReleaseCharge
  (bind _skeletalmesh (Variables|Default|GetSkeletalMesh))
  (Variables|Punch|SetIsCharging? false)
  (Utilities|FlowControl|Sequence
    (:then_0
      (CallFunction|SwitchArms)
      (if (Variables|Default|GetIsRight?)
        (Animation|Montage|PlayMontage _skeletalmesh "/Game/FIrstPersonPunchAnims/Anims/AttacksAndBlocks/AM_Punch1.AM_Punch1" 2.0)
        (else
          (Animation|Montage|PlayMontage _skeletalmesh "/Game/FIrstPersonPunchAnims/Anims/AttacksAndBlocks/AM_Punch2.AM_Punch2" 2.0))))
    (:then_1
      (Utilities|FlowControl|Delay 0.21)
      (CallFunction|SetPunchForce)
      (Punch|HitObject)
      (Utilities|FlowControl|Sequence
        (:then_0
          (Utilities|FlowControl|Delay 0.2)
          (Variables|Punch|SetPunchForce 2e+05)
          (Variables|Punch|SetCanPunch? true)
          (Variables|Punch|SetImpactSize "1.000000,1.000000,1.000000")
          (Components|Timeline|SetPlayRate (Variables|Default|GetChargePunch) 1.0)
          (bind _chargealpha (Timeline|ChargePunch Reverse)
            (:Update
              (bind _output_get (Variables|Punch|SetCurrentCharge (Math|Float|Clamp(Float) _chargealpha)))
              (if (>= _output_get 1.0)
                (Variables|Punch|SetCanPunch? false)
                (CallFunction|ReleaseCharge)))))
        (:then_1
          (Utilities|FlowControl|Delay 1.25)
          (Variables|Punch|SetForceUnleashed 1))))))

(event Custom|SwitchArms
  (Utilities|FlowControl|FlipFlop
    (:A
      (Variables|Default|SetIsRight? true))
    (:B
      (Variables|Default|SetIsRight? false))))

(event Custom|SetPunchForce
  (bind _currentcharge (Variables|Punch|GetCurrentCharge))
  (bind _currentcharge_2 (Variables|Punch|GetCurrentCharge))
  (bind _currentcharge_3 (Variables|Punch|GetCurrentCharge))
  ;[0 1 0.9537] Set Punch Force
  (if (< (Variables|Punch|GetCurrentCharge) 0.1)
    (Variables|Punch|SetPunchForce 2e+05)
    (Variables|Default|SetHitStopDuration 0.2)
    (Variables|Punch|SetForceUnleashed 0)
    (Variables|Punch|SetImpactSize "1.000000,1.000000,1.000000")
    (elif (and (>= _currentcharge 0.1) (< _currentcharge 0.33))
      (Variables|Punch|SetPunchForce (* (Variables|Punch|GetPunchForce) 1.0))
      (Variables|Default|SetHitStopDuration 0.2)
      (Variables|Punch|SetForceUnleashed 1)
      (Variables|Punch|SetImpactSize "1.250000,1.250000,1.250000")
      (elif (and (>= _currentcharge_2 0.33) (< _currentcharge_2 0.66))
        (Variables|Punch|SetPunchForce (* (Variables|Punch|GetPunchForce) 2.0))
        (Variables|Default|SetHitStopDuration 0.2)
        (Variables|Punch|SetForceUnleashed 2)
        (Variables|Punch|SetImpactSize "1.500000,1.500000,1.500000")
        (elif (and (>= _currentcharge_3 0.66) (<= _currentcharge_3 0.99))
          (Variables|Punch|SetPunchForce (* (Variables|Punch|GetPunchForce) 3.0))
          (Variables|Default|SetHitStopDuration 0.2)
          (Variables|Punch|SetForceUnleashed 3)
          (Variables|Punch|SetImpactSize "1.750000,1.750000,1.750000")
          (elif (>= (Variables|Punch|GetCurrentCharge) 1.0)
            (Variables|Punch|SetPunchForce (* (Variables|Punch|GetPunchForce) 5.0))
            (Variables|Default|SetHitStopDuration 0.5)
            (Variables|Punch|SetForceUnleashed 4)
            (Variables|Punch|SetImpactSize "2.000000,2.000000,2.000000")))))))

(event Custom|ActivateHitstop
  (Utilities|FlowControl|Sequence
    (:then_0
      (bind _dilationalpha (Timeline|HitStopTimeline PlayFromStart)
        (:Update
          (Utilities|Time|SetGlobalTimeDilation _dilationalpha))))))

(event Custom|ChargeSpecial
  (if (Variables|Special|GetSpecialAvailable?)
    (Components|Timeline|SetPlayRate (Variables|Default|GetChargingSpecial) (/ 1.0 (Variables|Punch|GetChargeTime)))
    (bind _chargealpha (Timeline|ChargingSpecial Play)
      (:Update
        (bind _output_get (Variables|Obsolete|SetSpecialCharge (Math|Float|Clamp(Float) _chargealpha)))
        (if (>= _output_get 1.0)
          (Variables|Special|SetSpecialAvailable? false)
          (CallFunction|ReleaseSpecial))))))

(event Custom|ReleaseSpecial
  (Utilities|FlowControl|Sequence
    (:then_0
      (Components|Timeline|SetPlayRate (Variables|Default|GetChargingSpecial) 1.0)
      (bind _chargealpha (Timeline|ChargingSpecial Reverse)
        (:Update
          (bind _output_get (Variables|Obsolete|SetSpecialCharge (Math|Float|Clamp(Float) _chargealpha)))
          (if (>= _output_get 1.0)
            (Variables|Special|SetSpecialAvailable? false)
            (CallFunction|ReleaseSpecial)))))
    (:then_1
      (switch Utilities|FlowControl|Switch|SwitchonE_SpecialMove (Variables|Special|GetE_SpecialMoveType)
        (:NewEnumerator5
          (CallFunction|Uppercut))
        (:NewEnumerator6
          (CallFunction|Fireball))))))

(event Custom|Uppercut
  (bind _skeletalmesh (Variables|Default|GetSkeletalMesh))
  (Utilities|FlowControl|Sequence
    (:then_0
      (CallFunction|SwitchArms)
      (if (Variables|Default|GetIsRight?)
        (Animation|Montage|PlayMontage _skeletalmesh "/Game/FIrstPersonPunchAnims/Anims/AttacksAndBlocks/AM_Punch5.AM_Punch5" 2.0
          (:then
            _))
        (else
          (Animation|Montage|PlayMontage _skeletalmesh "/Game/FIrstPersonPunchAnims/Anims/AttacksAndBlocks/AM_Punch6.AM_Punch6" 2.0
            (:then
              _))))
      (Audio|PlaySoundatLocation "/Game/RollingWithThePunches/Assets/Sounds/PunchWhiff/PunchWhiff.PunchWhiff" (Transformation|GetActorLocation) "0, 0, 0" 1.0 1.0 0.0 0 0 0 0))
    (:then_1
      (Utilities|FlowControl|Delay 0.21)
      (CallFunction|SetPunchForce)
      (Uppercut|UppercutObject)
      (Variables|Special|SetSpecialAvailable? false)
      (Utilities|FlowControl|Sequence
        (:then_0
          (Utilities|FlowControl|Delay 0.2)
          (Variables|Punch|SetPunchForce 2e+05)
          (Variables|Punch|SetCanPunch? true)
          (Variables|Punch|SetImpactSize "1.000000,1.000000,1.000000"))
        (:then_1
          (Utilities|FlowControl|Delay 1.25)
          (Variables|Punch|SetForceUnleashed 1))))))

(event Custom|Fireball
  (bind _skeletalmesh (Variables|Default|GetSkeletalMesh))
  (bind _playerref (Variables|Default|GetPlayerRef))
  (bind _firstpersoncamera (Variables|/Game/RollingWithThePunches/Blueprints/PlayerCharaacters/BP_FirstPersonCharacter.BP_FirstPersonCharacter_C|GetFirstPersonCamera _playerref))
  (Utilities|FlowControl|Sequence
    (:then_0
      (CallFunction|SwitchArms)
      (if (Variables|Default|GetIsRight?)
        (Animation|Montage|PlayMontage _skeletalmesh "/Game/FIrstPersonPunchAnims/Anims/AttacksAndBlocks/AM_Punch3.AM_Punch3" 2.0)
        (else
          (Animation|Montage|PlayMontage _skeletalmesh "/Game/FIrstPersonPunchAnims/Anims/AttacksAndBlocks/AM_Punch4.AM_Punch4" 2.0))))
    (:then_1
      (Utilities|FlowControl|Delay 0.45)
      (Game|SpawnActorfromClass "/Game/RollingWithThePunches/Blueprints/Actors/Projectiles/BP_ProjectileParent.BP_ProjectileParent_C" (Math|Transform|MakeTransform (Transformation|GetWorldLocation _firstpersoncamera) (Transformation|GetWorldRotation _firstpersoncamera) "1.000000,1.000000,1.000000") "Undefined" 0 0))))

(event Custom|ActivateSpecial
  (Variables|Special|SetSpecialAvailable? false)
  (switch Utilities|FlowControl|Switch|SwitchonE_SpecialMove (Variables|Special|GetE_SpecialMoveType)
    (:NewEnumerator5
      (CallFunction|Uppercut))
    (:NewEnumerator6
      (CallFunction|Fireball))))

(event Custom|SpecialCooldown
  (if (not (Variables|Special|GetSpecialAvailable?))
    (bind _output_get (Variables|Special|SetCurrentCooldown (Math|Float|Clamp(Float) (- (Variables|Special|GetCurrentCooldown) 0.01) 0.0 (Variables|Special|GetMaxCooldown))))
    (if (<= _output_get 0.0)
      (Variables|Special|SetSpecialAvailable? true)
      (Variables|Special|SetCurrentCooldown (Variables|Special|GetMaxCooldown)))))

(event EventTick
  (params (DeltaSeconds :type Float%20%28single-precision%29))
  (CallFunction|SpecialCooldown))

(event EventBeginPlay
  (bind _asbp_first_person_character (Utilities|Casting|CastToBP_FirstPersonCharacter (Game|GetPlayerCharacter 0)))
  (Variables|Default|SetPlayerRef _asbp_first_person_character)
  (Variables|Special|SetSpecialAvailable? true)
  (Variables|Default|SetDamageType "/Game/RollingWithThePunches/Blueprints/DamageType/BP_DamageArms.BP_DamageArms_C"))

(fn ConstructionScript)

(fn HitObject
  (bind _playerref (Variables|Default|GetPlayerRef))
  (bind _firstpersoncamera (Variables|/Game/RollingWithThePunches/Blueprints/PlayerCharaacters/BP_FirstPersonCharacter.BP_FirstPersonCharacter_C|GetFirstPersonCamera _playerref))
  (bind _returnvalue (Transformation|GetWorldRotation _firstpersoncamera))
  (bind _returnvalue_2 (Transformation|GetWorldLocation _firstpersoncamera))
  (bind _returnvalue_3 (Math|Vector|GetForwardVector _returnvalue))
  (if (not (Variables|Punch|GetIsCharging?))
    (LocalVariables|SetPunchDirection _returnvalue_3)
    (bind _outhit (Collision|SphereTraceByChannel _returnvalue_2 (+ _returnvalue_2 (* _returnvalue_3 (Variables|Punch|GetPunchingRange))) 15.0 "TraceTypeQuery1" false 0 "None"))
    (if (.bBlockingHit (Collision|BreakHitResult _outhit))
      (Variables|Punch|SetImpact%20Point (.ImpactPoint (Collision|BreakHitResult _outhit)))
      (Punch|IdentifyTarget (.HitActor (Collision|BreakHitResult _outhit)) (.HitComponent (Collision|BreakHitResult _outhit)) (LocalVariables|GetPunchDirection)))))

(fn StartHitStop
  (params (Duration :type Float%20%28single-precision%29))
  (Variables|Default|SetCustomTimeDilation 0.0)
  (Utilities|Time|SetTimerbyFunctionName 0 "EndHitStop" Duration))

(fn EndHitStop
  (Variables|Default|SetCustomTimeDilation 1.0)
  (Utilities|Time|SetGlobalTimeDilation 1.0))

(fn HitBoulder
  (params (ActorComponent :type Primitive%20Component%20Object%20Reference) (HitActor :type Actor%20Object%20Reference) (PunchDirection :type Vector))
  (Audio|PlaySoundatLocation "/Game/RollingWithThePunches/Assets/Sounds/Ball/Ball1.Ball1" (Variables|Punch|GetImpact%20Point) "0, 0, 0" 1.0 1.0 0.0 0 0 0 0)
  (Audio|PlaySound2D (Utilities|Array|Get(acopy) (Variables|Default|GetHornSoundArray) (Variables|Punch|GetForceUnleashed)) 1.0 1.0 0.0 0 0)
  (Game|Damage|ApplyDamage HitActor 1.0 0 0 (Variables|Default|GetDamageType))
  (CallFunction|ActivateHitstop)
  (Physics|AddImpulseatLocation ActorComponent (* PunchDirection (Variables|Punch|GetPunchForce)) (Variables|Punch|GetImpact%20Point) "None")
  (Effects|SpawnEmitteratLocation "/Game/RollingWithThePunches/Assets/VFX/P_ComicBoom.P_ComicBoom" (Variables|Punch|GetImpact%20Point) "0, 0, 0" (Variables|Punch|GetImpactSize))
  (Game|SpawnActorfromClass "/Game/RollingWithThePunches/Blueprints/Actors/Effects/BP_PunchForceIndicator.BP_PunchForceIndicator_C" (Math|Transform|MakeTransform (Variables|Punch|GetImpact%20Point) "0, 0, 0" "1.000000,1.000000,1.000000") "Undefined" 0 0)
  (Variables|/Game/RollingWithThePunches/Blueprints/PlayerCharaacters/BP_FirstPersonCharacter.BP_FirstPersonCharacter_C|SetNumberOfPunches (Variables|Default|GetPlayerRef) (+ (Variables|/Game/RollingWithThePunches/Blueprints/PlayerCharaacters/BP_FirstPersonCharacter.BP_FirstPersonCharacter_C|GetNumberOfPunches (Variables|Default|GetPlayerRef)) 1))
  (Variables|Punch|SetPunchForce 2e+05))

(fn HitPhysicsObject
  (params (HitActor :type Actor%20Object%20Reference) (ActorComponent :type Primitive%20Component%20Object%20Reference) (PunchDirection :type Vector))
  (Game|Damage|ApplyDamage HitActor 1.0 0 0 (Variables|Default|GetDamageType))
  (CallFunction|StartHitStop (Variables|Default|GetHitStopDuration))
  (Physics|AddImpulseatLocation ActorComponent (* PunchDirection (Variables|Punch|GetPunchForce)) (Variables|Punch|GetImpact%20Point) "None")
  (Effects|SpawnEmitteratLocation "/Game/RollingWithThePunches/Assets/VFX/P_ComicBoom.P_ComicBoom" (Variables|Punch|GetImpact%20Point) "0, 0, 0" (Variables|Punch|GetImpactSize))
  (Game|SpawnActorfromClass "/Game/RollingWithThePunches/Blueprints/Actors/Effects/BP_PunchForceIndicator.BP_PunchForceIndicator_C" (Math|Transform|MakeTransform (Variables|Punch|GetImpact%20Point) "0, 0, 0" "1.000000,1.000000,1.000000") "Undefined" 0 0)
  (Variables|Punch|SetPunchForce 2e+05))

(fn HitSwitch
  (params (HitActor :type Actor%20Object%20Reference))
  (Game|Damage|ApplyDamage HitActor 1.0 0 0 (Variables|Default|GetDamageType))
  (CallFunction|StartHitStop (Variables|Default|GetHitStopDuration))
  (Effects|SpawnEmitteratLocation "/Game/RollingWithThePunches/Assets/VFX/P_ComicBoom.P_ComicBoom" (Variables|Punch|GetImpact%20Point) "0, 0, 0" (Variables|Punch|GetImpactSize))
  (Game|SpawnActorfromClass "/Game/RollingWithThePunches/Blueprints/Actors/Effects/BP_PunchForceIndicator.BP_PunchForceIndicator_C" (Math|Transform|MakeTransform (Variables|Punch|GetImpact%20Point) "0, 0, 0" "1.000000,1.000000,1.000000") "Undefined" 0 0)
  (Variables|Punch|SetPunchForce 2e+05))

(fn HitSecret
  (params (HitActor :type Actor%20Object%20Reference))
  (Game|Damage|ApplyDamage HitActor 1.0 0 0 (Variables|Default|GetDamageType))
  (CallFunction|StartHitStop (Variables|Default|GetHitStopDuration))
  (Effects|SpawnEmitteratLocation "/Game/RollingWithThePunches/Assets/VFX/P_ComicBoom.P_ComicBoom" (Variables|Punch|GetImpact%20Point) "0, 0, 0" (Variables|Punch|GetImpactSize))
  (Game|SpawnActorfromClass "/Game/RollingWithThePunches/Blueprints/Actors/Effects/BP_PunchForceIndicator.BP_PunchForceIndicator_C" (Math|Transform|MakeTransform (Variables|Punch|GetImpact%20Point) "0, 0, 0" "1.000000,1.000000,1.000000") "Undefined" 0 0)
  (Variables|Punch|SetPunchForce 2e+05))

(fn IdentifyTarget
  (params (HitActor :type Actor%20Object%20Reference) (ActorComponent :type Primitive%20Component%20Object%20Reference) (PunchDirection :type Vector))
  (if (Physics|IsSimulatingPhysics ActorComponent "None")
    (if (Components|ComponentHasTag ActorComponent "Boulder")
      (Punch|HitBoulder ActorComponent HitActor PunchDirection)
      (else
        (Punch|HitPhysicsObject HitActor ActorComponent PunchDirection)))
    (elif (Components|ComponentHasTag ActorComponent "Switch")
      (Punch|HitSwitch HitActor)
      (elif (Components|ComponentHasTag ActorComponent "Secret")
        (Punch|HitSecret HitActor)
        (elif (Components|ComponentHasTag ActorComponent "Enemy")
          (Punch|HitEnemy HitActor)
          (elif (Utilities|DoesObjectImplementInterface HitActor "/Game/RollingWithThePunches/Blueprints/Interface/BPI_Projectile.BPI_Projectile_C")
            (CallFunction|HitProjectile HitActor PunchDirection)
            (elif (Utilities|DoesObjectImplementInterface HitActor "/Game/RollingWithThePunches/Blueprints/Interface/BPI_Electricity.BPI_Electricity_C")
              (Class|BPIElectricity|RotateElectricalDevice(Message) HitActor)
              (else
                (CallFunction|LaunchPlayer)))))))))

(fn UppercutBoulder
  (params (ActorComponent :type Primitive%20Component%20Object%20Reference) (HitActor :type Actor%20Object%20Reference) (PunchDirection :type Vector))
  (Audio|PlaySoundatLocation "/Game/RollingWithThePunches/Assets/Sounds/Ball/Ball1.Ball1" (Variables|Punch|GetImpact%20Point) "0, 0, 0" 1.0 1.0 0.0 0 0 0 0)
  (Audio|PlaySound2D (Utilities|Array|Get(acopy) (Variables|Default|GetHornSoundArray) (Variables|Punch|GetForceUnleashed)) 1.0 1.0 0.0 0 0)
  (Game|Damage|ApplyDamage HitActor 1.0 0 0 (Variables|Default|GetDamageType))
  (CallFunction|ActivateHitstop)
  (Physics|AddImpulseatLocation ActorComponent (Math|Vector|MakeVector (.x (* PunchDirection (Variables|Punch|GetPunchForce))) (.y (* PunchDirection (Variables|Punch|GetPunchForce))) (+ (.z (* PunchDirection (Variables|Punch|GetPunchForce))) (* (Variables|Punch|GetPunchForce) (Variables|Uppercut|GetUppercutForce)))) (Variables|Punch|GetImpact%20Point) "None")
  (Effects|SpawnEmitteratLocation "/Game/RollingWithThePunches/Assets/VFX/P_ComicBoom.P_ComicBoom" (Variables|Punch|GetImpact%20Point) "0, 0, 0" (Variables|Punch|GetImpactSize))
  (Game|SpawnActorfromClass "/Game/RollingWithThePunches/Blueprints/Actors/Effects/BP_UppercutIndicator.BP_UppercutIndicator_C" (Math|Transform|MakeTransform (Variables|Punch|GetImpact%20Point) "0, 0, 0" "1.000000,1.000000,1.000000") "Undefined" 0 0)
  (Variables|/Game/RollingWithThePunches/Blueprints/PlayerCharaacters/BP_FirstPersonCharacter.BP_FirstPersonCharacter_C|SetNumberOfPunches (Variables|Default|GetPlayerRef) (+ (Variables|/Game/RollingWithThePunches/Blueprints/PlayerCharaacters/BP_FirstPersonCharacter.BP_FirstPersonCharacter_C|GetNumberOfPunches (Variables|Default|GetPlayerRef)) 1))
  (Variables|Punch|SetPunchForce 2e+05))

(fn UppercutObject
  (bind _playerref (Variables|Default|GetPlayerRef))
  (bind _firstpersoncamera (Variables|/Game/RollingWithThePunches/Blueprints/PlayerCharaacters/BP_FirstPersonCharacter.BP_FirstPersonCharacter_C|GetFirstPersonCamera _playerref))
  (bind _returnvalue (Transformation|GetWorldRotation _firstpersoncamera))
  (bind _returnvalue_2 (Transformation|GetWorldLocation _firstpersoncamera))
  (bind _returnvalue_3 (Math|Vector|GetForwardVector _returnvalue))
  (if (not (Variables|Punch|GetIsCharging?))
    (LocalVariables|SetPunchDirection _returnvalue_3)
    (bind _outhit (Collision|SphereTraceByChannel _returnvalue_2 (+ _returnvalue_2 (* _returnvalue_3 (Variables|Punch|GetPunchingRange))) 15.0 "TraceTypeQuery1" false 0 "None"))
    (if (.bBlockingHit (Collision|BreakHitResult _outhit))
      (Variables|Punch|SetImpact%20Point (.ImpactPoint (Collision|BreakHitResult _outhit)))
      (Uppercut|IdentifyUppercutTarget (.HitActor (Collision|BreakHitResult _outhit)) (.HitComponent (Collision|BreakHitResult _outhit)) (LocalVariables|GetPunchDirection)))))

(fn IdentifyUppercutTarget
  (params (HitActor :type Actor%20Object%20Reference) (ActorComponent :type Primitive%20Component%20Object%20Reference) (PunchDirection :type Vector))
  (if (Physics|IsSimulatingPhysics ActorComponent "None")
    (if (Components|ComponentHasTag ActorComponent "Boulder")
      (Uppercut|UppercutBoulder ActorComponent HitActor PunchDirection)
      (else
        (Uppercut|UppercutPhysicsObject HitActor ActorComponent PunchDirection)))
    (elif (Components|ComponentHasTag ActorComponent "Switch")
      (Punch|HitSwitch HitActor)
      (elif (Components|ComponentHasTag ActorComponent "Secret")
        (Punch|HitSecret HitActor)
        (elif (Components|ComponentHasTag ActorComponent "Enemy")
          (Punch|HitEnemy HitActor)
          (else
            (CallFunction|LaunchPlayer)))))))

(fn UppercutPhysicsObject
  (params (HitActor :type Actor%20Object%20Reference) (ActorComponent :type Primitive%20Component%20Object%20Reference) (PunchDirection :type Vector))
  (Game|Damage|ApplyDamage HitActor 1.0 0 0 (Variables|Default|GetDamageType))
  (CallFunction|StartHitStop (Variables|Default|GetHitStopDuration))
  (Physics|AddImpulseatLocation ActorComponent (Math|Vector|MakeVector (.x (* PunchDirection (Variables|Punch|GetPunchForce))) (.y (* PunchDirection (Variables|Punch|GetPunchForce))) (+ (.z (* PunchDirection (Variables|Punch|GetPunchForce))) (* (Variables|Punch|GetPunchForce) (Variables|Uppercut|GetUppercutForce)))) (Variables|Punch|GetImpact%20Point) "None")
  (Effects|SpawnEmitteratLocation "/Game/RollingWithThePunches/Assets/VFX/P_ComicBoom.P_ComicBoom" (Variables|Punch|GetImpact%20Point) "0, 0, 0" (Variables|Punch|GetImpactSize))
  (Game|SpawnActorfromClass "/Game/RollingWithThePunches/Blueprints/Actors/Effects/BP_UppercutIndicator.BP_UppercutIndicator_C" (Math|Transform|MakeTransform (Variables|Punch|GetImpact%20Point) "0, 0, 0" "1.000000,1.000000,1.000000") "Undefined" 0 0)
  (Variables|Punch|SetPunchForce 2e+05))

(fn SetSpecialCooldown
  (switch Utilities|FlowControl|Switch|SwitchonE_SpecialMove (Variables|Special|GetE_SpecialMoveType)
    (:NewEnumerator5
      (bind _output_get (Variables|Special|SetMaxCooldown 1.0))
      (Variables|Special|SetCurrentCooldown _output_get))
    (:NewEnumerator6
      (bind _output_get_2 (Variables|Special|SetMaxCooldown 2.5))
      (Variables|Special|SetCurrentCooldown _output_get_2))
    (:NewEnumerator7
      (bind _output_get_3 (Variables|Special|SetMaxCooldown 2.0))
      (Variables|Special|SetCurrentCooldown _output_get_3))
    (:NewEnumerator8
      (bind _output_get_4 (Variables|Special|SetMaxCooldown 2.5))
      (Variables|Special|SetCurrentCooldown _output_get_4))))

(fn LaunchPlayer
  (bind _playerref (Variables|Default|GetPlayerRef))
  (bind _forceunleashed (Variables|Punch|GetForceUnleashed))
  (bind _returnvalue (* _forceunleashed -1.1e+02))
  (bind _firstpersoncamera (Variables|/Game/RollingWithThePunches/Blueprints/PlayerCharaacters/BP_FirstPersonCharacter.BP_FirstPersonCharacter_C|GetFirstPersonCamera _playerref))
  (bind _returnvalue_2 (Transformation|GetWorldRotation _firstpersoncamera))
  (bind _returnvalue_3 (Math|Vector|GetForwardVector _returnvalue_2))
  (bind _returnvalue_4 (* _returnvalue_3 _returnvalue))
  (Utilities|FlowControl|Sequence
    (:then_0
      (Character|LaunchCharacter (Variables|Default|GetPlayerRef) (Math|Vector|MakeVector (.x _returnvalue_4) (.y _returnvalue_4) (+ (.z _returnvalue_4) 1e+03)) false false)
      (Effects|SpawnEmitteratLocation "/Game/RollingWithThePunches/Assets/VFX/P_ComicBoom.P_ComicBoom" (Variables|Punch|GetImpact%20Point) "0, 0, 0" (Variables|Punch|GetImpactSize))
      (Game|SpawnActorfromClass "/Game/RollingWithThePunches/Blueprints/Actors/Effects/BP_PunchForceIndicator.BP_PunchForceIndicator_C" (Math|Transform|MakeTransform (Variables|Punch|GetImpact%20Point) "0, 0, 0" "1.000000,1.000000,1.000000") "Undefined" 0 0)
      (Variables|Punch|SetPunchForce 2e+05))
    (:then_1
      (Audio|PlaySound2D (Utilities|Array|Get(acopy) (Variables|Default|GetHornSoundArray) (Variables|Punch|GetForceUnleashed)) 1.0 1.0 0.0 0 0)
      (CallFunction|ActivateHitstop))))

(fn HitEnemy
  (params (HitActor :type Actor%20Object%20Reference))
  (bind _asbp_enemy_parent (Utilities|Casting|CastToBP_EnemyParent HitActor))
  (Variables|/Game/RollingWithThePunches/Blueprints/Actors/Obstacles/Enemies/BP_EnemyParent.BP_EnemyParent_C|SetStun? _asbp_enemy_parent true)
  (Default|BeginEnemyLogic _asbp_enemy_parent))

(fn HitProjectile
  (params (HitActor :type Actor%20Object%20Reference) (PunchDirection :type Vector))
  (Audio|PlaySound2D (Utilities|Array|Get(acopy) (Variables|Default|GetHornSoundArray) (Variables|Punch|GetForceUnleashed)) 1.0 1.0 0.0 0 0)
  (Class|BPIProjectile|ActivateProjectileAction(Message) HitActor (Variables|Punch|GetForceUnleashed) PunchDirection)
  (CallFunction|ActivateHitstop)
  (Effects|SpawnEmitteratLocation "/Game/RollingWithThePunches/Assets/VFX/P_ComicBoom.P_ComicBoom" (Variables|Punch|GetImpact%20Point) "0, 0, 0" (Variables|Punch|GetImpactSize))
  (Game|SpawnActorfromClass "/Game/RollingWithThePunches/Blueprints/Actors/Effects/BP_PunchForceIndicator.BP_PunchForceIndicator_C" (Math|Transform|MakeTransform (Variables|Punch|GetImpact%20Point) "0, 0, 0" "1.000000,1.000000,1.000000") "Undefined" 0 0)
  (Variables|Punch|SetPunchForce 2e+05))