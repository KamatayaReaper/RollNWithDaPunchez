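; BP_SignWall is a hub actor, a signpost that shows a direction widget when the level-select player comes near.
; On BeginPlay it applies the SignColor material to its static mesh and cone.
; A sphere trigger shows the DirectionWidget when a BP_LevelSelectPlayer begins overlapping and hides it when the overlap ends.
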(event OnComponentBeginOverlap(Sphere)
  (params (OverlappedComponent :type Primitive%20Component%20Object%20Reference) (OtherActor :type Actor%20Object%20Reference) (OtherComp :type Primitive%20Component%20Object%20Reference) (OtherBodyIndex :type Integer) (bFromSweep :type Boolean) (SweepResult :type Hit%20Result%20Structure%20%28by%20ref%29))
  (Utilities|Casting|CastToBP_LevelSelectPlayer OtherActor)
  (Rendering|SetVisibility (Variables|Default|GetDirectionWidget) true false))

(event OnComponentEndOverlap(Sphere)
  (params (OverlappedComponent :type Primitive%20Component%20Object%20Reference) (OtherActor :type Actor%20Object%20Reference) (OtherComp :type Primitive%20Component%20Object%20Reference) (OtherBodyIndex :type Integer))
  (Utilities|Casting|CastToBP_LevelSelectPlayer OtherActor)
  (Rendering|SetVisibility (Variables|Default|GetDirectionWidget) false false))

(event EventBeginPlay
  (Rendering|Material|SetMaterial (Variables|Default|GetStaticMesh) 0 (Variables|Default|GetSignColor))
  (Rendering|Material|SetMaterial (Variables|Default|GetCone) 0 (Variables|Default|GetSignColor)))

(event Collision|EventActorBeginOverlap
  (params (OtherActor :type Actor%20Object%20Reference)))

(event EventTick
  (params (DeltaSeconds :type Float%20%28single-precision%29)))

(fn ConstructionScript)