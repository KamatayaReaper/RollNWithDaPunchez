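; Level-select platform in the hub that represents one level and opens its setup menu.
; On BeginPlay it colors its cylinder green or red by whether a save slot named after the level exists, and applies a level-number decal.
; Sphere overlap by the level-select player adjusts camera zoom and toggles an interact prompt.
; Interact passes level details to the setup menu, pauses the game and enables mouse input; direct level-loading logic is left unconnected.
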(event OnComponentBeginOverlap(Sphere)
  (params (OverlappedComponent :type Primitive%20Component%20Object%20Reference) (OtherActor :type Actor%20Object%20Reference) (OtherComp :type Primitive%20Component%20Object%20Reference) (OtherBodyIndex :type Integer) (bFromSweep :type Boolean) (SweepResult :type Hit%20Result%20Structure%20%28by%20ref%29))
  (bind _asbp_level_select_player (Utilities|Casting|CastToBP_LevelSelectPlayer OtherActor))
  (Default|ZoomCamerain _asbp_level_select_player)
  (Rendering|SetVisibility (Variables|Default|GetInteractWidget) true false))

(event OnComponentEndOverlap(Sphere)
  (params (OverlappedComponent :type Primitive%20Component%20Object%20Reference) (OtherActor :type Actor%20Object%20Reference) (OtherComp :type Primitive%20Component%20Object%20Reference) (OtherBodyIndex :type Integer))
  (bind _asbp_level_select_player (Utilities|Casting|CastToBP_LevelSelectPlayer OtherActor))
  (Default|ZoomCameraBack(In) _asbp_level_select_player)
  (Rendering|SetVisibility (Variables|Default|GetInteractWidget) false false))

(event EventBeginPlay
  (Utilities|FlowControl|Sequence
    (:then_1
      (CallFunction|SetLevelData))))

(event EventInteract
  (bind _returnvalue (Game|GetPlayerController 0))
  (Utilities|FlowControl|Sequence
    (:then_0
      (bind _returnvalue_2 (UserInterface|CreateWidget "/Game/RollingWithThePunches/Blueprints/HUDs/Menu/LevelSetup/LevelSetupMenu_HUD.LevelSetupMenu_HUD_C"))
      (UserInterface|Viewport|AddtoViewport _returnvalue_2 0)
      (Variables|/Game/RollingWithThePunches/Blueprints/HUDs/LevelInfo/LevelInfo_HUD_V3.LevelInfo_HUD_V3_C|SetLevelLabel (Variables|/Game/RollingWithThePunches/Blueprints/HUDs/Menu/LevelSetup/LevelSetupMenu_HUD.LevelSetupMenu_HUD_C|GetLevelInfo_HUD_V3 _returnvalue_2) (Variables|Default|GetLevelLabel))
      (Variables|/Game/RollingWithThePunches/Blueprints/HUDs/LevelInfo/LevelInfo_HUD_V3.LevelInfo_HUD_V3_C|SetLevel_Mat (Variables|/Game/RollingWithThePunches/Blueprints/HUDs/Menu/LevelSetup/LevelSetupMenu_HUD.LevelSetupMenu_HUD_C|GetLevelInfo_HUD_V3 _returnvalue_2) (Variables|Default|GetLevelPreviewImage))
      (Variables|/Game/RollingWithThePunches/Blueprints/HUDs/LevelInfo/LevelInfo_HUD_V3.LevelInfo_HUD_V3_C|SetNameLevel (Variables|/Game/RollingWithThePunches/Blueprints/HUDs/Menu/LevelSetup/LevelSetupMenu_HUD.LevelSetupMenu_HUD_C|GetLevelInfo_HUD_V3 _returnvalue_2) (Variables|Default|GetLevelName))
      (Rendering|SetVisibility (Variables|Default|GetInteractWidget) false false))
    (:then_1
      (Game|SetGamePaused true)
      (Variables|/Script/Engine.PlayerController|SetbShowMouseCursor _returnvalue true)
      (Input|SetInputModeGameandUI _returnvalue 0 "LockInFullscreen" true))))

(fn ConstructionScript)

(fn SetLevelData
  (bind _cylinder (Variables|Default|GetCylinder))
  (Utilities|FlowControl|Sequence
    (:then_0
      (bind _returnvalue (SaveGame|DoesSaveGameExist (Utilities|String|ToString(Name) (Variables|Default|GetLevelName))))
      (if _returnvalue
        (Rendering|Material|SetMaterial _cylinder 0 "/Game/RollingWithThePunches/Blockmesh/Materials/Solid_Colors/Solid_Green.Solid_Green")
        (else
          (Rendering|Material|SetMaterial _cylinder 0 "/Game/RollingWithThePunches/Blockmesh/Materials/Solid_Colors/Solid_Red.Solid_Red")))
      (Development|PrintString ""))
    (:then_1
      (Rendering|Components|Decal|SetDecalMaterial (Variables|Default|GetDecal) (Utilities|Array|Get(acopy) (Variables|Default|GetNumberDecalMaterial) (Variables|Default|GetLevelNumber))))))