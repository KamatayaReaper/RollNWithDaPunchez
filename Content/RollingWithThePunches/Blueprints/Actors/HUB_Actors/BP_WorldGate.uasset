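; BP_WorldGate is a hub-world gate that opens for the level-select player once enough levels are completed.
; A box overlap shows a WorldGateHUD widget displaying the required level count and hides it on exit.
; On Interact it compares the player's completed levels to the requirement, then plays a sound, lowers the gate mesh via a timeline and destroys itself.
; The construction script applies a configurable decal scale.
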(event OnComponentBeginOverlap(Box)
  (params (OverlappedComponent :type Primitive%20Component%20Object%20Reference) (OtherActor :type Actor%20Object%20Reference) (OtherComp :type Primitive%20Component%20Object%20Reference) (OtherBodyIndex :type Integer) (bFromSweep :type Boolean) (SweepResult :type Hit%20Result%20Structure%20%28by%20ref%29))
  (bind _asbp_level_select_player (Utilities|Casting|CastToBP_LevelSelectPlayer OtherActor))
  (Rendering|SetVisibility (Variables|Default|GetWidget) true false))

(event OnComponentEndOverlap(Box)
  (params (OverlappedComponent :type Primitive%20Component%20Object%20Reference) (OtherActor :type Actor%20Object%20Reference) (OtherComp :type Primitive%20Component%20Object%20Reference) (OtherBodyIndex :type Integer))
  (Utilities|Casting|CastToBP_LevelSelectPlayer OtherActor)
  (Rendering|SetVisibility (Variables|Default|GetWidget) false false))

(event EventBeginPlay
  (bind _asworld_gate_hud (Utilities|Casting|CastToWorldGateHUD (UserInterface|GetWidget (Variables|Default|GetWidget))))
  (Variables|/Game/RollingWithThePunches/Blueprints/HUDs/WorldGateHUD.WorldGateHUD_C|SetLevelsRequired _asworld_gate_hud (Variables|Default|GetLevelsRequired)))

(event Collision|EventActorBeginOverlap
  (params (OtherActor :type Actor%20Object%20Reference)))

(event EventTick
  (params (DeltaSeconds :type Float%20%28single-precision%29)))

(event EventInteract
  (if (>= (Variables|/Game/RollingWithThePunches/Blueprints/PlayerCharaacters/BP_LevelSelectPlayer.BP_LevelSelectPlayer_C|GetLevelsCompleted (stale OnComponentBeginOverlap(Box) _asbp_level_select_player)) (Variables|Default|GetLevelsRequired))
    (Audio|PlaySoundatLocation "/Game/RollingWithThePunches/Assets/Sounds/SlidingDoor.SlidingDoor" (Transformation|GetActorLocation) "0, 0, 0" 1.0 1.0 0.0 0 0 0 0)
    (bind _openalpha (Timeline|OpenGate Play)
      (:Update
        (Transformation|SetRelativeLocation (Variables|Default|GetCube) (Math|Vector|Lerp(Vector) "0, 0, 0" "0, 0,-450.000000" _openalpha) false false))
      (:Finished
        (Utilities|FlowControl|Delay 0.2)
        (Actor|DestroyActor)))))

(fn ConstructionScript
  (Transformation|SetRelativeScale3D (Variables|Default|GetDecal) (Variables|Default|GetDecalScale)))