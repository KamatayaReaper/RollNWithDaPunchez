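; Secret boombox actor, filed as obsolete, that simulates physics and plays a song once the level begins.
; On BeginPlay it creates an audio component at runtime, plays a tuning-in sound, then starts the music after a fixed delay.
; Without waiting for that delay, it hands its horn sound array to the first-person character and shows a song-name HUD widget.
; Any damage fades the music out.
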(event EventBeginPlay
  (|CallParentFunction)
  (Utilities|FlowControl|Sequence
    (:then_0
      (Physics|SetSimulatePhysics (Variables|Default|GetStaticMesh) true))
    (:then_1
      (bind _returnvalue (AddComponent|AddAudioComponent false))
      (Audio|Components|Audio|SetSound _returnvalue (Variables|Default|GetBoomboxMusic))
      (Variables|Default|SetBoomboxAudioComponent _returnvalue))
    (:then_2
      (Audio|PlaySound2D "/Game/RollingWithThePunches/Assets/Sounds/TuningIn.TuningIn" 1.0 1.0 0.0 0 0)
      (Utilities|FlowControl|Delay 9.0)
      (Audio|Components|Audio|Play (Variables|Default|GetBoomboxAudioComponent) 0.0))
    (:then_3
      (bind _asbp_first_person_character (Utilities|Casting|CastToBP_FirstPersonCharacter (Game|GetPlayerCharacter 0)))
      (bind _output_get (Variables|Default|SetPlayerRef _asbp_first_person_character))
      (Variables|/Game/RollingWithThePunches/Blueprints/PlayerCharaacters/BP_FirstPersonCharacter.BP_FirstPersonCharacter_C|SetLevel%20Horn%20Sound%20Array _output_get (Variables|Default|GetLevel%20Horn%20Sound%20Array))
      (Default|SetArmHornArray (Variables|Default|GetPlayerRef)))
    (:then_4
      (bind _returnvalue_2 (UserInterface|CreateWidget "/Game/RollingWithThePunches/Blueprints/HUDs/PlayMusic_HUD.PlayMusic_HUD_C"))
      (Variables|/Game/RollingWithThePunches/Blueprints/HUDs/PlayMusic_HUD.PlayMusic_HUD_C|SetSong_Name _returnvalue_2 (Variables|Default|GetSong%20Name))
      (UserInterface|Viewport|AddtoViewport _returnvalue_2 0))))

(event Collision|EventActorBeginOverlap
  (params (OtherActor :type Actor%20Object%20Reference))
  (|CallParentFunction OtherActor) ; This node is disabled and will not be called.\nDrag off pins to build functionality.
)

(event EventTick
  (params (DeltaSeconds :type Float%20%28single-precision%29))
  (|CallParentFunction DeltaSeconds) ; This node is disabled and will not be called.\nDrag off pins to build functionality.
)

(event Game|Damage|EventAnyDamage
  (params (Damage :type Float%20%28single-precision%29) (DamageType :type Damage%20Type%20Object%20Reference) (InstigatedBy :type Controller%20Object%20Reference) (DamageCauser :type Actor%20Object%20Reference))
  (Audio|Components|Audio|FadeOut (Variables|Default|GetBoomboxAudioComponent) 0.2 0.0 "Linear" :!class /Script/Engine.AudioComponent))

(fn ConstructionScript
  (|CallParentFunction))