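; BP_MuffleMusicZone is a trigger volume that quiets the secret turntable's boombox music while the player is inside it.
; On BeginPlay it caches the first-person player character, then on begin and end overlap fades the referenced TurntableSecret's audio component down to low volume and back to full with a short linear AdjustVolume.
; The construction script sizes the box from a BoxRange variable.
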(event EventBeginPlay
  (bind _asbp_first_person_character (Utilities|Casting|CastToBP_FirstPersonCharacter (Game|GetPlayerCharacter 0)))
  (Variables|Default|SetPlayerRef _asbp_first_person_character))

(event Collision|EventActorBeginOverlap
  (params (OtherActor :type Actor%20Object%20Reference))
  (if (== OtherActor (Variables|Default|GetPlayerRef))
    (Audio|Components|Audio|AdjustVolume (Variables|/Game/RollingWithThePunches/Blueprints/Actors/Secret/BP_TurntableSecret.BP_TurntableSecret_C|GetBoomboxAudioComponent (Variables|Default|GetTurntableSecretRef)) 0.2 0.2 "Linear" :!class /Script/Engine.AudioComponent)))

(event Collision|EventActorEndOverlap
  (params (OtherActor :type Actor%20Object%20Reference))
  (if (== OtherActor (Variables|Default|GetPlayerRef))
    (Audio|Components|Audio|AdjustVolume (Variables|/Game/RollingWithThePunches/Blueprints/Actors/Secret/BP_TurntableSecret.BP_TurntableSecret_C|GetBoomboxAudioComponent (Variables|Default|GetTurntableSecretRef)) 0.2 1.0 "Linear" :!class /Script/Engine.AudioComponent)))

(fn ConstructionScript
  (Components|Box|SetBoxExtent (Variables|Default|GetBox) (Variables|Default|GetBoxRange) true))