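; Secret unlockable actor that grants either a boulder character or a special move, as set by IsBoulder.
; BeginPlay caches the player and pre-creates an unlock notification widget.
; Unlock briefly flashes the mesh material, plays a sound and shows the widget with the unlock's symbol and a display name mapped from its type enum.
; After a short delay it saves the unlock to the matching roster through the player's game instance reference.
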(event EventBeginPlay
  (bind _asbp_first_person_character (Utilities|Casting|CastToBP_FirstPersonCharacter (Game|GetPlayerCharacter 0)))
  (Variables|Default|SetPlayerRef _asbp_first_person_character)
  (bind _returnvalue (UserInterface|CreateWidget "/Game/RollingWithThePunches/Blueprints/HUDs/Effect_HUDs/Notifications/Unlock_NotificationHUD.Unlock_NotificationHUD_C"))
  (Variables|Default|SetUnlockNotificationRef _returnvalue))

(event EventUnlock
  (bind _unlocknotificationref (Variables|Default|GetUnlockNotificationRef))
  (Utilities|FlowControl|Sequence
    (:then_0
      (Rendering|Material|SetMaterial (Variables|Default|GetStaticMesh) 1 "/Game/RollingWithThePunches/Blockmesh/Materials/Emmissive/MI_EM_White.MI_EM_White")
      (Utilities|FlowControl|Delay 0.2)
      (Rendering|Material|SetMaterial (Variables|Default|GetStaticMesh) 1 "/Game/RollingWithThePunches/Blockmesh/Materials/Metal/Solid_Black_Metal.Solid_Black_Metal"))
    (:then_1
      (if (Variables|Default|GetIsBoulder?)
        (CallFunction|SetBoulder)
        (Variables|/Game/RollingWithThePunches/Blueprints/HUDs/Effect_HUDs/Notifications/Unlock_NotificationHUD.Unlock_NotificationHUD_C|SetUnlockedContent (Variables|Default|GetUnlockNotificationRef) (Variables|Default|GetBoulderSaved))
        (else
          (CallFunction|SetSpecial)
          (Variables|/Game/RollingWithThePunches/Blueprints/HUDs/Effect_HUDs/Notifications/Unlock_NotificationHUD.Unlock_NotificationHUD_C|SetUnlockedContent (Variables|Default|GetUnlockNotificationRef) (Variables|Default|GetSpecialSaved?))))
      (Variables|/Game/RollingWithThePunches/Blueprints/HUDs/Effect_HUDs/Notifications/Unlock_NotificationHUD.Unlock_NotificationHUD_C|SetUnlockSymbolImage (Variables|Default|GetUnlockNotificationRef) (Variables|Default|GetUnlock%20Symbol%20Image))
      (if (not (UserInterface|Viewport|IsinViewport _unlocknotificationref))
        (UserInterface|Viewport|AddtoViewport _unlocknotificationref 0)))
    (:then_2
      (Utilities|FlowControl|Delay 0.2)
      (if (Variables|Default|GetIsBoulder?)
        (Default|SaveBoulderRoster (Variables|/Game/RollingWithThePunches/Blueprints/PlayerCharaacters/BP_FirstPersonCharacter.BP_FirstPersonCharacter_C|GetGameInstanceRef (Variables|Default|GetPlayerRef)) (Variables|Default|GetBoulderType))
        (else
          (Default|SaveSpecialRoster (Variables|/Game/RollingWithThePunches/Blueprints/PlayerCharaacters/BP_FirstPersonCharacter.BP_FirstPersonCharacter_C|GetGameInstanceRef (Variables|Default|GetPlayerRef)) (Variables|Default|GetSpecialType)))))
    (:then_3
      (Audio|PlaySoundatLocation "/Game/RollingWithThePunches/Assets/Sounds/UnloockableOpen.UnloockableOpen" (Transformation|GetWorldLocation (Variables|Default|GetStaticMesh)) "0, 0, 0" 1.0 1.0 0.0 0 0 0 0))))

(fn ConstructionScript)

(fn SetBoulder
  (switch Utilities|FlowControl|Switch|SwitchonE_BoulderType (Variables|Default|GetBoulderType)
    (:NewEnumerator0
      (Variables|Default|SetBoulderSaved "CRAZY FACE"))
    (:NewEnumerator1
      (Variables|Default|SetBoulderSaved "WUV DUV"))
    (:NewEnumerator2
      (Variables|Default|SetBoulderSaved "GRRR"))
    (:NewEnumerator4
      (Variables|Default|SetBoulderSaved "MUNCH LUNCH"))
    (:NewEnumerator7
      (Variables|Default|SetBoulderSaved "D-PRESS"))
    (:NewEnumerator6
      (Variables|Default|SetBoulderSaved "BABY FACE"))
    (:NewEnumerator5
      (Variables|Default|SetBoulderSaved "JACK ATTACK"))
    (:NewEnumerator3
      (Variables|Default|SetBoulderSaved "DOOM BOOM"))
    (:NewEnumerator8
      (Variables|Default|SetBoulderSaved "SMUG LUG"))
    (:NewEnumerator9
      (Variables|Default|SetBoulderSaved "NINJAJA"))
    (:NewEnumerator11
      (Variables|Default|SetBoulderSaved "DOO-D-G"))
    (:NewEnumerator13
      (Variables|Default|SetBoulderSaved "JELLY BELLE"))
    (:NewEnumerator12
      (Variables|Default|SetBoulderSaved "ITA NIMU"))
    (:NewEnumerator14
      (Variables|Default|SetBoulderSaved "G-ZONE"))
    (:NewEnumerator10
      (Variables|Default|SetBoulderSaved "DOMOGATO"))
    (:NewEnumerator15
      (Variables|Default|SetBoulderSaved "QTB"))
    (:NewEnumerator16
      (Variables|Default|SetBoulderSaved "HUMP DUMP"))
    (:NewEnumerator17
      (Variables|Default|SetBoulderSaved "GLOU-CHESTER"))
    (:NewEnumerator18
      (Variables|Default|SetBoulderSaved "JAWR"))
    (:NewEnumerator19
      (Variables|Default|SetBoulderSaved "MEE-BA"))
    (:NewEnumerator20
      (Variables|Default|SetBoulderSaved "BOB CRASHLEY"))
    (:NewEnumerator21
      (Variables|Default|SetBoulderSaved "KARAT HEAD"))
    (:NewEnumerator22
      (Variables|Default|SetBoulderSaved "OKI-DOKI"))
    (:NewEnumerator23
      (Variables|Default|SetBoulderSaved "GOOGLES"))
    (:NewEnumerator24
      (Variables|Default|SetBoulderSaved "GO-Z"))
    (:NewEnumerator25
      (Variables|Default|SetBoulderSaved "FRANK-E"))
    (:NewEnumerator26
      (Variables|Default|SetBoulderSaved "SLING"))
    (:NewEnumerator27
      (Variables|Default|SetBoulderSaved "OJO"))
    (:NewEnumerator28
      (Variables|Default|SetBoulderSaved "CRACK-A-CHACK"))
    (:NewEnumerator29
      (Variables|Default|SetBoulderSaved "GRIMM"))
    (:NewEnumerator30
      (Variables|Default|SetBoulderSaved "FOO-GOO"))
    (:NewEnumerator31
      (Variables|Default|SetBoulderSaved "SAGUARO"))
    (:NewEnumerator32
      (Variables|Default|SetBoulderSaved "IRON HEDD"))
    (:NewEnumerator33
      (Variables|Default|SetBoulderSaved "MOLON"))
    (:NewEnumerator34
      (Variables|Default|SetBoulderSaved "TAB-TAB"))
    (:NewEnumerator35
      (Variables|Default|SetBoulderSaved "PSYCHO FACE"))))

(fn SetSpecial
  (switch Utilities|FlowControl|Switch|SwitchonE_SpecialMove (Variables|Default|GetSpecialType)
    (:NewEnumerator4
      (Variables|Default|SetSpecialSaved? ""))
    (:NewEnumerator5
      (Variables|Default|SetSpecialSaved? "UPPERCUT"))
    (:NewEnumerator6
      (Variables|Default|SetSpecialSaved? "MISSILE"))
    (:NewEnumerator7
      (Variables|Default|SetSpecialSaved? "GRAPPLE"))
    (:NewEnumerator8
      (Variables|Default|SetSpecialSaved? "PLATFORM"))
    (:NewEnumerator10
      (Variables|Default|SetSpecialSaved? "FREEZE"))
    (:NewEnumerator11
      (Variables|Default|SetSpecialSaved? "ULTRA PUNCH"))
    (:NewEnumerator12
      (Variables|Default|SetSpecialSaved? "TELEPORT"))
    (:NewEnumerator13
      (Variables|Default|SetSpecialSaved? "WALL"))
    (:NewEnumerator14
      (Variables|Default|SetSpecialSaved? "DASH"))
    (:NewEnumerator15
      (Variables|Default|SetSpecialSaved? "DUMMY"))))