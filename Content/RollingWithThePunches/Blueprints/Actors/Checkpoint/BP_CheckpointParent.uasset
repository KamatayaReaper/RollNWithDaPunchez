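; Checkpoint parent actor that sets a new boulder spawn point when a boulder that has not just spawned overlaps it.
; Activation shows a HUD widget, plays a sound and fires a do-once effect that hides the root and spawns an effect actor.
; Reusable checkpoints reappear and re-arm after a delay, while others destroy themselves.
; The player character overlapping it instead triggers an error buzz and a notification widget.
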(event Custom|CheckpointFX
  (Utilities|FlowControl|DoOnce false
    (:Completed
      (Rendering|SetVisibility (Variables|Default|GetDefaultSceneRoot) false false)
      (Game|SpawnActorfromClass "/Game/RollingWithThePunches/Blueprints/Actors/Effects/CheckPointEffectActor.CheckPointEffectActor_C" (Math|Transform|MakeTransform (Transformation|GetWorldLocation (Variables|Default|GetSpawnPoint)) "0, 0,90.000000" "1.000000,1.000000,1.000000") "Undefined" 0 0))))

(event EventBeginPlay
  (bind _asbp_first_person_character (Utilities|Casting|CastToBP_FirstPersonCharacter (Game|GetPlayerCharacter 0)))
  (Variables|Default|SetPlayerRef _asbp_first_person_character))

(event Collision|EventActorBeginOverlap
  (params (OtherActor :type Actor%20Object%20Reference))
  (Utilities|FlowControl|Sequence
    (:then_0
      (bind _asbp_boulder_parent (Utilities|Casting|CastToBP_BoulderParent OtherActor))
      (Utilities|FlowControl|Delay 0.5)
      (Utilities|FlowControl|DoOnce false :!label _label
        (:Completed
          (if (not (Variables|/Game/RollingWithThePunches/Blueprints/Actors/Boulders/BP_BoulderParent.BP_BoulderParent_C|GetJustSpawned? _asbp_boulder_parent))
            (Utilities|FlowControl|Sequence
              (:then_0
                (Default|SetNewBoulderSpawn _asbp_boulder_parent (Transformation|GetWorldLocation (Variables|Default|GetSpawnPoint)))
                (if (Variables|Default|GetReusable?)
                  (CallFunction|CheckpointFX)
                  (Utilities|FlowControl|Delay 1e+01)
                  (Utilities|FlowControl|Sequence
                    (:then_0
                      (Rendering|SetVisibility (Variables|Default|GetDefaultSceneRoot) true false)
                      (goto _label Reset))
                    (:then_1
                      (Utilities|FlowControl|DoOnce false) ; enters at Reset
                    ))
                  (else
                    (CallFunction|CheckpointFX)
                    (Utilities|FlowControl|Delay 0.2)
                    (Actor|DestroyActor))))
              (:then_1
                (bind _returnvalue (UserInterface|CreateWidget "/Game/RollingWithThePunches/Blueprints/HUDs/Effect_HUDs/Notifications/CheckpointSet_HUD.CheckpointSet_HUD_C"))
                (UserInterface|Viewport|AddtoViewport _returnvalue 0))
              (:then_2
                (Audio|PlaySoundatLocation "/Game/Interface_And_Item_Sounds/WAV/Futuristic_Click_02.Futuristic_Click_02" (Transformation|GetActorLocation) "0, 0, 0" 1.0 1.0 0.0 0 0 0 0)))))))
    (:then_1
      (if (== OtherActor (Variables|Default|GetPlayerRef))
        (bind _returnvalue_2 (UserInterface|CreateWidget "/Game/RollingWithThePunches/Blueprints/HUDs/Effect_HUDs/Notifications/Checkpoint_NotificationHUD.Checkpoint_NotificationHUD_C"))
        (if (not (UserInterface|Viewport|IsinViewport _returnvalue_2))
          (Audio|PlaySoundatLocation "/Game/Interface_And_Item_Sounds/WAV/Error_Buzz_04.Error_Buzz_04" (Transformation|GetActorLocation) "0, 0, 0" 1.0 1.0 0.0 0 0 0 0)
          (UserInterface|Viewport|AddtoViewport _returnvalue_2 0))))))

(event EventTick
  (params (DeltaSeconds :type Float%20%28single-precision%29)))

(fn ConstructionScript)