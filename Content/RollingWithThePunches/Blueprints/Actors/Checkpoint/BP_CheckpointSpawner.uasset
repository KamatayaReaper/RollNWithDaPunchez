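; Spawner actor that places a checkpoint in the level when the player character has checkpoints enabled.
; On BeginPlay it caches the first-person player character and calls SpawnCheckpoint if that character's CheckpointsOn flag is set.
; SpawnCheckpoint rechecks the flag, then spawns either a reusable or a disposable checkpoint at the SpawnRef location, chosen by the ReusableCheckpoint boolean.
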(event Custom|SpawnCheckpoint
  (if (Variables|/Game/RollingWithThePunches/Blueprints/PlayerCharaacters/BP_FirstPersonCharacter.BP_FirstPersonCharacter_C|GetCheckpointsOn? (Variables|Default|GetPlayerRef))
    (if (Variables|Default|GetReusableCheckpoint?)
      (Game|SpawnActorfromClass "/Game/RollingWithThePunches/Blueprints/Actors/Checkpoint/BP_ReusableCheckpoint.BP_ReusableCheckpoint_C" (Math|Transform|MakeTransform (Transformation|GetWorldLocation (Variables|Default|GetSpawnRef)) "0, 0, 0" "1.000000,1.000000,1.000000") "Undefined" 0 0)
      (else
        (Game|SpawnActorfromClass "/Game/RollingWithThePunches/Blueprints/Actors/Checkpoint/BP_DisposableCheckpoint.BP_DisposableCheckpoint_C" (Math|Transform|MakeTransform (Transformation|GetWorldLocation (Variables|Default|GetSpawnRef)) "0, 0, 0" "1.000000,1.000000,1.000000") "Undefined" 0 0)))))

(event EventBeginPlay
  (bind _asbp_first_person_character (Utilities|Casting|CastToBP_FirstPersonCharacter (Game|GetPlayerCharacter 0)))
  (bind _output_get (Variables|Default|SetPlayerRef _asbp_first_person_character))
  (if (Variables|/Game/RollingWithThePunches/Blueprints/PlayerCharaacters/BP_FirstPersonCharacter.BP_FirstPersonCharacter_C|GetCheckpointsOn? _output_get)
    (CallFunction|SpawnCheckpoint)))

(fn ConstructionScript)