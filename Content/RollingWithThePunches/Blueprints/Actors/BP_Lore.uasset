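; BP_Lore is an actor that shows a lore entry on screen when unlocked.
; On BeginPlay it creates a Lore_HUD widget and fills it with the instance's title, three texts, image and per-text font sizes.
; Unlock works once: it briefly flashes the mesh material white, restores black metal, then adds the widget to the viewport just afterwards.
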(event EventBeginPlay
  (bind _asbp_first_person_character (Utilities|Casting|CastToBP_FirstPersonCharacter (Game|GetPlayerCharacter 0)))
  (Variables|Default|SetPlayerRef _asbp_first_person_character)
  (Variables|Default|SetLoreOpened? false)
  (bind _returnvalue (UserInterface|CreateWidget "/Game/RollingWithThePunches/Blueprints/HUDs/Unlockables/Lore_HUD.Lore_HUD_C"))
  (bind _output_get (Variables|Default|SetLoreHUD_Ref _returnvalue))
  (Variables|/Game/RollingWithThePunches/Blueprints/HUDs/Unlockables/Lore_HUD.Lore_HUD_C|SetLoreTitle _output_get (Variables|Default|GetLore%20Title))
  (Variables|/Game/RollingWithThePunches/Blueprints/HUDs/Unlockables/Lore_HUD.Lore_HUD_C|SetLore1 (Variables|Default|GetLoreHUD_Ref) (Variables|Default|GetLore1))
  (Variables|/Game/RollingWithThePunches/Blueprints/HUDs/Unlockables/Lore_HUD.Lore_HUD_C|SetLore2 (Variables|Default|GetLoreHUD_Ref) (Variables|Default|GetLore%202))
  (Variables|/Game/RollingWithThePunches/Blueprints/HUDs/Unlockables/Lore_HUD.Lore_HUD_C|SetLore3 (Variables|Default|GetLoreHUD_Ref) (Variables|Default|GetLore%203))
  (Variables|/Game/RollingWithThePunches/Blueprints/HUDs/Unlockables/Lore_HUD.Lore_HUD_C|SetLoreImage (Variables|Default|GetLoreHUD_Ref) (Variables|Default|GetLore%20Image))
  (Class|TextBlock|SetFont (Variables|/Game/RollingWithThePunches/Blueprints/HUDs/Unlockables/Lore_HUD.Lore_HUD_C|GetLoreText1 (Variables|Default|GetLoreHUD_Ref)) (Variables|Default|GetLoreFontSize1))
  (Class|TextBlock|SetFont (Variables|/Game/RollingWithThePunches/Blueprints/HUDs/Unlockables/Lore_HUD.Lore_HUD_C|GetLoreText2 (Variables|Default|GetLoreHUD_Ref)) (Variables|Default|GetLoreFontSize2))
  (Class|TextBlock|SetFont (Variables|/Game/RollingWithThePunches/Blueprints/HUDs/Unlockables/Lore_HUD.Lore_HUD_C|GetLoreText3 (Variables|Default|GetLoreHUD_Ref)) (Variables|Default|GetLoreFontSize3)))

(event EventUnlock
  (if (not (Variables|Default|GetLoreOpened?))
    (Utilities|FlowControl|Sequence
      (:then_0
        (Rendering|Material|SetMaterial (Variables|Default|GetStaticMesh) 1 "/Game/RollingWithThePunches/Blockmesh/Materials/MI_EM_White.MI_EM_White")
        (Utilities|FlowControl|Delay 0.2)
        (Rendering|Material|SetMaterial (Variables|Default|GetStaticMesh) 1 "/Game/RollingWithThePunches/Blockmesh/Materials/Metal/Solid_Black_Metal.Solid_Black_Metal"))
      (:then_1
        (Utilities|FlowControl|Delay 0.21)
        (if (not (UserInterface|Viewport|IsinViewport (Variables|Default|GetLoreHUD_Ref)))
          (UserInterface|Viewport|AddtoViewport (Variables|Default|GetLoreHUD_Ref) 0)))
      (:then_2
        (Variables|Default|SetLoreOpened? true)))))

(fn ConstructionScript)