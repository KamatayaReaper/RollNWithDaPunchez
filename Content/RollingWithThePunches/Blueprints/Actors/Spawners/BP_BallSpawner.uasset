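; Spawner actor that creates the player's boulder and links it to the first-person character.
; On BeginPlay it registers itself on that character, waits briefly, then spawns BoulderClass at the SpawnRef location and stores the boulder on the character.
; SetBoulderType maps the character's boulder-type enum to one of many face-themed Blueprint classes, but nothing in this graph calls it.
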(event Custom|SpawnBoulder
  (bind _returnvalue (Game|SpawnActorfromClass (Variables|Default|GetBoulderClass) (Math|Transform|MakeTransform (Transformation|GetWorldLocation (Variables|Default|GetSpawnRef)) "0, 0, 0" "1.000000,1.000000,1.000000") "Undefined" 0 0))
  (Variables|/Game/RollingWithThePunches/Blueprints/PlayerCharaacters/BP_FirstPersonCharacter.BP_FirstPersonCharacter_C|SetBoulderRef (Variables|Default|GetPlayerRef) _returnvalue))

(event EventBeginPlay
  (bind _asbp_first_person_character (Utilities|Casting|CastToBP_FirstPersonCharacter (Game|GetPlayerCharacter 0)))
  (bind _output_get (Variables|Default|SetPlayerRef _asbp_first_person_character))
  (Variables|/Game/RollingWithThePunches/Blueprints/PlayerCharaacters/BP_FirstPersonCharacter.BP_FirstPersonCharacter_C|SetBallSpawnerRef _output_get self)
  (Utilities|FlowControl|Delay 0.2)
  (CallFunction|SpawnBoulder))

(event Collision|EventActorBeginOverlap
  (params (OtherActor :type Actor%20Object%20Reference)))

(event EventTick
  (params (DeltaSeconds :type Float%20%28single-precision%29)))

(fn ConstructionScript)

(fn SetBoulderType
  (switch Utilities|FlowControl|Switch|SwitchonE_BoulderType (Variables|/Game/RollingWithThePunches/Blueprints/PlayerCharaacters/BP_FirstPersonCharacter.BP_FirstPersonCharacter_C|GetEN_BoulderType (Variables|Default|GetPlayerRef))
    (:NewEnumerator0
      (Variables|Default|SetBoulderClass "/Game/RollingWithThePunches/Blueprints/Actors/Boulders/BP_CrazyFace.BP_CrazyFace_C"))
    (:NewEnumerator1
      (Variables|Default|SetBoulderClass "/Game/RollingWithThePunches/Blueprints/Actors/Boulders/PorcelainGarden/BP_WuvFace.BP_WuvFace_C"))
    (:NewEnumerator2
      (Variables|Default|SetBoulderClass "/Game/RollingWithThePunches/Blueprints/Actors/Boulders/PorcelainGarden/BP_GrrFace.BP_GrrFace_C"))
    (:NewEnumerator4
      (Variables|Default|SetBoulderClass "/Game/RollingWithThePunches/Blueprints/Actors/Boulders/PorcelainGarden/BP_MunchFace.BP_MunchFace_C"))
    (:NewEnumerator7
      (Variables|Default|SetBoulderClass "/Game/RollingWithThePunches/Blueprints/Actors/Boulders/PorcelainGarden/BP_DPressFace.BP_DPressFace_C"))
    (:NewEnumerator6
      (Variables|Default|SetBoulderClass "/Game/RollingWithThePunches/Blueprints/Actors/Boulders/PorcelainGarden/BP_BabuFace.BP_BabuFace_C"))
    (:NewEnumerator5
      (Variables|Default|SetBoulderClass "/Game/RollingWithThePunches/Blueprints/Actors/Boulders/BP_JackedFace.BP_JackedFace_C"))
    (:NewEnumerator3
      (Variables|Default|SetBoulderClass "/Game/RollingWithThePunches/Blueprints/Actors/Boulders/BP_DoomFace.BP_DoomFace_C"))
    (:NewEnumerator8
      (Variables|Default|SetBoulderClass "/Game/RollingWithThePunches/Blueprints/Actors/Boulders/PorcelainGarden/BP_SmugFace.BP_SmugFace_C"))
    (:NewEnumerator9
      (Variables|Default|SetBoulderClass "/Game/RollingWithThePunches/Blueprints/Actors/Boulders/BP_Ninjaja.BP_Ninjaja_C"))
    (:NewEnumerator11
      (Variables|Default|SetBoulderClass "/Game/RollingWithThePunches/Blueprints/Actors/Boulders/BP_Doo-D-G.BP_Doo-D-G_C"))
    (:NewEnumerator13
      (Variables|Default|SetBoulderClass "/Game/RollingWithThePunches/Blueprints/Actors/Boulders/PorcelainGarden/BP_Joll-E-Bel.BP_Joll-E-Bel_C"))
    (:NewEnumerator12
      (Variables|Default|SetBoulderClass "/Game/RollingWithThePunches/Blueprints/Actors/Boulders/BP_ItaNimu.BP_ItaNimu_C"))
    (:NewEnumerator14
      (Variables|Default|SetBoulderClass "/Game/RollingWithThePunches/Blueprints/Actors/Boulders/BP_UFB.BP_UFB_C"))
    (:NewEnumerator10
      (Variables|Default|SetBoulderClass "/Game/RollingWithThePunches/Blueprints/Actors/Boulders/BP_DomoGato.BP_DomoGato_C"))
    (:NewEnumerator15
      (Variables|Default|SetBoulderClass "/Game/RollingWithThePunches/Blueprints/Actors/Boulders/BP_QTB.BP_QTB_C"))
    (:NewEnumerator16
      (Variables|Default|SetBoulderClass "/Game/RollingWithThePunches/Blueprints/Actors/Boulders/BP_HumpDump.BP_HumpDump_C"))
    (:NewEnumerator17
      (Variables|Default|SetBoulderClass "/Game/RollingWithThePunches/Blueprints/Actors/Boulders/BP_GlouChester.BP_GlouChester_C"))
    (:NewEnumerator18
      (Variables|Default|SetBoulderClass "/Game/RollingWithThePunches/Blueprints/Actors/Boulders/MegavoltSewer/BP_Jawr.BP_Jawr_C"))
    (:NewEnumerator19
      (Variables|Default|SetBoulderClass "/Game/RollingWithThePunches/Blueprints/Actors/Boulders/BP_AmeeBa.BP_AmeeBa_C"))
    (:NewEnumerator20
      (Variables|Default|SetBoulderClass "/Game/RollingWithThePunches/Blueprints/Actors/Boulders/BP_CrashBob.BP_CrashBob_C"))
    (:NewEnumerator21
      (Variables|Default|SetBoulderClass "/Game/RollingWithThePunches/Blueprints/Actors/Boulders/BP_KaratHead.BP_KaratHead_C"))
    (:NewEnumerator22
      (Variables|Default|SetBoulderClass "/Game/RollingWithThePunches/Blueprints/Actors/Boulders/BP_OkiDoki.BP_OkiDoki_C"))
    (:NewEnumerator23
      (Variables|Default|SetBoulderClass "/Game/RollingWithThePunches/Blueprints/Actors/Boulders/MegavoltSewer/BP_Googles.BP_Googles_C"))
    (:NewEnumerator24
      (Variables|Default|SetBoulderClass "/Game/RollingWithThePunches/Blueprints/Actors/Boulders/BP_GO-Z.BP_GO-Z_C"))
    (:NewEnumerator25
      (Variables|Default|SetBoulderClass "/Game/RollingWithThePunches/Blueprints/Actors/Boulders/BP_FRANK-E.BP_FRANK-E_C"))
    (:NewEnumerator26
      (Variables|Default|SetBoulderClass "/Game/RollingWithThePunches/Blueprints/Actors/Boulders/BP_Sling.BP_Sling_C"))
    (:NewEnumerator27
      (Variables|Default|SetBoulderClass "/Game/RollingWithThePunches/Blueprints/Actors/Boulders/BP_Ojo.BP_Ojo_C"))
    (:NewEnumerator28
      (Variables|Default|SetBoulderClass "/Game/RollingWithThePunches/Blueprints/Actors/Boulders/BP_Crackachack.BP_Crackachack_C"))
    (:NewEnumerator29
      (Variables|Default|SetBoulderClass "/Game/RollingWithThePunches/Blueprints/Actors/Boulders/BP_Grimm.BP_Grimm_C"))
    (:NewEnumerator30
      (Variables|Default|SetBoulderClass "/Game/RollingWithThePunches/Blueprints/Actors/Boulders/MegavoltSewer/BP_FooGoo.BP_FooGoo_C"))
    (:NewEnumerator31
      (Variables|Default|SetBoulderClass "/Game/RollingWithThePunches/Blueprints/Actors/Boulders/BP_Saguaro.BP_Saguaro_C"))
    (:NewEnumerator32
      (Variables|Default|SetBoulderClass "/Game/RollingWithThePunches/Blueprints/Actors/Boulders/BP_IronHedd.BP_IronHedd_C"))
    (:NewEnumerator33
      (Variables|Default|SetBoulderClass "/Game/RollingWithThePunches/Blueprints/Actors/Boulders/BP_Molon.BP_Molon_C"))
    (:NewEnumerator34
      (Variables|Default|SetBoulderClass "/Game/RollingWithThePunches/Blueprints/Actors/Boulders/BP_TabTab.BP_TabTab_C"))
    (:NewEnumerator35
      (Variables|Default|SetBoulderClass "/Game/RollingWithThePunches/Blueprints/Actors/Boulders/BP_PsychoFace.BP_PsychoFace_C"))
    (:NewEnumerator36
      (Variables|Default|SetBoulderClass "/Game/RollingWithThePunches/Blueprints/Actors/Boulders/MegavoltSewer/BP_Barrels.BP_Barrels_C"))
    (:NewEnumerator37
      (Variables|Default|SetBoulderClass "/Game/RollingWithThePunches/Blueprints/Actors/Boulders/MegavoltSewer/BP_UTOT.BP_UTOT_C"))
    (:NewEnumerator38
      (Variables|Default|SetBoulderClass "/Game/RollingWithThePunches/Blueprints/Actors/Boulders/MegavoltSewer/BP_Brrr.BP_Brrr_C"))
    (:NewEnumerator39
      (Variables|Default|SetBoulderClass "/Game/RollingWithThePunches/Blueprints/Actors/Boulders/MegavoltSewer/BP_DavyD.BP_DavyD_C"))
    (:NewEnumerator40
      (Variables|Default|SetBoulderClass "/Game/RollingWithThePunches/Blueprints/Actors/Boulders/MegavoltSewer/BP_DeQuak.BP_DeQuak_C"))
    (:NewEnumerator41
      (Variables|Default|SetBoulderClass "/Game/RollingWithThePunches/Blueprints/Actors/Boulders/MegavoltSewer/BP_Takayaki.BP_Takayaki_C"))
    (:NewEnumerator42
      (Variables|Default|SetBoulderClass "/Game/RollingWithThePunches/Blueprints/Actors/Boulders/BP_Gachango.BP_Gachango_C"))))