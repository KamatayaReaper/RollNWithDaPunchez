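; BP_UppercutIndicator is a short-lived effect actor that floats an uppercut force widget upward from its spawn point.
; On BeginPlay it confirms its widget component holds an UppercutForce_HUD, then sets an end point above and slightly offset in world space.
; The MoveActor timeline lerps the actor to that point without sweeping, and the actor destroys itself when the timeline finishes.
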(event EventBeginPlay
  (Utilities|Casting|CastToUppercutForce_HUD (UserInterface|GetWidget (Variables|Default|GetWidget)))
  (bind _output_get (Variables|Default|SetStartLocation (Transformation|GetActorLocation)))
  (Variables|Default|SetEndLocation (+ _output_get "-25.000000,-25.000000,100.000000"))
  (bind _movealpha (Timeline|MoveActor Play)
    (:Update
      (Transformation|SetActorLocation (Math|Vector|Lerp(Vector) (Variables|Default|GetStartLocation) (Variables|Default|GetEndLocation) _movealpha) false false))
    (:Finished
      (Actor|DestroyActor))))

(fn ConstructionScript)