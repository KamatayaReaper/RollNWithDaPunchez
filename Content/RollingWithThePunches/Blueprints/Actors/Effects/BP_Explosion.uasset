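; BP_Explosion is a short-lived explosion actor that pushes nearby physics objects, then destroys itself.
; On BeginPlay, Boom sphere-traces for PhysicsBody objects and applies a randomly scaled LaunchForcePhysicsMultiplier impulse to simulating components.
; The normalized direction toward each hit actor feeds the impulse's Location input, rather than the impulse itself.
; After a brief delay it hides its root and destroys itself; the emitter spawn is disconnected.
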(event Custom|Boom
  (bind _returnvalue (Transformation|GetActorLocation))
  (bind _outhits (Collision|MultiSphereTraceForObjects _returnvalue _returnvalue 5e+01 (Utilities|Array|MakeArray "ObjectTypeQuery4") false 0 "None"))
  (for _array_element _outhits
    (if (Physics|IsSimulatingPhysics (.HitComponent (Collision|BreakHitResult _array_element)) "None")
      (Physics|AddImpulseatLocation (.HitComponent (Collision|BreakHitResult _array_element)) (* (Variables|Default|GetLaunch%20Force%20Physics%20Multiplier) (Math|Random|RandomFloatinRange 5e+03 1.5e+04)) (Math|Vector|Normalize (- (Transformation|GetActorLocation (.HitActor (Collision|BreakHitResult _array_element))) (Transformation|GetActorLocation))) "None"))))

(event EventBeginPlay
  (CallFunction|Boom)
  (Utilities|FlowControl|Delay 0.3)
  (Rendering|SetVisibility (Variables|Default|GetDefaultSceneRoot) false false)
  (Actor|DestroyActor))

(event Collision|EventActorBeginOverlap
  (params (OtherActor :type Actor%20Object%20Reference)))

(event EventTick
  (params (DeltaSeconds :type Float%20%28single-precision%29)))

(fn ConstructionScript)