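; BP_Ninjaja is a boulder actor that briefly vanishes whenever it takes damage.
; AnyDamage calls the Dissapear event, which hides the Sphere component, waits a random whole number of seconds, then shows it again.
; Only the sphere's visibility is toggled, with no change to collision or propagation to child components.
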(event Custom|Dissapear
  (Rendering|SetVisibility (Variables|Default|GetSphere) false false)
  (Utilities|FlowControl|Delay (Math|Conversions|ToFloat(Integer) (Math|Random|RandomIntegerinRange 1 3)))
  (Rendering|SetVisibility (Variables|Default|GetSphere) true false))

(event EventBeginPlay
  (|CallParentFunction) ; This node is disabled and will not be called.\nDrag off pins to build functionality.
)

(event Collision|EventActorBeginOverlap
  (params (OtherActor :type Actor%20Object%20Reference)))

(event EventTick
  (params (DeltaSeconds :type Float%20%28single-precision%29))
  (|CallParentFunction DeltaSeconds) ; This node is disabled and will not be called.\nDrag off pins to build functionality.
)

(event Game|Damage|EventAnyDamage
  (params (Damage :type Float%20%28single-precision%29) (DamageType :type Damage%20Type%20Object%20Reference) (InstigatedBy :type Controller%20Object%20Reference) (DamageCauser :type Actor%20Object%20Reference))
  (CallFunction|Dissapear))

(fn ConstructionScript
  (|CallParentFunction))