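; BP_DPressFace is a child boulder Blueprint that keeps growing over time and shrinks when it takes damage.
; A looping timer started at BeginPlay increases BoulderSize and rescales the Sphere up to a maximum.
; AnyDamage subtracts size based on the player arms' ForceUnleashed, clamps to a minimum, then rescales after a short delay before calling the parent handler.
; An older timeline-driven growth path remains but is unreachable.
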(event Custom|Grow
  (bind _output_get (Variables|Default|SetBoulderSize (+ (Variables|Default|GetBoulderSize) 0.01)))
  (if (>= (.z (Variables|Default|GetBoulderSize)) (.z (Variables|Default|GetMaxBoulderSize)))
    (bind _output_get_2 (Variables|Default|SetBoulderSize (Variables|Default|GetMaxBoulderSize)))
    (Transformation|SetRelativeScale3D (Variables|Default|GetSphere) _output_get_2)
    (else
      (Transformation|SetRelativeScale3D (Variables|Default|GetSphere) _output_get))))

(event EventBeginPlay
  (|CallParentFunction)
  (Utilities|Time|SetTimerbyEvent (delegate Custom|Grow) 0.1 true))

(event Collision|EventActorBeginOverlap
  (params (OtherActor :type Actor%20Object%20Reference)))

(event EventTick
  (params (DeltaSeconds :type Float%20%28single-precision%29))
  (|CallParentFunction DeltaSeconds) ; This node is disabled and will not be called.\nDrag off pins to build functionality.
)

(event Game|Damage|EventAnyDamage
  (params (Damage :type Float%20%28single-precision%29) (DamageType :type Damage%20Type%20Object%20Reference) (InstigatedBy :type Controller%20Object%20Reference) (DamageCauser :type Actor%20Object%20Reference))
  (bind _output_get (Variables|Default|SetBoulderSize (+ (Variables|Default|GetBoulderSize) (* (Variables|/Game/RollingWithThePunches/Blueprints/Actors/BP_Arms.BP_Arms_C|GetForceUnleashed (Variables|/Game/RollingWithThePunches/Blueprints/PlayerCharaacters/BP_FirstPersonCharacter.BP_FirstPersonCharacter_C|GetArmsRef (Variables|Default|GetPlayerRef))) -0.5))))
  (if (<= (.z _output_get) (.z (Variables|Default|GetMinimumBoulderSize)))
    (Variables|Default|SetBoulderSize (Variables|Default|GetMinimumBoulderSize)))
  (Utilities|FlowControl|Delay 0.2)
  (Transformation|SetRelativeScale3D (Variables|Default|GetSphere) (Variables|Default|GetBoulderSize))
  (|CallParentFunction 0.0 0 0 0))

(fn ConstructionScript
  (|CallParentFunction))