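; BP_Crackachack is a boulder actor that occasionally sets off an explosion when it hits something.
; Each hit has a very small random chance to spawn BP_Explosion at the impact point, gated by a CanExplode flag.
; The flag turns on after a short delay at BeginPlay, resets on a cooldown after each blast, and is re-enabled immediately by any damage.
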(event Custom|SpawnExplosion
  (params (BlastLocation :type Vector))
  (if (and (> (Math|Random|RandomIntegerinRange 1 500) 499) (Variables|Default|GetCanExplode?))
    (Game|SpawnActorfromClass "/Game/RollingWithThePunches/Blueprints/Actors/Effects/BP_Explosion.BP_Explosion_C" (Math|Transform|MakeTransform BlastLocation "0, 0, 0" "1.000000,1.000000,1.000000") "Undefined" 0 0)
    (Variables|Default|SetCanExplode? false)
    (Utilities|FlowControl|Delay 3.0)
    (Variables|Default|SetCanExplode? true)))

(event EventBeginPlay
  (|CallParentFunction)
  (Utilities|FlowControl|Delay 3.0)
  (Variables|Default|SetCanExplode? true))

(event Collision|EventActorBeginOverlap
  (params (OtherActor :type Actor%20Object%20Reference)))

(event EventTick
  (params (DeltaSeconds :type Float%20%28single-precision%29))
  (|CallParentFunction DeltaSeconds) ; This node is disabled and will not be called.\nDrag off pins to build functionality.
)

(event Collision|EventHit
  (params (MyComp :type Primitive%20Component%20Object%20Reference) (Other :type Actor%20Object%20Reference) (OtherComp :type Primitive%20Component%20Object%20Reference) (bSelfMoved :type Boolean) (HitLocation :type Vector :default "0, 0, 0") (HitNormal :type Vector :default "0, 0, 0") (NormalImpulse :type Vector :default "0, 0, 0") (Hit :type Hit%20Result%20Structure%20%28by%20ref%29))
  (CallFunction|SpawnExplosion HitLocation)
  (|CallParentFunction MyComp Other OtherComp bSelfMoved HitLocation HitNormal NormalImpulse Hit))

(event Game|Damage|EventAnyDamage
  (params (Damage :type Float%20%28single-precision%29) (DamageType :type Damage%20Type%20Object%20Reference) (InstigatedBy :type Controller%20Object%20Reference) (DamageCauser :type Actor%20Object%20Reference))
  (Variables|Default|SetCanExplode? true)
  (|CallParentFunction Damage DamageType InstigatedBy DamageCauser))

(fn ConstructionScript
  (|CallParentFunction))