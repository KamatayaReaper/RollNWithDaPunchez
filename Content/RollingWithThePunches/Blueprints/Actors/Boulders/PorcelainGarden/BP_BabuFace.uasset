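; BP_BabuFace is a Porcelain Garden boulder actor that cries like a baby while left undamaged.
; BeginPlay starts a retriggerable delay, after which it plays the crying sound in 2D and repeats it on a looping timer.
; AnyDamage restarts that delay and clears the timer, so each hit silences the crying until the quiet period elapses again.
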(event Custom|PrepareCrying
  (Utilities|FlowControl|RetriggerableDelay 5.0)
  (bind _returnvalue (Utilities|Time|SetTimerbyEvent (delegate Custom|PlayCrying) 2.0 true))
  (Audio|PlaySound2D "/Game/RollingWithThePunches/Assets/Sounds/BallEffects/CryingBaby.CryingBaby" 1.0 1.0 0.0 0 0)
  (Variables|Default|SetCryingTimer _returnvalue))

(event Custom|PlayCrying
  (Audio|PlaySound2D "/Game/RollingWithThePunches/Assets/Sounds/BallEffects/CryingBaby.CryingBaby" 1.0 1.0 0.0 0 0))

(event EventBeginPlay
  (|CallParentFunction)
  (CallFunction|PrepareCrying))

(event Collision|EventActorBeginOverlap
  (params (OtherActor :type Actor%20Object%20Reference)))

(event EventTick
  (params (DeltaSeconds :type Float%20%28single-precision%29))
  (|CallParentFunction DeltaSeconds) ; This node is disabled and will not be called.\nDrag off pins to build functionality.
)

(event Game|Damage|EventAnyDamage
  (params (Damage :type Float%20%28single-precision%29) (DamageType :type Damage%20Type%20Object%20Reference) (InstigatedBy :type Controller%20Object%20Reference) (DamageCauser :type Actor%20Object%20Reference))
  (|CallParentFunction 0.0 0 0 0)
  (Utilities|FlowControl|Sequence
    (:then_0
      (CallFunction|PrepareCrying))
    (:then_1
      (if (Utilities|Time|IsValidTimerHandle (Variables|Default|GetCryingTimer))
        (Utilities|Time|ClearandInvalidateTimerbyHandle (Variables|Default|GetCryingTimer))))))

(fn ConstructionScript
  (|CallParentFunction))