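; BP_KaratHead is a boulder actor that changes shape when it takes damage.
; Each AnyDamage event calls ChangeShape, then passes the damage on to the parent implementation.
; ChangeShape uses a FlipFlop to alternate the Sphere component's static mesh between a cube and a material sphere, starting with the cube.
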(event Custom|ChangeShape
  (Utilities|FlowControl|FlipFlop
    (:A
      (Components|StaticMesh|SetStaticMesh (Variables|Default|GetSphere) "/Game/LevelPrototyping/Meshes/SM_Cube.SM_Cube"))
    (:B
      (Components|StaticMesh|SetStaticMesh (Variables|Default|GetSphere) "/Game/PhysicsCollisionSound/Materials/SM_MaterialSphere.SM_MaterialSphere"))))

(event EventBeginPlay
  (|CallParentFunction) ; This node is disabled and will not be called.\nDrag off pins to build functionality.
)

(event Collision|EventActorBeginOverlap
  (params (OtherActor :type Actor%20Object%20Reference)))

(event EventTick
  (params (DeltaSeconds :type Float%20%28single-precision%29))
  (|CallParentFunction DeltaSeconds) ; This node is disabled and will not be called.\nDrag off pins to build functionality.
)

(event Game|Damage|EventAnyDamage
  (params (Damage :type Float%20%28single-precision%29) (DamageType :type Damage%20Type%20Object%20Reference) (InstigatedBy :type Controller%20Object%20Reference) (DamageCauser :type Actor%20Object%20Reference))
  (CallFunction|ChangeShape)
  (|CallParentFunction Damage DamageType InstigatedBy DamageCauser))

(fn ConstructionScript
  (|CallParentFunction))