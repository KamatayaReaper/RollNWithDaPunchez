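; BP_MunchFace is a boulder actor variant that grows when it takes damage and otherwise shrinks steadily over time.
; Damage raises BoulderSize, caps it at MaxBoulderSize, rescales the Sphere after a short delay, then calls the parent's damage logic.
; From BeginPlay, the ShrinkBall timeline lerps the size downward to MinimumBoulderSize, re-triggering Shrink after each run to form a continuous loop.
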(event Custom|Shrink
  (bind _shrinkalpha (Timeline|ShrinkBall Play)
    (:Update
      (bind _output_get (Variables|Default|SetBoulderSize (Math|Vector|Lerp(Vector) (Variables|Default|GetBoulderSize) (- (Variables|Default|GetBoulderSize) 0.1) _shrinkalpha)))
      (if (<= (.z (Variables|Default|GetBoulderSize)) (.z (Variables|Default|GetMinimumBoulderSize)))
        (bind _output_get_2 (Variables|Default|SetBoulderSize (Variables|Default|GetMinimumBoulderSize)))
        (Transformation|SetRelativeScale3D (Variables|Default|GetSphere) _output_get_2)
        (else
          (Transformation|SetRelativeScale3D (Variables|Default|GetSphere) _output_get))))
    (:Finished
      (Utilities|FlowControl|Delay _shrinkalpha)
      (CallFunction|Shrink))))

(event EventBeginPlay
  (|CallParentFunction)
  (CallFunction|Shrink))

(event Collision|EventActorBeginOverlap
  (params (OtherActor :type Actor%20Object%20Reference)))

(event EventTick
  (params (DeltaSeconds :type Float%20%28single-precision%29))
  (|CallParentFunction DeltaSeconds))

(event Game|Damage|EventAnyDamage
  (params (Damage :type Float%20%28single-precision%29) (DamageType :type Damage%20Type%20Object%20Reference) (InstigatedBy :type Controller%20Object%20Reference) (DamageCauser :type Actor%20Object%20Reference))
  (bind _output_get (Variables|Default|SetBoulderSize (+ (Variables|Default|GetBoulderSize) 0.5)))
  (if (>= (.z _output_get) (.z (Variables|Default|GetMaxBoulderSize)))
    (Variables|Default|SetBoulderSize (Variables|Default|GetMaxBoulderSize)))
  (Utilities|FlowControl|Delay 0.2)
  (Transformation|SetRelativeScale3D (Variables|Default|GetSphere) (Variables|Default|GetBoulderSize))
  (|CallParentFunction 0.0 0 0 0))

(fn ConstructionScript
  (|CallParentFunction))