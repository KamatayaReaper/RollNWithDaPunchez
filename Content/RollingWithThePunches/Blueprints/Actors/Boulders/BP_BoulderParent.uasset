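; Parent boulder actor: a physics sphere that damages Enemy-tagged actors on hit, notifies BPI_Physics objects, and can reset to an updatable spawn point.
; Tick toggles a widget by player distance and applies clamped, size-scaled upward buoyancy impulses while in water.
; Taking damage triggers hitstop through custom time dilation and a timer.
; An overlap volume swaps the sphere to a transparent material while the player is inside.
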(event OnComponentBeginOverlap(TransparentCollision)
  (params (OverlappedComponent :type Primitive%20Component%20Object%20Reference) (OtherActor :type Actor%20Object%20Reference) (OtherComp :type Primitive%20Component%20Object%20Reference) (OtherBodyIndex :type Integer) (bFromSweep :type Boolean) (SweepResult :type Hit%20Result%20Structure%20%28by%20ref%29))
  (if (== OtherActor (Variables|Default|GetPlayerRef))
    (Rendering|Material|SetMaterial (Variables|Default|GetSphere) 0 (Variables|Default|GetTransparentMat))))

(event OnComponentEndOverlap(TransparentCollision)
  (params (OverlappedComponent :type Primitive%20Component%20Object%20Reference) (OtherActor :type Actor%20Object%20Reference) (OtherComp :type Primitive%20Component%20Object%20Reference) (OtherBodyIndex :type Integer))
  (if (== OtherActor (Variables|Default|GetPlayerRef))
    (Rendering|Material|SetMaterial (Variables|Default|GetSphere) 0 (Variables|Default|GetBaseMaterial))))

(event Custom|StopBall
  (Utilities|FlowControl|RetriggerableDelay 5.0))

(event Custom|CheckDistance
  (bind _widget (Variables|Default|GetWidget))
  (Utilities|FlowControl|Delay 0.2)
  (if (>= (Class|KismetMathLibrary|Round64 (/ (Math|Vector|VectorLength (- (Variables|/Script/Engine.SceneComponent|GetRelativeLocation (Variables|Default|GetSphere)) (Transformation|GetActorLocation (Pawn|GetControlledPawn (Game|GetPlayerController 0))))) 1e+02)) (Variables|Default|GetDistanceLimit))
    (Rendering|SetVisibility _widget true false)
    (else
      (Rendering|SetVisibility _widget false false))))

(event Custom|ResetBoulder
  (bind _sphere (Variables|Default|GetSphere))
  (Transformation|SetWorldTransform _sphere (Math|Transform|MakeTransform (Variables|Default|GetBoulderSpawnPoint) (Variables|/Script/Engine.SceneComponent|GetRelativeRotation _sphere) (Variables|Size|GetBoulderSize)) false true)
  (Variables|Default|SetJustSpawned? true)
  (Utilities|FlowControl|Sequence
    (:then_0
      (Physics|SetSimulatePhysics (Variables|Default|GetSphere) false)
      (Utilities|FlowControl|Delay 1e-05)
      (Physics|SetSimulatePhysics (Variables|Default|GetSphere) true))
    (:then_1
      (Utilities|FlowControl|Delay 1.0)
      (Variables|Default|SetJustSpawned? false))))

(event Custom|DestroyBall
  (Actor|DestroyActor))

(event Custom|FloatBall
  (if (Variables|Water|GetInWater)
    (Physics|AddImpulse (Variables|Default|GetSphere) (Math|Vector|MakeVector 0.0 0.0 (Math|Float|Clamp(Float) (Math|Float|Absolute(Float) (.z (* (* (Variables|Water|GetUpVector) (- (Variables|Water|GetWaterVolume) (.z (Transformation|GetWorldLocation (Variables|Default|GetSphere))))) (* (Variables|Size|GetBoulderSize) (Variables|Water|GetBuoyancyForce))))) 1e+04 (Variables|Default|GetMaxWaterPush))) "None" false)))

(event Custom|SetNewBoulderSpawn
  (params (NewSpawn :type Vector))
  (Variables|Default|SetBoulderSpawnPoint NewSpawn))

(event Custom|FreezeBall
  (Physics|SetSimulatePhysics (Variables|Default|GetSphere) false)
  (Utilities|FlowControl|Delay 1e-05)
  (Physics|SetSimulatePhysics (Variables|Default|GetSphere) true))

(event EventBeginPlay
  (bind _bouldersize (Variables|Size|GetBoulderSize))
  (Utilities|FlowControl|Sequence
    (:then_0
      (Variables|Default|SetBoulderSpawnPoint (Variables|/Script/Engine.SceneComponent|GetRelativeLocation (Variables|Default|GetSphere)))
      (Variables|Size|SetDefaultBoulderSize _bouldersize)
      (Variables|Size|SetMinimumBoulderSize (/ _bouldersize 2.0))
      (Variables|Size|SetMaxBoulderSize (* _bouldersize 2.0))
      (Variables|Default|SetJustSpawned? false))
    (:then_1
      (bind _asbp_first_person_character (Utilities|Casting|CastToBP_FirstPersonCharacter (Game|GetPlayerCharacter 0)))
      (Variables|Default|SetPlayerRef _asbp_first_person_character))))

(event EventTick
  (params (DeltaSeconds :type Float%20%28single-precision%29))
  (Utilities|FlowControl|Sequence
    (:then_0
      (CallFunction|CheckDistance))
    (:then_1
      (CallFunction|FloatBall))
    (:then_2
      (Utilities|FlowControl|Delay 1.0))))

(event Game|Damage|EventAnyDamage
  (params (Damage :type Float%20%28single-precision%29) (DamageType :type Damage%20Type%20Object%20Reference) (InstigatedBy :type Controller%20Object%20Reference) (DamageCauser :type Actor%20Object%20Reference))
  (CallFunction|StartHitstop (Variables|Default|GetHitStopDuration)))

(event Collision|EventHit
  (params (MyComp :type Primitive%20Component%20Object%20Reference) (Other :type Actor%20Object%20Reference) (OtherComp :type Primitive%20Component%20Object%20Reference) (bSelfMoved :type Boolean) (HitLocation :type Vector :default "0, 0, 0") (HitNormal :type Vector :default "0, 0, 0") (NormalImpulse :type Vector :default "0, 0, 0") (Hit :type Hit%20Result%20Structure%20%28by%20ref%29))
  (Utilities|FlowControl|Sequence
    (:then_0
      (if (Actor|ActorHasTag Other "Enemy")
        (Game|Damage|ApplyDamage Other 1.0 0 self)))
    (:then_1
      (if (Utilities|DoesObjectImplementInterface Other "/Game/RollingWithThePunches/Blueprints/Interface/BPI_Physics.BPI_Physics_C")
        (Class|BPIPhysics|StartPhysics(Message) Other)))))

(fn ConstructionScript
  (bind _sphere (Variables|Default|GetSphere))
  (Transformation|SetRelativeTransform _sphere (Math|Transform|MakeTransform (Variables|Default|GetBoulderSpawnPoint) (Transformation|GetWorldRotation _sphere) (Variables|Size|GetBoulderSize)) false false))

(fn StartHitstop
  (params (Duration :type Float%20%28single-precision%29))
  (Variables|Default|SetCustomTimeDilation 0.0)
  (Utilities|Time|SetTimerbyFunctionName 0 "EndHitStop" Duration))

(fn EndHitstop
  (Variables|Default|SetCustomTimeDilation 1.0))