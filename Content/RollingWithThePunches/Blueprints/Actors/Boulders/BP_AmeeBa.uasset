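; BP_AmeeBa is a boulder actor that shrinks and sheds a copy of itself when it takes damage.
; Each hit reduces BoulderSize by a fixed step, rescales the Sphere and spawns a BP_AmeeBa_Fake at the Sphere's relative location.
; Once the Z size reaches MinimumBoulderSize, further hits only hold it at that minimum without spawning.
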(event EventBeginPlay
  (|CallParentFunction) ; This node is disabled and will not be called.\nDrag off pins to build functionality.
)

(event Collision|EventActorBeginOverlap
  (params (OtherActor :type Actor%20Object%20Reference)))

(event EventTick
  (params (DeltaSeconds :type Float%20%28single-precision%29))
  (|CallParentFunction DeltaSeconds) ; This node is disabled and will not be called.\nDrag off pins to build functionality.
)

(event Game|Damage|EventAnyDamage
  (params (Damage :type Float%20%28single-precision%29) (DamageType :type Damage%20Type%20Object%20Reference) (InstigatedBy :type Controller%20Object%20Reference) (DamageCauser :type Actor%20Object%20Reference))
  (if (not (<= (.z (Variables|Default|GetBoulderSize)) (.z (Variables|Default|GetMinimumBoulderSize))))
    (Variables|Default|SetBoulderSize (+ (Variables|Default|GetBoulderSize) (* 1.0 -0.25)))
    (Transformation|SetRelativeScale3D (Variables|Default|GetSphere) (Variables|Default|GetBoulderSize))
    (Game|SpawnActorfromClass "/Game/RollingWithThePunches/Blueprints/Actors/PhysicsProps/Boulders/BP_AmeeBa_Fake.BP_AmeeBa_Fake_C" (Math|Transform|MakeTransform (Variables|/Script/Engine.SceneComponent|GetRelativeLocation (Variables|Default|GetSphere)) "0, 0, 0" "1.250000,1.250000,1.250000") "Undefined" 0 0)
    (else
      (bind _output_get (Variables|Default|SetBoulderSize (Variables|Default|GetMinimumBoulderSize)))
      (Transformation|SetRelativeScale3D (Variables|Default|GetSphere) _output_get))))

(fn ConstructionScript
  (|CallParentFunction))