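; BP_UTOT is a boulder actor for the MegavoltSewer set that adds its own sound cue to inherited boulder behavior.
; PlayUniqueNoise plays UTOT_Cue at the sphere's location, while FartNoise does the same behind a one-second CanFart cooldown flag.
; The calls to FartNoise, including a rare random trigger, are disconnected and never run.
; Damage and hit events only forward to the parent.
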(event Custom|FartNoise
  (Variables|Default|SetCanFart false)
  (Audio|PlaySoundatLocation "/Game/RollingWithThePunches/Assets/Sounds/BallEffects/Farts/UTOT_Cue.UTOT_Cue" (Transformation|GetWorldLocation (Variables|Default|GetSphere)) "0, 0, 0" 1.0 1.0 0.0 0 0 0 0)
  (Utilities|FlowControl|Delay 1.0)
  (Variables|Default|SetCanFart true))

(event EventBeginPlay
  (|CallParentFunction)
  (Variables|Default|SetCanFart true))

(event Collision|EventActorBeginOverlap
  (params (OtherActor :type Actor%20Object%20Reference)))

(event EventTick
  (params (DeltaSeconds :type Float%20%28single-precision%29))
  (|CallParentFunction DeltaSeconds) ; This node is disabled and will not be called.\nDrag off pins to build functionality.
)

(event Game|Damage|EventAnyDamage
  (params (Damage :type Float%20%28single-precision%29) (DamageType :type Damage%20Type%20Object%20Reference) (InstigatedBy :type Controller%20Object%20Reference) (DamageCauser :type Actor%20Object%20Reference))
  (|CallParentFunction Damage DamageType InstigatedBy DamageCauser))

(event Collision|EventHit
  (params (MyComp :type Primitive%20Component%20Object%20Reference) (Other :type Actor%20Object%20Reference) (OtherComp :type Primitive%20Component%20Object%20Reference) (bSelfMoved :type Boolean) (HitLocation :type Vector :default "0, 0, 0") (HitNormal :type Vector :default "0, 0, 0") (NormalImpulse :type Vector :default "0, 0, 0") (Hit :type Hit%20Result%20Structure%20%28by%20ref%29))
  (|CallParentFunction MyComp Other OtherComp bSelfMoved HitLocation HitNormal NormalImpulse Hit))

(event EventPlayUniqueNoise
  (Audio|PlaySoundatLocation "/Game/RollingWithThePunches/Assets/Sounds/BallEffects/Farts/UTOT_Cue.UTOT_Cue" (Transformation|GetWorldLocation (Variables|Default|GetSphere)) "0, 0, 0" 1.0 1.0 0.0 0 0 0 0))

(fn ConstructionScript
  (|CallParentFunction))