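; BP_Takayaki is a boulder actor for Megavolt Sewer that can splat an ink stain on the screen when it receives damage.
; On AnyDamage it runs the parent handler, then has a one-in-three chance to create a random widget from the InkStainHUD class array and add it to the viewport.
; BeginPlay, overlap and Tick are disabled stubs, and the construction script only calls its parent.
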(event EventBeginPlay
  (|CallParentFunction) ; This node is disabled and will not be called.\nDrag off pins to build functionality.
)

(event Collision|EventActorBeginOverlap
  (params (OtherActor :type Actor%20Object%20Reference)))

(event EventTick
  (params (DeltaSeconds :type Float%20%28single-precision%29))
  (|CallParentFunction DeltaSeconds) ; This node is disabled and will not be called.\nDrag off pins to build functionality.
)

(event Game|Damage|EventAnyDamage
  (params (Damage :type Float%20%28single-precision%29) (DamageType :type Damage%20Type%20Object%20Reference) (InstigatedBy :type Controller%20Object%20Reference) (DamageCauser :type Actor%20Object%20Reference))
  (|CallParentFunction 0.0 0 0 0)
  (if (<= (Math|Random|RandomIntegerinRange 0 2) 0)
    (bind _returnvalue (UserInterface|CreateWidget (Utilities|Array|Get(acopy) (Variables|Default|GetInkStainHUD) (Math|Random|RandomIntegerinRange 0 4))))
    (UserInterface|Viewport|AddtoViewport _returnvalue 0)))

(fn ConstructionScript
  (|CallParentFunction))