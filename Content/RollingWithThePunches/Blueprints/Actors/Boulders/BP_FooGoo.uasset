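; BP_FooGoo is a boulder actor that inflates when damaged, then shrinks back after a pause.
; Each hit grows BoulderSize by the player arms' ForceUnleashed, up to a maximum, and applies it to the Sphere after a short delay with gravity disabled.
; A retriggerable delay postpones deflation during repeated hits, then a timeline lerps the scale to default and restores gravity when finished.
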(event Custom|Inflate
  (Utilities|FlowControl|Sequence
    (:then_0
      (bind _output_get (Variables|Default|SetBoulderSize (+ (Variables|Default|GetBoulderSize) (* (Variables|/Game/RollingWithThePunches/Blueprints/Actors/BP_Arms.BP_Arms_C|GetForceUnleashed (Variables|/Game/RollingWithThePunches/Blueprints/PlayerCharaacters/BP_FirstPersonCharacter.BP_FirstPersonCharacter_C|GetArmsRef (Variables|Default|GetPlayerRef))) 2.5))))
      (if (>= (.z _output_get) (.z (Variables|Default|GetMaxBoulderSize)))
        (Variables|Default|SetBoulderSize (Variables|Default|GetMaxBoulderSize)))
      (Utilities|FlowControl|Delay 0.2)
      (Transformation|SetRelativeScale3D (Variables|Default|GetSphere) (Variables|Default|GetBoulderSize))
      (Utilities|FlowControl|RetriggerableDelay 3.0)
      (bind _deflatealpha (Timeline|Deflate PlayFromStart)
        (:Update
          (Transformation|SetRelativeScale3D (Variables|Default|GetSphere) (Math|Vector|Lerp(Vector) (Variables|Default|GetBoulderSize) (Variables|Default|GetDefaultBoulderSize) _deflatealpha)))
        (:Finished
          (Physics|SetEnableGravity (Variables|Default|GetSphere) true))))
    (:then_1
      (Physics|SetEnableGravity (Variables|Default|GetSphere) false))))

(event EventBeginPlay
  (|CallParentFunction) ; This node is disabled and will not be called.\nDrag off pins to build functionality.
)

(event Collision|EventActorBeginOverlap
  (params (OtherActor :type Actor%20Object%20Reference)))

(event EventTick
  (params (DeltaSeconds :type Float%20%28single-precision%29))
  (|CallParentFunction DeltaSeconds) ; This node is disabled and will not be called.\nDrag off pins to build functionality.
)

(event Game|Damage|EventAnyDamage
  (params (Damage :type Float%20%28single-precision%29) (DamageType :type Damage%20Type%20Object%20Reference) (InstigatedBy :type Controller%20Object%20Reference) (DamageCauser :type Actor%20Object%20Reference))
  (CallFunction|Inflate)
  (|CallParentFunction Damage DamageType InstigatedBy DamageCauser))

(fn ConstructionScript
  (|CallParentFunction))