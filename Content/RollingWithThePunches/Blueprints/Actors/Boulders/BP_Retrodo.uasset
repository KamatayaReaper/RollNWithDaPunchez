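; BP_Retrodo is a retro-themed boulder actor that switches the level to a retro presentation.
; On BeginPlay, after the parent logic, it calls ShowRetro on the player reference, then runs one custom event per interactable type.
; Each event finds every actor of its class (buttons, ball reset buttons, goals, sliding doors, pressure pads) and overwrites its sound effect variables with retro sounds.
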(event Custom|SetButtonSounds
  (bind _outactors (Actor|GetAllActorsOfClass "/Game/RollingWithThePunches/Blueprints/Actors/Switches/Buttons/ButtonBasic_BP.ButtonBasic_BP_C"))
  (for _array_element _outactors
    (Variables|/Game/RollingWithThePunches/Blueprints/Actors/Switches/Buttons/ButtonBasic_BP.ButtonBasic_BP_C|SetSwitchSFX1 _array_element "/Game/RollingWithThePunches/Assets/Sounds/Retro/RetroClick.RetroClick")
    (Variables|/Game/RollingWithThePunches/Blueprints/Actors/Switches/Buttons/ButtonBasic_BP.ButtonBasic_BP_C|SetSwitchSFX2 _array_element "/Game/RollingWithThePunches/Assets/Sounds/Retro/RetroButton.RetroButton")
    (Variables|/Game/RollingWithThePunches/Blueprints/Actors/Switches/Buttons/ButtonBasic_BP.ButtonBasic_BP_C|SetErrorSFX _array_element "/Game/RollingWithThePunches/Assets/Sounds/Retro/RetroWrong.RetroWrong")))

(event Custom|SetResetButtonSounds
  (bind _outactors (Actor|GetAllActorsOfClass "/Game/RollingWithThePunches/Blueprints/Actors/Switches/Buttons/BP_ResetBallButton.BP_ResetBallButton_C"))
  (for _array_element _outactors
    (Variables|/Game/RollingWithThePunches/Blueprints/Actors/Switches/Buttons/BP_ResetBallButton.BP_ResetBallButton_C|SetButtonSFX1 _array_element "/Game/RollingWithThePunches/Assets/Sounds/Retro/RetroClick.RetroClick")
    (Variables|/Game/RollingWithThePunches/Blueprints/Actors/Switches/Buttons/BP_ResetBallButton.BP_ResetBallButton_C|SetButtonSFX2 _array_element "/Game/RollingWithThePunches/Assets/Sounds/Retro/RetroButton.RetroButton")
    (Variables|/Game/RollingWithThePunches/Blueprints/Actors/Switches/Buttons/BP_ResetBallButton.BP_ResetBallButton_C|SetMockLaughSFX _array_element "/Game/RollingWithThePunches/Assets/Sounds/Retro/RetroReset.RetroReset")))

(event Custom|SetGoalSounds
  (bind _outactors (Actor|GetAllActorsOfClass "/Game/RollingWithThePunches/Blueprints/Actors/BP_Goal.BP_Goal_C"))
  (for _array_element _outactors
    (Variables|/Game/RollingWithThePunches/Blueprints/Actors/BP_Goal.BP_Goal_C|SetActivateSFX _array_element "/Game/RollingWithThePunches/Assets/Sounds/Retro/RetroActivate.RetroActivate")
    (Variables|/Game/RollingWithThePunches/Blueprints/Actors/BP_Goal.BP_Goal_C|SetDeactivateSFX _array_element "/Game/RollingWithThePunches/Assets/Sounds/Retro/RetroDeactivate.RetroDeactivate")))

(event Custom|SetSlidingDoorSounds
  (bind _outactors (Actor|GetAllActorsOfClass "/Game/RollingWithThePunches/Blueprints/Actors/Switches/Activators/BP_SlidingDoor.BP_SlidingDoor_C"))
  (for _array_element _outactors
    (Variables|/Game/RollingWithThePunches/Blueprints/Actors/Switches/Activators/BP_SlidingDoor.BP_SlidingDoor_C|SetSlidingDoorSFX _array_element "/Game/RollingWithThePunches/Assets/Sounds/Retro/RetroDoor.RetroDoor")))

(event Custom|SetPressurePlateSounds
  (bind _outactors (Actor|GetAllActorsOfClass "/Game/RollingWithThePunches/Blueprints/Actors/Switches/BP_PressurePad.BP_PressurePad_C"))
  (for _array_element _outactors
    (Variables|/Game/RollingWithThePunches/Blueprints/Actors/Switches/BP_PressurePad.BP_PressurePad_C|SetSwitchSFX1 _array_element "/Game/RollingWithThePunches/Assets/Sounds/Retro/RetroClick.RetroClick")
    (Variables|/Game/RollingWithThePunches/Blueprints/Actors/Switches/BP_PressurePad.BP_PressurePad_C|SetSwitchSFX2 _array_element "/Game/RollingWithThePunches/Assets/Sounds/Retro/RetroButton.RetroButton")))

(event EventBeginPlay
  (|CallParentFunction)
  (Utilities|FlowControl|Sequence
    (:then_0
      (Default|ShowRetro (Variables|Default|GetPlayerRef)))
    (:then_1
      (CallFunction|SetButtonSounds)
      (CallFunction|SetResetButtonSounds)
      (CallFunction|SetGoalSounds)
      (CallFunction|SetSlidingDoorSounds)
      (CallFunction|SetPressurePlateSounds))))

(event Collision|EventActorBeginOverlap
  (params (OtherActor :type Actor%20Object%20Reference)))

(event EventTick
  (params (DeltaSeconds :type Float%20%28single-precision%29))
  (|CallParentFunction DeltaSeconds) ; This node is disabled and will not be called.\nDrag off pins to build functionality.
)

(fn ConstructionScript
  (|CallParentFunction))