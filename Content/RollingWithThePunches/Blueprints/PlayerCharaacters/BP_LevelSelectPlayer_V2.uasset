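; Level select player that opens the world menu with keyboard focus and views the level through placed BP_LevelSelectCamera actors.
; BeginPlay gathers the cameras, loads completed levels and boulder/special setup from the game instance, and prepares ambience audio.
; Events control ambience and blend between cameras with index wraparound, while hits play a ball sound.
; Rolling, look, pause and camera-cycling logic is disconnected, and zoom timelines no longer drive arm length.
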(event Custom|ZoomCameraIn
  ;[0 0.7629 1] Zoom Functions
)

(event Custom|ZoomCameraBack%28Out%29
  ;[0 0.7629 1] Zoom Functions
  (bind _zoomalpha (Timeline|ZoomOutTimeline Reverse)))

(event Custom|OpenWorldMenu
  (bind _returnvalue (Game|GetPlayerController 0))
  (bind _returnvalue_2 (UserInterface|CreateWidget "/Game/RollingWithThePunches/Blueprints/HUDs/LevelSelect/LVS_WorldMenu.LVS_WorldMenu_C"))
  (UserInterface|Viewport|AddtoViewport _returnvalue_2 0)
  (Input|SetInputModeGameandUI _returnvalue (Variables|/Game/RollingWithThePunches/Blueprints/HUDs/LevelSelect/LVS_WorldMenu.LVS_WorldMenu_C|GetLVS_TutorialButton _returnvalue_2) "DoNotLock" true)
  (Variables|/Script/Engine.PlayerController|SetbShowMouseCursor _returnvalue true)
  (Utilities|FlowControl|Delay 0.2)
  (Widget|SetKeyboardFocus (Variables|/Game/RollingWithThePunches/Blueprints/HUDs/LevelSelect/LVS_WorldMenu.LVS_WorldMenu_C|GetLVS_TutorialButton _returnvalue_2)))

(event Custom|SwitchWorldCamera
  (if (> (Variables|Default|GetCurrentCamera) (- (Utilities|Array|Length (Variables|Default|GetLevelSelectCameras)) 1))
    (Variables|Default|SetCurrentCamera 0))
  (if (< (Variables|Default|GetCurrentCamera) 0)
    (Variables|Default|SetCurrentCamera (- (Utilities|Array|Length (Variables|Default|GetLevelSelectCameras)) 1)))
  (Game|Player|SetViewTargetwithBlend (Game|GetPlayerController 0) (Utilities|Array|Get(acopy) (Variables|Default|GetLevelSelectCameras) (Variables|Default|GetCurrentCamera)) 1.0 "VTBlend_Linear" 0.0 false))

(event Custom|ZoomCameraBack%28In%29
  ;[0 0.7629 1] Zoom Functions
)

(event Custom|PlayAmbience
  (Audio|Components|Audio|Play (Variables|Default|GetAmbienceAudio) 0.0))

(event Custom|ZoomCameraOut
  ;[0 0.7629 1] Zoom Functions
  (bind _zoomalpha (Timeline|ZoomOutTimeline Play)))

(event Custom|CheckForZoomHUD
  ;[0 0.5001 1] Zoom-Out
  (Utilities|IsValid 0
    (:Is%20Valid
      (if true
        _))))

(event Custom|StopAmbience
  (bind _ambienceaudio (Variables|Default|GetAmbienceAudio))
  (Audio|Components|Audio|FadeOut _ambienceaudio 0.1 0.0 "Linear" :!class /Script/Engine.AudioComponent)
  (Audio|Components|Audio|Stop _ambienceaudio))

(event Custom|NormalVolume
  (Audio|Components|Audio|SetVolumeMultiplier (Variables|Default|GetAmbienceAudio) 1.0 :!class /Script/Engine.AudioComponent))

(event Custom|LowereredVolume
  (Audio|Components|Audio|SetVolumeMultiplier (Variables|Default|GetAmbienceAudio) 0.5 :!class /Script/Engine.AudioComponent))

(event Collision|EventHit
  (params (MyComp :type Primitive%20Component%20Object%20Reference) (Other :type Actor%20Object%20Reference) (OtherComp :type Primitive%20Component%20Object%20Reference) (bSelfMoved :type Boolean) (HitLocation :type Vector :default "0, 0, 0") (HitNormal :type Vector :default "0, 0, 0") (NormalImpulse :type Vector :default "0, 0, 0") (Hit :type Hit%20Result%20Structure%20%28by%20ref%29))
  (Audio|PlaySoundatLocation "/Game/RollingWithThePunches/Assets/Sounds/Ball/Ball_Cue.Ball_Cue" HitLocation "0, 0, 0" 1.0 1.0 0.0 0 0 0 0))

(event EventBeginPlay
  (Utilities|FlowControl|Sequence
    (:then_0
      (CallFunction|Initialize))
    (:then_1
      (CallFunction|LoadGame))
    (:then_2
      (Audio|PlaySound2D "/Game/RollingWithThePunches/Assets/Sounds/HUD_SFX/Backspin.Backspin" 1.0 1.0 0.0 0 0)
      (Utilities|FlowControl|Delay 1.1)
      (bind _returnvalue (AddComponent|AddAudioComponent false))
      (Variables|Default|SetAmbienceAudio _returnvalue))))

(event Input|ActionEvents|InputActionJump/StopBall
  (params (Key :type Key%20Structure :default "None")))

(event Input|ActionEvents|InputActionSprint
  (params (Key :type Key%20Structure :default "None"))
  ;[0 0.5001 1] Zoom-Out
)

(event Input|ActionEvents|InputActionPauseGame
  (params (Key :type Key%20Structure :default "None")))

(event Input|AxisEvents|InputAxisMoveForward/Backward
  (params (AxisValue :type Float%20%28single-precision%29))
  ;[1 0.8504 0] Movement
)

(event Input|AxisEvents|InputAxisMoveRight/Left
  (params (AxisValue :type Float%20%28single-precision%29))
  ;[1 0.8504 0] Movement
)

(event Input|AxisEvents|InputAxisTurnRight/LeftMouse
  (params (AxisValue :type Float%20%28single-precision%29)))

(event Input|AxisEvents|InputAxisLookUp/DownMouse
  (params (AxisValue :type Float%20%28single-precision%29)))

(event Input|KeyboardEvents|Q
  (params (Key :type Key%20Structure :default "None"))
  (:Pressed
    (Development|PrintString (Utilities|String|ToString(Integer) (Utilities|Array|Length (Variables|Default|GetLevelSelectCameras))))))

(fn ConstructionScript)

(fn Initialize
  (Utilities|FlowControl|Sequence
    (:then_0
      (CallFunction|OpenWorldMenu))
    (:then_1
      (bind _outactors (Actor|GetAllActorsOfClass "/Game/RollingWithThePunches/Blueprints/Actors/BP_LevelSelectCamera.BP_LevelSelectCamera_C"))
      (bind _output_get (Variables|Default|SetLevelSelectCameras _outactors)))
    (:then_2
      (Game|Player|SetViewTargetwithBlend (Game|GetPlayerController 0) (Utilities|Array|Get(acopy) (Variables|Default|GetLevelSelectCameras)) 0.0 "VTBlend_Linear" 0.0 false))))

(fn LoadGame
  (bind _asbp_roll_ninstance (Utilities|Casting|CastToBP_RollNInstance (Game|GetGameInstance)))
  (Utilities|FlowControl|Sequence
    (:then_0
      (bind _returnvalue (Default|LoadHubData _asbp_roll_ninstance))
      (Variables|OldLevelSelect|SetLevelsCompleted _returnvalue))
    (:then_1
      (bind (_e_boulders _e_specials) (Default|LoadSetupData _asbp_roll_ninstance))
      (Variables|Default|SetCurrentBoulder _e_boulders)
      (Variables|Default|SetCurrentSpecial _e_specials))))