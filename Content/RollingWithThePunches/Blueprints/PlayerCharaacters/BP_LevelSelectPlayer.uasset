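; Player pawn for the level select hub: a physics ball rolled by camera-relative angular impulses.
; Holding Jump/StopBall freezes physics; Sprint then zooms the spring-arm camera out, otherwise showing a can't-zoom widget.
; Separate zoom-in events use their own timeline, and Interact messages the first overlapping BPI_Interact actor.
; BeginPlay creates the HUD and loads hub and setup data from BP_RollNInstance; pause toggles a menu.
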(event Custom|ZoomCameraIn
  ;[0 0.7629 1] Zoom Functions
  (Variables|Zoom|SetZoomedIn? true)
  (bind _zoomalpha (Timeline|ZoomInTimeline Play)
    (:Update
      (Variables|/Script/Engine.SpringArmComponent|SetTargetArmLength (Variables|Default|GetSpringArm) (Math|Float|Lerp (Variables|Zoom|GetDefaultArmLength) (Variables|Zoom|GetZoomInArmLength) _zoomalpha)))))

(event Custom|ZoomCameraBack%28Out%29
  ;[0 0.7629 1] Zoom Functions
  (bind _zoomalpha (Timeline|ZoomOutTimeline Reverse)
    (:Update
      (Variables|/Script/Engine.SpringArmComponent|SetTargetArmLength (Variables|Default|GetSpringArm) (Math|Float|Lerp (Variables|Zoom|GetDefaultArmLength) (Variables|Zoom|GetZoomOutArmLength) _zoomalpha)))))

(event Custom|ZoomCameraBack%28In%29
  ;[0 0.7629 1] Zoom Functions
  (Variables|Zoom|SetZoomedIn? false)
  (bind _zoomalpha (Timeline|ZoomInTimeline Reverse)
    (:Update
      (Variables|/Script/Engine.SpringArmComponent|SetTargetArmLength (Variables|Default|GetSpringArm) (Math|Float|Lerp (Variables|Zoom|GetDefaultArmLength) (Variables|Zoom|GetZoomInArmLength) _zoomalpha)))))

(event Custom|ZoomCameraOut
  ;[0 0.7629 1] Zoom Functions
  (bind _zoomalpha (Timeline|ZoomOutTimeline Play)
    (:Update
      (Variables|/Script/Engine.SpringArmComponent|SetTargetArmLength (Variables|Default|GetSpringArm) (Math|Float|Lerp (Variables|Zoom|GetDefaultArmLength) (Variables|Zoom|GetZoomOutArmLength) _zoomalpha)))))

(event Custom|CheckForZoomHUD
  ;[0 0.5001 1] Zoom-Out
  (Utilities|IsValid (stale Input|ActionEvents|InputActionSprint _returnvalue_2)
    (:Is%20Valid
      (if (UserInterface|Viewport|IsinViewport (stale Input|ActionEvents|InputActionSprint _returnvalue_2))
        (Default|FadeOut (stale Input|ActionEvents|InputActionSprint _returnvalue_2))))))

(event Collision|EventHit
  (params (MyComp :type Primitive%20Component%20Object%20Reference) (Other :type Actor%20Object%20Reference) (OtherComp :type Primitive%20Component%20Object%20Reference) (bSelfMoved :type Boolean) (HitLocation :type Vector :default "0, 0, 0") (HitNormal :type Vector :default "0, 0, 0") (NormalImpulse :type Vector :default "0, 0, 0") (Hit :type Hit%20Result%20Structure%20%28by%20ref%29))
  (Audio|PlaySoundatLocation "/Game/RollingWithThePunches/Assets/Sounds/Ball/Ball_Cue.Ball_Cue" HitLocation "0, 0, 0" 1.0 1.0 0.0 0 0 0 0))

(event EventBeginPlay
  (Utilities|FlowControl|Sequence
    (:then_0
      (CallFunction|Initialize))
    (:then_1
      (CallFunction|LoadGame))))

(event Input|ActionEvents|InputActionInteract
  (params (Key :type Key%20Structure :default "None"))
  ;[1 0 0.1143] Interact
  (:Pressed
    (bind _array_element (Utilities|Array|ForEachLoopwithBreak (Collision|GetOverlappingActors 0 :!class /Script/Engine.Actor) :!label _label)
      (:LoopBody
        (if (Utilities|DoesObjectImplementInterface _array_element "/Game/RollingWithThePunches/Blueprints/Interface/BPI_Interact.BPI_Interact_C")
          (Class|BPIInteract|Interact(Message) _array_element)
          (goto _label Break))))))

(event Input|ActionEvents|InputActionJump/StopBall
  (params (Key :type Key%20Structure :default "None"))
  (bind _sphere (Variables|Default|GetSphere))
  (bind _sphere_2 (Variables|Default|GetSphere))
  (:Pressed
    (Physics|SetSimulatePhysics _sphere_2 false)
    (Physics|SetPhysicsLinearVelocity _sphere "0, 0, 0" false "None")
    (Class|PrimitiveComponent|SetPhysicsAngularVelocityinDegrees _sphere "0, 0, 0" false "None")
    (Transformation|SetActorRotation (Variables|Default|GetDefaultRotation)))
  (:Released
    (Physics|SetSimulatePhysics _sphere_2 true)))

(event Input|ActionEvents|InputActionSprint
  (params (Key :type Key%20Structure :default "None"))
  (bind _zoomedin_ (Variables|Zoom|GetZoomedIn?))
  (bind _returnvalue (not _zoomedin_))
  ;[0 0.5001 1] Zoom-Out
  (:Pressed
    (if (and _returnvalue (not (Physics|IsSimulatingPhysics (Variables|Default|GetSphere) "None")))
      (CallFunction|ZoomCameraOut)
      (else
        (Utilities|FlowControl|DoOnce false :!label _label
          (:Completed
            (bind _returnvalue_2 (UserInterface|CreateWidget "/Game/RollingWithThePunches/Blueprints/HUDs/CantZoom_HUD.CantZoom_HUD_C"))
            (UserInterface|Viewport|AddtoViewport _returnvalue_2 0))))))
  (:Released
    (Utilities|FlowControl|Sequence
      (:then_0
        (if _returnvalue
          (CallFunction|ZoomCameraBack(Out))))
      (:then_1
        (CallFunction|CheckforZoomHUD)
        (goto _label Reset)))))

(event Input|ActionEvents|InputActionPauseGame
  (params (Key :type Key%20Structure :default "None"))
  (bind _returnvalue (Game|GetPlayerController 0))
  (:Pressed
    (if true
      (Utilities|IsValid (Variables|Default|GetPauseRef)
        (:Is%20Valid
          _)
        (:Is%20Not%20Valid
          (bind _returnvalue_2 (UserInterface|CreateWidget "/Game/RollingWithThePunches/Blueprints/HUDs/Menu/Pause_HUD.Pause_HUD_C"))
          (Variables|Default|SetPauseRef _returnvalue_2)))
      (Variables|/Game/RollingWithThePunches/Blueprints/HUDs/Menu/Pause_HUD.Pause_HUD_C|SetIsFirstPersonPlayer? _returnvalue_2 false)
      (if (Game|IsGamePaused)
        (Widget|RemovefromParent (Variables|Default|GetPauseRef))
        (Game|SetGamePaused false)
        (Variables|/Script/Engine.PlayerController|SetbShowMouseCursor _returnvalue false)
        (Input|SetInputModeGameOnly _returnvalue)
        (else
          (UserInterface|Viewport|AddtoViewport (Variables|Default|GetPauseRef) 0)
          (Game|SetGamePaused true)
          (Variables|/Script/Engine.PlayerController|SetbShowMouseCursor _returnvalue true)
          (Input|SetInputModeGameandUI _returnvalue (Variables|Default|GetPauseRef) "LockInFullscreen" true))))))

(event Input|ActionEvents|InputActionOpenLevelSetup
  (params (Key :type Key%20Structure :default "None")))

(event Input|AxisEvents|InputAxisMoveForward/Backward
  (params (AxisValue :type Float%20%28single-precision%29))
  ;[1 0.8504 0] Movement
  (if (Physics|IsSimulatingPhysics (Variables|Default|GetSphere) "None")
    (Class|PrimitiveComponent|AddAngularImpulseinDegrees (Variables|Default|GetSphere) (* (* (Variables|Default|GetRotationSpeed) AxisValue) (Math|Vector|GetForwardVector (Math|Rotator|MakeRotator 0.0 0.0 (.yaw (Pawn|GetControlRotation :!class /Script/Engine.Pawn))))) "None" true)))

(event Input|AxisEvents|InputAxisMoveRight/Left
  (params (AxisValue :type Float%20%28single-precision%29))
  (bind _returnvalue (Pawn|GetControlRotation :!class /Script/Engine.Pawn))
  ;[1 0.8504 0] Movement
  (if (Physics|IsSimulatingPhysics (Variables|Default|GetSphere) "None")
    (Class|PrimitiveComponent|AddAngularImpulseinDegrees (Variables|Default|GetSphere) (* (* (Variables|Default|GetRotationSpeed) AxisValue) (Math|Vector|GetRightVector (Math|Rotator|MakeRotator (.roll _returnvalue) 0.0 (.yaw _returnvalue)))) "None" true)))

(event Input|AxisEvents|InputAxisTurnRight/LeftMouse
  (params (AxisValue :type Float%20%28single-precision%29))
  (Pawn|Input|AddControllerYawInput AxisValue))

(event Input|AxisEvents|InputAxisLookUp/DownMouse
  (params (AxisValue :type Float%20%28single-precision%29))
  (Pawn|Input|AddControllerPitchInput AxisValue))

(fn ConstructionScript)

(fn Initialize
  (Utilities|FlowControl|Sequence
    (:then_0
      (Input|SetInputModeGameOnly (Game|GetPlayerController 0))
      (Variables|Zoom|SetDefaultArmLength (Variables|/Script/Engine.SpringArmComponent|GetTargetArmLength (Variables|Default|GetSpringArm)))
      (Variables|Default|SetDefaultRotation (Transformation|GetActorRotation)))
    (:then_1
      (bind _returnvalue (UserInterface|CreateWidget "/Game/RollingWithThePunches/Blueprints/HUDs/PlayerHUD_UI/LevelSelectPlayer/LevelSelect_PlayerHUD.LevelSelect_PlayerHUD_C"))
      (UserInterface|Viewport|AddtoViewport _returnvalue 0))))

(fn LoadGame
  (bind _asbp_roll_ninstance (Utilities|Casting|CastToBP_RollNInstance (Game|GetGameInstance)))
  (Utilities|FlowControl|Sequence
    (:then_0
      (bind _returnvalue (Default|LoadHubData _asbp_roll_ninstance))
      (Variables|Default|SetLevelsCompleted _returnvalue))
    (:then_1
      (bind (_e_boulders _e_specials) (Default|LoadSetupData _asbp_roll_ninstance))
      (Variables|Default|SetCurrentBoulder _e_boulders)
      (Variables|Default|SetCurrentSpecial _e_specials))))