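; Game instance for Rolling With The Punches that persists level records, loadout setup, and unlocked boulder and special rosters.
; Init creates one BP_RollNSave object, reused for every write, and caches each level's saved record in LevelDataMap.
; Each level saves to a slot named after it, keeping the fastest time with its punches, retries and boulder.
; Setup and rosters use fixed slots, and hub progress counts existing level slots.
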(event EventInit
  (Utilities|FlowControl|Sequence
    (:then_0
      (bind _returnvalue (SaveGame|CreateSaveGameObject "/Game/RollingWithThePunches/Blueprints/Saves/BP_RollNSave.BP_RollNSave_C"))
      (Variables|Default|SetSaveGameData _returnvalue)
      (CallFunction|LoadLevelData))
    (:then_1
      (Variables|Default|SetUnlock? false))))

(fn SaveLevelData
  (bind _asbp_first_person_character (Utilities|Casting|CastToBP_FirstPersonCharacter (Game|GetPlayerCharacter 0)))
  (Variables|Default|SetPlayerRef _asbp_first_person_character)
  (bind _returnvalue (Game|GetCurrentLevelName true))
  (bind _output_get (Variables|Default|SetCurrentLevelName _returnvalue))
  (bind _returnvalue_2 (SaveGame|DoesSaveGameExist _output_get))
  (if _returnvalue_2
    (LevelTime|SaveCheckforNewLevelTime)
    (else
      (LevelTime|SaveNewLevelTime))))

(fn LoadLevelData
  (for _array_element (Variables|Default|GetAllLevelNames)
    (bind _returnvalue (SaveGame|LoadGamefromSlot _array_element))
    (bind _asbp_roll_nsave (Utilities|Casting|CastToBP_RollNSave _returnvalue))
    (Utilities|Map|Add (Variables|Default|GetLevelDataMap) _array_element (Variables|/Game/RollingWithThePunches/Blueprints/Saves/BP_RollNSave.BP_RollNSave_C|GetLevelDataStruct _asbp_roll_nsave))))

(fn ClearSaveData)

(fn LoadHubData
  (Variables|Default|SetLevelsCompleted 0)
  (for _array_element (Variables|Default|GetAllHubLevelNames)
    (bind _returnvalue (SaveGame|DoesSaveGameExist _array_element))
    (if _returnvalue
      (Variables|Default|SetLevelsCompleted (+ (Variables|Default|GetLevelsCompleted) 1))))
  (bind _output_get (Variables|Default|SetLevelsCompleted (Variables|Default|GetLevelsCompleted)))
  (return _output_get))

(fn SaveSetupData
  (params (E_Boulders :type E_BoulderType%20Enum :default "NewEnumerator0") (E_Specials :type E_SpecialMove%20Enum :default "NewEnumerator4"))
  (bind _savegamedata (Variables|Default|GetSaveGameData))
  (Variables|/Game/RollingWithThePunches/Blueprints/Saves/BP_RollNSave.BP_RollNSave_C|SetE_Boulders _savegamedata E_Boulders)
  (Variables|/Game/RollingWithThePunches/Blueprints/Saves/BP_RollNSave.BP_RollNSave_C|SetE_Specials _savegamedata E_Specials)
  (SaveGame|SaveGametoSlot (Variables|Default|GetSaveGameData) "SaveSetup"))

(fn LoadSetupData
  (bind _returnvalue (SaveGame|LoadGamefromSlot "SaveSetup"))
  (bind _asbp_roll_nsave (Utilities|Casting|CastToBP_RollNSave _returnvalue))
  (return (Variables|/Game/RollingWithThePunches/Blueprints/Saves/BP_RollNSave.BP_RollNSave_C|GetE_Boulders _asbp_roll_nsave) (Variables|/Game/RollingWithThePunches/Blueprints/Saves/BP_RollNSave.BP_RollNSave_C|GetE_Specials _asbp_roll_nsave)))

(fn SetUnlock
  (switch string (Variables|Default|GetCurrentLevelName)
    (:PorcelainGarden1
      (Variables|Default|SetUnlock? false))
    (:PorcelainGarden2
      (Variables|Default|SetUnlock? false))
    (:PorcelainGarden3
      (Variables|Default|SetUnlock? true))
    (:PorcelainGarden4
      (Variables|Default|SetUnlock? false))
    (:PorcelainGarden5
      (Variables|Default|SetUnlock? true))
    (:PorcelainGarden6
      (Variables|Default|SetUnlock? false))
    (:PorcelainGarden7
      (Variables|Default|SetUnlock? true))
    (:PorcelainGarden8
      (Variables|Default|SetUnlock? false))
    (:PorcelainGarden9
      (Variables|Default|SetUnlock? true))
    (:PorcelainGarden10
      (Variables|Default|SetUnlock? false))
    (:RP_Tutorial
      (Variables|Default|SetUnlock? false))))

(fn SaveCheckforNewLevelTime
  (bind _leveldatamap (Variables|Default|GetLevelDataMap))
  (bind _playerref (Variables|Default|GetPlayerRef))
  (bind _currentlevelname (Variables|Default|GetCurrentLevelName))
  (bind _value (Utilities|Map|Find _leveldatamap _currentlevelname))
  (bind (_completiontimeundertime _numberofpunchesundertime _numberofretriesundertime _ballusedfortime) (Utilities|Struct|BreakBP_BasicStruct _value))
  ;[1 1 1] Compare Previous Records
  (if (< (Variables|/Game/RollingWithThePunches/Blueprints/PlayerCharaacters/BP_FirstPersonCharacter.BP_FirstPersonCharacter_C|GetLevelTime (Variables|Default|GetPlayerRef)) (Utilities|Struct|BreakBP_BasicStruct (.Value (Utilities|Map|Find (Variables|Default|GetLevelDataMap) (Variables|Default|GetCurrentLevelName)))))
    (Utilities|Struct|SetmembersinBP_BasicStruct (Variables|/Game/RollingWithThePunches/Blueprints/Saves/BP_RollNSave.BP_RollNSave_C|GetLevelDataStruct (Variables|Default|GetSaveGameData)) (Variables|/Game/RollingWithThePunches/Blueprints/PlayerCharaacters/BP_FirstPersonCharacter.BP_FirstPersonCharacter_C|GetLevelTime _playerref) (Variables|/Game/RollingWithThePunches/Blueprints/PlayerCharaacters/BP_FirstPersonCharacter.BP_FirstPersonCharacter_C|GetNumberOfPunches _playerref) (Variables|/Game/RollingWithThePunches/Blueprints/PlayerCharaacters/BP_FirstPersonCharacter.BP_FirstPersonCharacter_C|GetNumberOfRetries _playerref) (Variables|/Game/RollingWithThePunches/Blueprints/PlayerCharaacters/BP_FirstPersonCharacter.BP_FirstPersonCharacter_C|GetCurrentBoulderSymbol _playerref))
    (SaveGame|SaveGametoSlot (Variables|Default|GetSaveGameData) (Variables|Default|GetCurrentLevelName))
    (else
      (Utilities|Struct|SetmembersinBP_BasicStruct (Variables|/Game/RollingWithThePunches/Blueprints/Saves/BP_RollNSave.BP_RollNSave_C|GetLevelDataStruct (Variables|Default|GetSaveGameData)) _completiontimeundertime _numberofpunchesundertime _numberofretriesundertime _ballusedfortime)
      (SaveGame|SaveGametoSlot (Variables|Default|GetSaveGameData) (Variables|Default|GetCurrentLevelName)))))

(fn SaveNewLevelTime
  (bind _playerref (Variables|Default|GetPlayerRef))
  ;[1 1 1] Create New Save
  (bind _structout (Utilities|Struct|SetmembersinBP_BasicStruct (Variables|/Game/RollingWithThePunches/Blueprints/Saves/BP_RollNSave.BP_RollNSave_C|GetLevelDataStruct (Variables|Default|GetSaveGameData)) (Variables|/Game/RollingWithThePunches/Blueprints/PlayerCharaacters/BP_FirstPersonCharacter.BP_FirstPersonCharacter_C|GetLevelTime _playerref) (Variables|/Game/RollingWithThePunches/Blueprints/PlayerCharaacters/BP_FirstPersonCharacter.BP_FirstPersonCharacter_C|GetNumberOfPunches _playerref) (Variables|/Game/RollingWithThePunches/Blueprints/PlayerCharaacters/BP_FirstPersonCharacter.BP_FirstPersonCharacter_C|GetNumberOfRetries _playerref) true (Variables|/Game/RollingWithThePunches/Blueprints/PlayerCharaacters/BP_FirstPersonCharacter.BP_FirstPersonCharacter_C|GetCurrentBoulderSymbol _playerref)))
  (Utilities|Map|Add (Variables|Default|GetLevelDataMap) (Variables|Default|GetCurrentLevelName) _structout)
  (SaveGame|SaveGametoSlot (Variables|Default|GetSaveGameData) (Variables|Default|GetCurrentLevelName)))

(fn SaveBoulderRoster
  (params (NewBoulder :type E_BoulderType%20Enum :default "NewEnumerator0"))
  (bind _savegamedata (Variables|Default|GetSaveGameData))
  (bind _returnvalue (SaveGame|DoesSaveGameExist "SaveBoulderRoster"))
  (if _returnvalue
    (bind _boulderroster (BoulderRoster|LoadBoulderRoster))
    (Utilities|Map|Add _boulderroster NewBoulder true)
    (Variables|/Game/RollingWithThePunches/Blueprints/Saves/BP_RollNSave.BP_RollNSave_C|SetBoulderRoster (Variables|Default|GetSaveGameData) _boulderroster)
    (SaveGame|SaveGametoSlot (Variables|Default|GetSaveGameData) "SaveBoulderRoster")
    (else
      (Utilities|Map|Add (Variables|/Game/RollingWithThePunches/Blueprints/Saves/BP_RollNSave.BP_RollNSave_C|GetBoulderRoster _savegamedata) NewBoulder true)
      (Variables|/Game/RollingWithThePunches/Blueprints/Saves/BP_RollNSave.BP_RollNSave_C|SetBoulderRoster _savegamedata (Variables|/Game/RollingWithThePunches/Blueprints/Saves/BP_RollNSave.BP_RollNSave_C|GetBoulderRoster _savegamedata))
      (SaveGame|SaveGametoSlot (Variables|Default|GetSaveGameData) "SaveBoulderRoster"))))

(fn LoadBoulderRoster
  (bind _returnvalue (SaveGame|DoesSaveGameExist "SaveBoulderRoster"))
  (if _returnvalue
    (bind _returnvalue_2 (SaveGame|LoadGamefromSlot "SaveBoulderRoster"))
    (bind _asbp_roll_nsave (Utilities|Casting|CastToBP_RollNSave _returnvalue_2))
    (return (Variables|/Game/RollingWithThePunches/Blueprints/Saves/BP_RollNSave.BP_RollNSave_C|GetBoulderRoster _asbp_roll_nsave))
    (else
      (SaveGame|SaveGametoSlot (Variables|Default|GetSaveGameData) "SaveBoulderRoster"))))

(fn SaveSpecialRoster
  (params (NewSpecial :type E_SpecialMove%20Enum :default "NewEnumerator4"))
  (bind _savegamedata (Variables|Default|GetSaveGameData))
  (bind _returnvalue (SaveGame|DoesSaveGameExist "SaveSpecialRoster"))
  (if _returnvalue
    (bind _specialroster (SpecialRoster|LoadSpecialRoster))
    (Utilities|Map|Add _specialroster NewSpecial true)
    (Variables|/Game/RollingWithThePunches/Blueprints/Saves/BP_RollNSave.BP_RollNSave_C|SetSpecialRoster (Variables|Default|GetSaveGameData) _specialroster)
    (SaveGame|SaveGametoSlot (Variables|Default|GetSaveGameData) "SaveSpecialRoster")
    (else
      (Utilities|Map|Add (Variables|/Game/RollingWithThePunches/Blueprints/Saves/BP_RollNSave.BP_RollNSave_C|GetSpecialRoster _savegamedata) NewSpecial true)
      (Variables|/Game/RollingWithThePunches/Blueprints/Saves/BP_RollNSave.BP_RollNSave_C|SetSpecialRoster _savegamedata (Variables|/Game/RollingWithThePunches/Blueprints/Saves/BP_RollNSave.BP_RollNSave_C|GetSpecialRoster _savegamedata))
      (SaveGame|SaveGametoSlot (Variables|Default|GetSaveGameData) "SaveSpecialRoster"))))

(fn LoadSpecialRoster
  (bind _returnvalue (SaveGame|DoesSaveGameExist "SaveSpecialRoster"))
  (if _returnvalue
    (bind _returnvalue_2 (SaveGame|LoadGamefromSlot "SaveSpecialRoster"))
    (bind _asbp_roll_nsave (Utilities|Casting|CastToBP_RollNSave _returnvalue_2))
    (return (Variables|/Game/RollingWithThePunches/Blueprints/Saves/BP_RollNSave.BP_RollNSave_C|GetSpecialRoster _asbp_roll_nsave))
    (else
      (SaveGame|SaveGametoSlot (Variables|Default|GetSaveGameData) "SaveSpecialRoster"))))